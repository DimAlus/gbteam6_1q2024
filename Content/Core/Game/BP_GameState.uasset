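; Game State Blueprint that applies configured audio volume levels when play begins.
; After calling the parent BeginPlay, a Sequence reads the master, music, effects and voice volumes through GetConfig.
; Each value becomes a Sound Class override with no fade on that category's Sound Mix, which is then pushed as a modifier.
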(event EventBeginPlay
  (|CallParentFunction)
  (Utilities|FlowControl|Sequence
    (:then_0
      (bind _config (CallFunction|GetConfig "F_SoundValue"))
      (Audio|SetSoundMixClassOverride "/Game/Sound/SoundClass/Mix_MasterSound.Mix_MasterSound" "/Game/Sound/SoundClass/MasterSound.MasterSound" (Utilities|Struct|BreakConfig _config) 1.0 0.0 true)
      (Audio|PushSoundMixModifier "/Game/Sound/SoundClass/Mix_MasterSound.Mix_MasterSound"))
    (:then_1
      (bind _config_2 (CallFunction|GetConfig "F_MusicValue"))
      (Audio|SetSoundMixClassOverride "/Game/Sound/SoundClass/Mix_MusicSound.Mix_MusicSound" "/Game/Sound/SoundClass/MusicSound.MusicSound" (Utilities|Struct|BreakConfig _config_2) 1.0 0.0 true)
      (Audio|PushSoundMixModifier "/Game/Sound/SoundClass/Mix_MusicSound.Mix_MusicSound"))
    (:then_2
      (bind _config_3 (CallFunction|GetConfig "F_EffectValue"))
      (Audio|SetSoundMixClassOverride "/Game/Sound/SoundClass/Mix_EffectsSound.Mix_EffectsSound" "/Game/Sound/SoundClass/EffectsSound.EffectsSound" (Utilities|Struct|BreakConfig _config_3) 1.0 0.0 true)
      (Audio|PushSoundMixModifier "/Game/Sound/SoundClass/Mix_EffectsSound.Mix_EffectsSound"))
    (:then_3
      (bind _config_4 (CallFunction|GetConfig "F_VoiceValue"))
      (Audio|SetSoundMixClassOverride "/Game/Sound/SoundClass/Mix_VoiceSound.Mix_VoiceSound" "/Game/Sound/SoundClass/VoiceSound.VoiceSound" (Utilities|Struct|BreakConfig _config_4) 1.0 0.0 true)
      (Audio|PushSoundMixModifier "/Game/Sound/SoundClass/Mix_VoiceSound.Mix_VoiceSound"))))

(fn ConstructionScript)