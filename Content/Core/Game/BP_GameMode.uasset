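; Game mode that caps frame rate, enables VSync and registers debug console commands at BeginPlay.
; Command names come from data table rows and are bound to callbacks by name prefix before the console commands are initialized.
; Callbacks add a resource to the inventory of the player pawn's selected core, or spawn a given number of actors of a chosen class at the pawn's location.
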(event Custom|ConsoleSpawn
  (params (Params :type Array%20of%20Console%20Command%20Param%20Structures))
  (bind _returnvalue (Class|GameModeDefault|GetPlayerPawnDefault))
  (bind _output (Utilities|Array|Get(acopy) Params))
  (bind _classvalue (Utilities|Struct|BreakConsoleCommandParam _output))
  (Utilities|IsValid _returnvalue
    (:Is%20Valid
      (if (Utilities|IsValidClass _classvalue)
        (for _index (range 1 (Utilities|Struct|BreakConsoleCommandParam (Utilities|Array|Get(acopy) Params 1)))
          (Game|SpawnActorfromClass _classvalue (Math|Transform|MakeTransform (Transformation|GetActorLocation _returnvalue) "0, 0, 0" "1.000000,1.000000,1.000000") "Undefined" "MultiplyWithRoot" 0 0))))))

(event Custom|ConsoleAddResource
  (params (Params :type Array%20of%20Console%20Command%20Param%20Structures))
  (bind _returnvalue (Class|GameModeDefault|GetPlayerPawnDefault))
  (bind _currentselectedcore (Variables|/Script/GBTeam6.PlayerPawnDefault|GetCurrentSelectedCore _returnvalue))
  (Utilities|IsValid _returnvalue
    (:Is%20Valid
      (Utilities|IsValid _currentselectedcore
        (:Is%20Valid
          (bind _returnvalue_2 (Class|GameObjectCore|GetComponent _currentselectedcore "Inventory"))
          (bind _asinventory_base_component (Utilities|Casting|CastToInventoryBaseComponent _returnvalue_2))
          (Class|InventoryBaseComponent|ChangeInventory _asinventory_base_component (Utilities|Array|MakeArray (Utilities|Struct|MakePrice (Utilities|Struct|BreakConsoleCommandParam (Utilities|Array|Get(acopy) Params)) (Utilities|Struct|BreakConsoleCommandParam (Utilities|Array|Get(acopy) Params 1)))) false))))))

(event EventBeginPlay
  (Utilities|FlowControl|Sequence
    (:then_0
      (Development|ExecuteConsoleCommand "t.MaxFPS 60" 0)
      (Development|ExecuteConsoleCommand "r.Vsync 1" 0))
    (:then_1
      (bind _outrownames (DataTable|GetDataTableRowNames (Variables|Default|GetDT_ConsoleCommands)))
      (for _array_element _outrownames
        (switch string (CallFunction|GetPrefix _array_element)
          (:g.r
            (Class|GameModeDefault|AddConsoleCommand _array_element (EventDispatchers|CreateEvent :!event Custom|ConsoleAddResource)))
          (:g.s
            (Class|GameModeDefault|AddConsoleCommand _array_element (EventDispatchers|CreateEvent :!event Custom|ConsoleSpawn))))))
    (:then_2
      (Class|GameModeDefault|InitializeConsoleCommands))))

(fn ConstructionScript)

(fn GetPrefix
  (params (name :type Name))
  (bind _returnvalue (Utilities|String|ToString(Name) name))
  (for _array_element (LocalVariables|Getprefixes)
    (if (Utilities|String|StartsWith _returnvalue _array_element)
      (return _array_element)))
  (return _returnvalue))