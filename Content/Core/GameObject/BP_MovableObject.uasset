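; Base Blueprint for a movable, selectable AI unit that runs a behavior tree and wires itself to its Core's components once created.
; AI, Social and Health events drive walk speed, team-relation selection materials and ragdoll death.
; Skill intentions turn the unit, lock movement via blackboard and play a montage whose notify casts the skill.
; It also attaches a weapon, initializes a health bar and freezes physics on game pause.
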(event Custom|OnSelectionTouch_Event
  (bind _timermanager (CallFunction|GetGameTimerManager))
  ;[1 1 1 1 60] Selection
  (Class|TimerService|InvalidateTimer _timermanager (Variables|Default|GetOnSelectionTouchEnd_Handler))
  (CallFunction|SetSelectionObjectMaterial (Variables|Selection|GetSelectionCommandMaterial))
  (bind _returnvalue (Class|TimerService|SetTimer _timermanager (delegate Custom|OnSelectionTouchEnd_Event) 0.6 false -1.0 false true))
  (Variables|Default|SetOnSelectionTouchEnd_Handler _returnvalue))

(event Custom|OnSelectionChanging_Event
  ;[1 1 1 1 60] Selection
  (bind _returnvalue (Class|GameObjectInterface|GetCore))
  (bind _returnvalue_2 (Class|GameObjectCore|GetComponent _returnvalue "AI"))
  (bind _asaibase_component (Utilities|Casting|CastToAIBaseComponent _returnvalue_2))
  (bind _returnvalue_3 (Class|AIBaseComponent|GetSelection _asaibase_component))
  (Utilities|FlowControl|Sequence
    (:then_0
      (if (.Preview (Utilities|Struct|BreakObjectSelection _returnvalue_3))
        (CallFunction|SetSelectionObjectMaterial (Variables|Selection|GetSelectionPreviewMaterial))
        (elif (.Selection (Utilities|Struct|BreakObjectSelection _returnvalue_3))
          (CallFunction|SetSelectionObjectMaterial (Variables|Selection|GetSelectionMaterial))
          (elif (.MouseTurn (Utilities|Struct|BreakObjectSelection _returnvalue_3))
            (CallFunction|SetSelectionObjectMaterial (Variables|Selection|GetSelectionMouseMaterial))
            (else
              (CallFunction|SetSelectionObjectMaterial))))))
    (:then_1
      (bind _aswbp_object_short_staticstic (Utilities|Casting|CastToWBP_ObjectShortStaticstic (UserInterface|GetWidget (Variables|Default|GetHealthBar))))
      (Default|SetMouseTurned _aswbp_object_short_staticstic (.MouseTurn (Utilities|Struct|BreakObjectSelection _returnvalue_3))))))

(event Custom|AddVelocityOnDamage
  (params (DamagedActor :type Actor%20Object%20Reference) (Damage :type Float%20%28single-precision%29) (DamageType :type Damage%20Type%20Object%20Reference) (InstigatedBy :type Controller%20Object%20Reference) (DamageCauser :type Actor%20Object%20Reference))
  ;[1 1 1 1 60] Dead
  ;;[1 1 1] Rewrite
  (Physics|SetPhysicsLinearVelocity (Variables|Character|GetMesh) (+ (* (Math|Vector|Normalize (* (- (Transformation|GetActorLocation DamagedActor) (Transformation|GetActorLocation DamageCauser)) "1.000000,1.000000,0.000000")) (Math|Float|MakeLiteralFloat 1e+03)) "0.000000,0.000000,400.000000") false "Spine2"))

(event Custom|OnCreatingAfter_Event
  (bind _healthbar (Variables|Default|GetHealthBar))
  (Utilities|FlowControl|Sequence
    (:then_0
      ;[1 1 1] Send Spawn message
      (bind _asgame_state_default (Utilities|Casting|CastToGameStateDefault (Game|GetGameState)))
      (Class|MessageService|Send (Class|GameStateDefault|GetMessageService _asgame_state_default) (Utilities|Set|MakeSet "GOASpawn") (Variables|Default|GetCore)))
    (:then_1
      ;[1 1 1] Dead Events
      (bind _returnvalue (Class|GameObjectCore|GetComponent (Variables|Default|GetCore) "Health"))
      (bind _ashealth_base_component (Utilities|Casting|CastToHealthBaseComponent _returnvalue))
      (EventDispatchers|BindEventtoOnDeath _ashealth_base_component (EventDispatchers|CreateEvent :!event Custom|OnDead_Event))
      (EventDispatchers|BindEventtoOnTryDead _ashealth_base_component (EventDispatchers|CreateEvent :!event Custom|OnDeadMovementDownBefore)))
    (:then_2
      (bind _returnvalue_2 (Class|GameObjectCore|GetComponent (Variables|Default|GetCore) "AI"))
      (bind _asaibase_component (Utilities|Casting|CastToAIBaseComponent _returnvalue_2))
      (EventDispatchers|AssignOnSelectionChanging _asaibase_component (EventDispatchers|CreateEvent :!event Custom|OnSelectionChanging_Event))
      (EventDispatchers|BindEventtoOnSelectionTouch _asaibase_component (EventDispatchers|CreateEvent :!event Custom|OnSelectionTouch_Event))
      (EventDispatchers|AssignOnSpeedChanging _asaibase_component (EventDispatchers|CreateEvent :!event Custom|OnSpeedChanging_Event))
      (bind _returnvalue_3 (Class|AIBaseComponent|GetSpeed _asaibase_component))
      (CallFunction|OnSpeedChangingEvent _returnvalue_3))
    (:then_3
      (bind _returnvalue_4 (Class|GameObjectCore|GetComponent (Variables|Default|GetCore) "SkillHeaver"))
      (bind _asskill_heaver_base_component (Utilities|Casting|CastToSkillHeaverBaseComponent _returnvalue_4))
      (EventDispatchers|BindEventtoOnSkillIntention _asskill_heaver_base_component (EventDispatchers|CreateEvent :!event Custom|OnSkillIntenrion_Event)))
    (:then_4
      (bind _asplayer_pawn_default (Utilities|Casting|CastToPlayerPawnDefault (Game|Player|GetPlayerPawn 0)))
      (EventDispatchers|BindEventtoOnGameSpeedChanged _asplayer_pawn_default (EventDispatchers|CreateEvent :!event Custom|PhysicsDebugOnGameSpeedChange)))
    (:then_5
      (bind _aswbp_object_short_staticstic (Utilities|Casting|CastToWBP_ObjectShortStaticstic (UserInterface|GetWidget _healthbar)))
      (Default|Init _aswbp_object_short_staticstic (Variables|Default|GetCore) _healthbar))
    (:then_6
      (CallFunction|LockMoving false))
    (:then_7
      (bind _returnvalue_5 (Class|GameObjectCore|GetComponent (Variables|Default|GetCore) "Social"))
      (bind _associal_base_component (Utilities|Casting|CastToSocialBaseComponent _returnvalue_5))
      (EventDispatchers|BindEventtoOnSocialTeamChanging _associal_base_component (EventDispatchers|CreateEvent :!event UpdateSelectionViewMaterials))
      (CallFunction|UpdateSelectionViewMaterials))
    (:then_8
      (CallFunction|EquipWeaponEvent))))

(event Custom|OnSkillIntenrion_Event
  (params (SkillSlot :type ESkillSlot%20Enum :default "None") (Targets :type Array%20of%20Game%20Object%20Core%20Object%20References) (Location :type Vector))
  (bind _returnvalue (Transformation|GetActorLocation))
  (bind _returnvalue_2 (Transformation|GetActorRotation))
  ;[1 1 1] Attack Animation
  (Utilities|FlowControl|Sequence
    (:then_0
      (if (Utilities|Array|IsEmpty Targets)
        (Transformation|SetActorRotation (Math|Rotator|MakeRotator (.roll _returnvalue_2) (.pitch _returnvalue_2) (.yaw (Math|Rotator|FindLookatRotation _returnvalue Location))))
        (else
          (bind _returnvalue_3 (Class|GameObjectCore|GetOwner (Utilities|Array|Get(acopy) Targets)))
          (Transformation|SetActorRotation (Math|Rotator|MakeRotator (.roll _returnvalue_2) (.pitch _returnvalue_2) (.yaw (Math|Rotator|FindLookatRotation _returnvalue (Transformation|GetActorLocation _returnvalue_3))))))))
    (:then_1
      (if (Utilities|Map|Contains (Variables|Attack|GetAttackAnimData) SkillSlot)
        (bind _returnvalue_4 (Class|GameObjectCore|GetComponent (Variables|Default|GetCore) "SkillHeaver"))
        (bind _asskill_heaver_base_component (Utilities|Casting|CastToSkillHeaverBaseComponent _returnvalue_4))
        (Class|SkillHeaverBaseComponent|CancelSkillCast _asskill_heaver_base_component)
        (CallFunction|LockMoving true)
        (Animation|Montage|PlayMontage (Variables|Character|GetMesh) (.OutItem (Utilities|Array|Random (Utilities|Struct|BreakBPS_AnimationArray (.Value (Utilities|Map|Find (Variables|Attack|GetAttackAnimData) SkillSlot)))))
          (:OnCompleted
            (CallFunction|LockMoving false :!label _label))
          (:OnBlendOut
            (goto _label))
          (:OnInterrupted)
          (:OnNotifyBegin
            (bind _returnvalue_5 (Class|GameObjectInterface|GetLocationbyTypes (Utilities|Array|MakeArray "SkillCast" "Actor")))
            (Class|SkillHeaverBaseComponent|CastSkill _asskill_heaver_base_component SkillSlot Targets Location (.Location (Math|Transform|BreakTransform _returnvalue_5)))))))))

(event Custom|OnDead_Event
  ;[1 1 1 1 60] Dead
  (CallFunction|NotDead)
  (CallFunction|DeadAnimation)
  (CallFunction|DestroyWeaponEvent))

(event Custom|DestroyWeapon_Event
  (bind _weaponactor (Variables|Weapon|GetWeaponActor))
  ;[0.15 0.15 0.15 0.5] Weapon
  (Utilities|IsValid _weaponactor
    (:Is%20Valid
      (Actor|DestroyActor _weaponactor))))

(event Custom|EquipWeapon_Event
  (bind _weaponclass (Variables|Weapon|GetWeaponClass))
  ;[0.15 0.15 0.15 0.5] Weapon
  (if (Utilities|IsValidClass _weaponclass)
    (bind _returnvalue (Game|SpawnActorfromClass _weaponclass (Math|Transform|MakeTransform "0, 0, 0") "Undefined" "MultiplyWithRoot" 0 0))
    (bind _output_get (Variables|Weapon|SetWeaponActor _returnvalue))
    (Transformation|AttachComponentToComponent _output_get (Variables|Character|GetMesh) (Variables|Weapon|GetWeaponSocketName) "SnapToTarget" "SnapToTarget" "SnapToTarget" true)))

(event Custom|PhysicsDebugOnGameSpeedChange
  (bind _mesh (Variables|Character|GetMesh))
  ;[1 1 1 1 60] OnChangeSpeed
  (bind _asplayer_pawn_default (Utilities|Casting|CastToPlayerPawnDefault (Game|Player|GetPlayerPawn 0)))
  (if (Variables|/Script/GBTeam6.PlayerPawnDefault|GetCurrentGamePaused _asplayer_pawn_default)
    (Class|SkeletalMeshComponent|SuspendClothingSimulation _mesh)
    (Physics|SetEnableGravity _mesh false)
    (for _array_element (Transformation|GetAllSocketNames _mesh)
      (Class|PrimitiveComponent|PutRigidBodytoSleep _mesh _array_element))
    (Actor|Tick|SetActorTickEnabled false)
    (Collision|SetCollisionObjectType _mesh "ECC_GameTraceChannel5")
    (else
      (Class|SkeletalMeshComponent|ResumeClothingSimulation _mesh)
      (Physics|SetEnableGravity _mesh true)
      (if (not (Variables|Default|GetIsLiquidationStarted))
        (Class|PrimitiveComponent|WakeAllRigidBodies _mesh)
        (Actor|Tick|SetActorTickEnabled true)
        (Collision|SetCollisionObjectType _mesh "ECC_Pawn")))))

(event Custom|NotDead
  ;[1 1 1 1 60] Dead
  (bind _returnvalue (Class|GameObjectInterface|GetCore))
  (bind _returnvalue_2 (Class|GameObjectCore|GetComponent _returnvalue "Health"))
  (bind _ashealth_base_component (Utilities|Casting|CastToHealthBaseComponent _returnvalue_2))
  (Class|HealthBaseComponent|NotDestroyNow _ashealth_base_component))

(event Custom|OnSelectionTouchEnd_Event
  ;[1 1 1 1 60] Selection
  (CallFunction|OnSelectionChangingEvent))

(event Custom|OnDeadMovementDown
  ;[1 1 1 1 60] Dead
  (CallFunction|PleaseDead))

(event Custom|DeadAnimation
  (bind _mesh (Variables|Character|GetMesh))
  ;[1 1 1 1 60] Dead
  (CallFunction|NotDead)
  (Pawn|UnPossess (Pawn|GetController))
  (Collision|SetCollisionEnabled _mesh "PhysicsOnly")
  (Physics|SetSimulatePhysics _mesh true)
  (Physics|SetEnableGravity _mesh true)
  (Utilities|Time|SetTimerbyEvent (EventDispatchers|CreateEvent :!event Custom|PleaseDead) 3.0))

(event Custom|PleaseDead
  ;[1 1 1 1 60] Dead
  (bind _returnvalue (Class|GameObjectInterface|GetCore))
  (bind _returnvalue_2 (Class|GameObjectCore|GetComponent _returnvalue "Health"))
  (bind _ashealth_base_component (Utilities|Casting|CastToHealthBaseComponent _returnvalue_2))
  (Class|HealthBaseComponent|PleaseDead _ashealth_base_component))

(event Custom|OnSpeedChanging_Event
  (params (Value :type Float%20%28single-precision%29))
  ;[1 1 1] MaxWalkSpeed
  (Variables|/Script/Engine.CharacterMovementComponent|SetMaxWalkSpeed (Variables|Character|GetCharacterMovement) Value))

(event Custom|OnDeadMovementDownBefore
  (params (Lifes :type Integer))
  (bind _mesh (Variables|Character|GetMesh))
  ;[1 1 1 1 60] Dead
  (if (== Lifes 1)
    (Physics|SetEnableGravity _mesh true)
    (Collision|SetCollisionResponsetoChannel _mesh "ECC_GameTraceChannel2" "ECR_Ignore")
    (Collision|SetCollisionObjectType _mesh "ECC_Destructible")
    (Variables|/Script/Engine.SkeletalMeshComponent|SetbPauseAnims _mesh true)
    (Collision|SetCollisionObjectType _mesh "ECC_GameTraceChannel5")
    (Variables|Default|SetIsLiquidationStarted true)
    (Variables|Local|SetCurrentDeathTime 1e+01)
    (Utilities|Time|SetTimerbyEvent (EventDispatchers|CreateEvent :!event Custom|OnDeadMovementDown) 2.0)))

(event EventBeginPlay
  (AI|RunBehaviorTree (AI|GetAIController self) (Variables|AI|GetBehaviourTree))
  (|CallParentFunction)
  (bind _returnvalue (Class|GameObjectInterface|GetCore))
  (Variables|Default|SetCore _returnvalue)
  (if (Class|GameObjectCore|GetIsCreated _returnvalue)
    (CallFunction|OnCreatingAfterEvent)
    (else
      (EventDispatchers|AssignOnCreatingAfter _returnvalue (delegate Custom|OnCreatingAfter_Event)))))

(fn ConstructionScript)

(fn LockMoving
  (params (IsLocked :type Boolean))
  (bind _returnvalue (Pawn|GetController))
  (bind _returnvalue_2 (AI|GetBlackboard _returnvalue))
  (Utilities|IsValid _returnvalue_2
    (:Is%20Valid
      (AI|Components|Blackboard|SetValueasBool _returnvalue_2 (LocalVariables|GetKeyMovingLocked) IsLocked))))

(fn GetLocationbyType
  (params (LocationType :type ELocationType%20Enum :default "None"))
  (switch Utilities|FlowControl|Switch|SwitchonELocationType LocationType
    (:None
      _)
    (:Actor
      _)
    (:SkillCast
      (return true (Math|Conversions|ToTransform(Vector) (Transformation|GetSocketLocation (Variables|Character|GetMesh) "RightHandSocket"))))
    (:Delivery
      _)
    (:Spawn
      _)
    (:Work
      _)
    (:Attach
      _))
  (bind (_found _returnvalue) (|CallParentFunction LocationType))
  (return _found _returnvalue))

(fn GetObjectBounds
  (bind _mousecollision (Variables|Default|GetMouseCollision))
  (return (Class|KismetMathLibrary|MakeBoxSphereBounds (Transformation|GetWorldLocation _mousecollision) (* (Transformation|GetWorldScale _mousecollision) "32.000000,32.000000,32.000000") 0.0)))

(fn SetCanWork
  (params (CanWork :type Boolean))
  (AI|Components|Blackboard|SetValueasBool (AI|GetBlackboard (Pawn|GetController)) (Utilities|Name|MakeLiteralName "bCanWork") CanWork))

(fn SetCustomDepthStencil
  (params (Value :type Integer))
  (Rendering|SetCustomDepthStencilValue (Variables|Character|GetMesh) Value))

(fn SetSelectionObjectMaterial
  (params (material :type Material%20Instance%20Object%20Reference))
  (bind _selectionobject_view (Variables|Selection|GetSelectionObject_View))
  (Utilities|IsValid material
    (:Is%20Valid
      (Rendering|SetVisibility _selectionobject_view true false)
      (Rendering|Material|SetMaterial _selectionobject_view 0 material))
    (:Is%20Not%20Valid
      (Rendering|SetVisibility _selectionobject_view false false))))

(fn UpdateSelectionViewMaterials
  (Utilities|FlowControl|Sequence
    (:then_0
      (bind _returnvalue (Class|GameObjectCore|GetComponent (Variables|Default|GetCore) "Social"))
      (bind _associal_base_component (Utilities|Casting|CastToSocialBaseComponent _returnvalue))
      (bind _returnvalue_2 (Class|SocialBaseComponent|GetSocialTeam _associal_base_component))
      (bind _returnvalue_3 (Class|SocialService|GetRelationsBetweenTeams (CallFunction|GetSocialService) "Friendly" _returnvalue_2))
      (Utilities|FlowControl|Sequence
        (:then_0
          (Variables|Selection|SetSelectionMaterial (.Value (Utilities|Map|Find (Variables|Selection|GetSelectionMaterials) _returnvalue_3))))
        (:then_1
          (Variables|Selection|SetSelectionCommandMaterial (.Value (Utilities|Map|Find (Variables|Selection|GetSelectionCommandMaterials) _returnvalue_3))))
        (:then_2
          (Variables|Selection|SetSelectionPreviewMaterial (.Value (Utilities|Map|Find (Variables|Selection|GetSelectionPreviewMaterials) _returnvalue_3))))
        (:then_3
          (Variables|Selection|SetSelectionMouseMaterial (.Value (Utilities|Map|Find (Variables|Selection|GetSelectionMouseMaterials) _returnvalue_3))))))
    (:then_1
      (CallFunction|OnSelectionChangingEvent))))

(fn CheckasTarget
  (return false))

(fn GetCurrentDeliveryTask
  (bind _returnvalue (Class|GameObjectInterface|GetCore))
  (bind _returnvalue_2 (Class|GameObjectCore|GetComponent _returnvalue "Tasker"))
  (bind _astasker_default_component (Utilities|Casting|CastToTaskerDefaultComponent _returnvalue_2)
    (:then
      (bind (_exists _returnvalue_3) (Class|TaskerBaseComponent|GetCurrentTask _astasker_default_component))
      (return _exists _returnvalue_3))
    (:CastFailed
      (return false ""))))

(fn GetSkillStatus
  (params (SkillName :type String)))

(fn GetTaskProcessLocation
  (params (Worker :type Game%20Object%20Core%20Object%20Reference) (Task :type Game%20Task%20Structure%20%28by%20ref%29))
  (return (Transformation|GetActorLocation)))

(fn PrepareSkill
  (params (SkillName :type String)))

(fn TryGetPowerStatus
  (return false false false 0))