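; Simple game object Blueprint that hooks into its Core's components for selection highlighting, skill casting and task work points.
; Once the Core is created, it binds AI selection events to custom depth stencil values on its mesh, including a brief touch flash.
; Skill intentions from SkillHeaver cancel any current cast and recast from AttackLocation.
; It counts as a target when its Generator level is above zero, and supplies work or delivery locations for tasks.
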(event Custom|OnSelectionTouch_Event
  ;[1 1 1] Selection
  (Rendering|SetCustomDepthStencilValue (Variables|Default|GetObjectMesh) 2)
  (Utilities|FlowControl|Delay 0.2)
  (CallFunction|OnSelectionChangingEvent))

(event Custom|OnSelectionChanging_Event
  (bind _objectmesh (Variables|Default|GetObjectMesh))
  ;[1 1 1] Selection
  (bind _returnvalue (Class|GameObjectCore|GetComponent (Variables|Default|GetCore) "AI"))
  (bind _asaibase_component (Utilities|Casting|CastToAIBaseComponent _returnvalue))
  (bind (_isselected _ispreview) (Class|AIBaseComponent|GetSelection _asaibase_component))
  (if _ispreview
    (Rendering|SetCustomDepthStencilValue _objectmesh 3)
    (elif _isselected
      (Rendering|SetCustomDepthStencilValue _objectmesh 1)
      (else
        (Rendering|SetCustomDepthStencilValue _objectmesh 0)))))

(event Custom|OnCreatingAfter_Event
  (Utilities|FlowControl|Sequence
    (:then_0
      (bind _returnvalue (Class|GameObjectCore|GetComponent (Variables|Default|GetCore) "AI"))
      (bind _asaibase_component (Utilities|Casting|CastToAIBaseComponent _returnvalue))
      (EventDispatchers|AssignOnSelectionChanging _asaibase_component (EventDispatchers|CreateEvent :!event Custom|OnSelectionChanging_Event))
      (EventDispatchers|BindEventtoOnSelectionTouch _asaibase_component (EventDispatchers|CreateEvent :!event Custom|OnSelectionTouch_Event)))
    (:then_1
      (bind _returnvalue_2 (Class|GameObjectCore|GetComponent (Variables|Default|GetCore) "SkillHeaver"))
      (bind _asskill_heaver_base_component (Utilities|Casting|CastToSkillHeaverBaseComponent _returnvalue_2))
      (EventDispatchers|BindEventtoOnSkillIntention _asskill_heaver_base_component (EventDispatchers|CreateEvent :!event Custom|OnSkillIntention)))))

(event Custom|OnSkillIntention
  (params (SkillSlot :type ESkillSlot%20Enum :default "Auto") (Targets :type Array%20of%20Game%20Object%20Core%20Object%20References))
  ;[1 1 1] Attack Animation
  (bind _returnvalue (Class|GameObjectCore|GetComponent (Variables|Default|GetCore) "SkillHeaver"))
  (bind _asskill_heaver_base_component (Utilities|Casting|CastToSkillHeaverBaseComponent _returnvalue))
  (Class|SkillHeaverBaseComponent|CancelSkillCast _asskill_heaver_base_component)
  (Class|SkillHeaverBaseComponent|CastSkill _asskill_heaver_base_component SkillSlot Targets (CallFunction|GetSkillSpawnLocation SkillSlot Targets)))

(event EventBeginPlay
  (|CallParentFunction)
  (bind _returnvalue (Class|GameObjectInterface|GetCore))
  (Variables|Default|SetCore _returnvalue)
  (if (Class|GameObjectCore|GetIsCreated _returnvalue)
    (CallFunction|OnCreatingAfterEvent)
    (else
      (EventDispatchers|AssignOnCreatingAfter _returnvalue (delegate Custom|OnCreatingAfter_Event)))))

(fn ConstructionScript)

(fn GetSkillSpawnLocation
  (params (Slot :type ESkillSlot%20Enum :default "None") (Targets :type Array%20of%20Game%20Object%20Core%20Object%20References))
  (return (Transformation|GetWorldLocation (Variables|Default|GetAttackLocation))))

(fn CheckasTarget
  (bind _returnvalue (Class|GameObjectInterface|GetCore))
  (Utilities|IsValid _returnvalue
    (:Is%20Valid
      (bind _returnvalue_2 (Class|GameObjectCore|GetComponent _returnvalue "Generator"))
      (bind _asgenerator_base_component (Utilities|Casting|CastToGeneratorBaseComponent _returnvalue_2)
        (:then
          (return (> (Class|GeneratorBaseComponent|GetLevel _asgenerator_base_component) 0)))
        (:CastFailed
          (return false))))
    (:Is%20Not%20Valid
      (return false))))

(fn GetTaskProcessLocation
  (params (Worker :type Game%20Object%20Core%20Object%20Reference) (Task :type Game%20Task%20Structure%20%28by%20ref%29))
  (if (Utilities|Enum|Equal(Enum) (.Resource (Utilities|Struct|BreakGameTask Task)) "Self")
    (return (Transformation|GetWorldLocation (Variables|Default|GetWorkPoint)))
    (else
      (return (Transformation|GetWorldLocation (Variables|Default|GetDeliveryPoint))))))