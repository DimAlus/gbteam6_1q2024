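; Skill component that tracks which skills its owner has and gates their use by cooldown.
; AvailableSkills maps skill names to timer handles; TryPrepareSkill accepts a known skill with no active timer and stores it as NextSkill.
; ActivateSkill starts a one-shot CooldownTime timer for NextSkill, whose callback clears the most recently created handle.
; CheckSkillStatus reports whether a skill exists and its remaining cooldown.
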(event Custom|ClearCooldownTimer
  (Utilities|Time|ClearandInvalidateTimerbyHandle (stale Custom|ActivateSkill _returnvalue)))

(event Custom|ActivateSkill
  (bind _returnvalue (Utilities|Time|SetTimerbyEvent (delegate Custom|ClearCooldownTimer) (Variables|Default|GetCooldownTime)))
  (Utilities|Map|Add (Variables|Default|GetAvailableSkills) (Variables|Default|GetNextSkill) _returnvalue))

(event EventBeginPlay)

(event EventTick
  (params (DeltaSeconds :type Float%20%28single-precision%29)))

(fn TryPrepareSkill
  (params (SkillName :type String))
  (bind _availableskills (Variables|Default|GetAvailableSkills))
  (bind (_value _returnvalue) (Utilities|Map|Find _availableskills SkillName))
  (if (Utilities|Map|IsNotEmpty (Variables|Default|GetAvailableSkills))
    (if (and _returnvalue (not (Utilities|Time|IsTimerActivebyHandle _value)))
      (Variables|Default|SetNextSkill SkillName)
      (return true)
      (else
        (return false)))
    (else
      (return false))))

(fn CheckSkillStatus
  (params (SkillName :type String))
  (bind _availableskills (Variables|Default|GetAvailableSkills))
  (bind (_value _returnvalue) (Utilities|Map|Find _availableskills SkillName))
  (if _returnvalue
    (if (Utilities|Time|IsTimerActivebyHandle _value)
      (return true (Utilities|Time|GetTimerRemainingTimebyHandle _value))
      (else
        (return true 0.0)))
    (else
      (return false 0.0))))