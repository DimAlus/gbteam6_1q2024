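; Actor component that tracks its owner's power, putting an AI owner to sleep when it runs out.
; SpiritDrain generator successes add power from a random barter price entry, while a looping timer counts consumption.
; A second timer folds both into a clamped level, firing low, off and full power events.
; Sleep is written to the blackboard; recovery from low power applies a cached state, though GetAIState's blackboard read is unwired.
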(event Custom|ConsumePower
  (Math|Integer|IncrementInt (Variables|PowerUtility|GetConsumedPower)
    (:%20%20
      (Default|CallOnPowerConsumed))))

(event Custom|DeliverPower
  (params (GeneratorName :type String) (Generator :type Generator%20Element%20Info%20Structure%20%28by%20ref%29))
  (if (Utilities|Enum|Equal(Enum) GeneratorName "SpiritDrain")
    (bind _output_get (Variables|PowerUtility|SetDeliveredPower (+ (Variables|PowerUtility|GetDeliveredPower) (.Count (Utilities|Struct|BreakPrice (.OutItem (Utilities|Array|Random (.Price (Utilities|Struct|BreakBarter (.Barter (Utilities|Struct|BreakGeneratorElementInfo Generator)))))))))))
    (Default|CallOnPowerDelivered _output_get)))

(event EventBeginPlay
  (Utilities|FlowControl|Sequence
    (:then_0
      (bind _returnvalue (Class|GameObjectInterface|GetCore(Message) (Components|GetOwner)))
      (Utilities|IsValid _returnvalue
        (:Is%20Valid
          (bind _returnvalue_2 (Class|GameObjectCore|GetComponent _returnvalue "Generator"))
          (bind _asgenerator_base_component (Utilities|Casting|CastToGeneratorBaseComponent _returnvalue_2))
          (EventDispatchers|BindEventtoOnGeneratorSuccess _asgenerator_base_component (delegate Custom|DeliverPower)))))
    (:then_1
      (bind _returnvalue_3 (Utilities|Time|SetTimerbyEvent (delegate Custom|ConsumePower) (Variables|PowerUtility|GetPowerConsumptionRate) true))
      (Variables|Utility|SetGrowPowerNeedsTimerHandle _returnvalue_3))
    (:then_2
      (Utilities|Time|SetTimerbyFunctionName 0 "UpdatePowerLevel" (Variables|PowerUtility|GetUpdatePowerLevelRate) true))))

(event EventTick
  (params (DeltaSeconds :type Float%20%28single-precision%29)))

(fn StartTurnOffTimer)

(fn SetAIState
  (params (AIState :type EAIState%20Enum :default "Default"))
  (bind _returnvalue (Utilities|Name|MakeLiteralName "AIState"))
  (bind _returnvalue_2 (Components|GetOwner))
  (bind _returnvalue_3 (Utilities|Enum|Equal(Enum) AIState "Sleep"))
  (bind _returnvalue_4 (AI|GetAIController _returnvalue_2))
  (bind _blackboard (Variables|/Script/AIModule.AIController|GetBlackboard _returnvalue_4))
  (Utilities|IsValid _returnvalue_4
    (:Is%20Valid
      (AI|Components|Blackboard|SetValueasBool _blackboard (Utilities|Name|MakeLiteralName "IsSleeped") _returnvalue_3)
      (if _returnvalue_3
        (AI|Components|Blackboard|SetValueasEnum _blackboard _returnvalue AIState :!label _label)
        (elif (Utilities|Enum|Equal(Enum) (Utilities|Enum|ByteToEnumEAIState (Class|BlackboardComponent|GetValueasEnum _blackboard _returnvalue)) "Sleep")
          (goto _label))))))

(fn UpdatePowerLevel
  (bind _output_get (Variables|PowerUtility|SetPowerLevel (Math|Integer|Clamp(Integer) (+ (Variables|PowerUtility|GetPowerLevel) (- (Variables|PowerUtility|GetDeliveredPower) (Variables|PowerUtility|GetConsumedPower))) 0 10)))
  (Variables|PowerUtility|SetDeliveredPower 0)
  (Variables|PowerUtility|SetConsumedPower 0)
  (if (>= _output_get (Variables|PowerUtility|GetLowPowerThreshhold))
    (if (Variables|PowerStatus|GetLowPower)
      (Variables|PowerStatus|SetLowPower false)
      (Variables|PowerStatus|SetPowerOff false)
      (CallFunction|SetAIState (Variables|Utility|GetCachedAIState))
      (Default|CallOnFullPower))
    (elif (== (Variables|PowerUtility|GetPowerLevel) 0)
      (if (not (Variables|PowerStatus|GetPowerOff))
        (Variables|PowerStatus|SetPowerOff true)
        (Variables|Utility|SetCachedAIState (Utilities|GetAIState))
        (CallFunction|SetAIState "Sleep")
        (Default|CallOnPowerOff))
      (elif (not (Variables|PowerStatus|GetLowPower))
        (Variables|PowerStatus|SetLowPower true)
        (Default|CallOnLowPower)))))

(fn GetPowerStatus
  (return (Variables|PowerStatus|GetLowPower) (Variables|PowerStatus|GetPowerOff) (Variables|PowerUtility|GetPowerLevel)))