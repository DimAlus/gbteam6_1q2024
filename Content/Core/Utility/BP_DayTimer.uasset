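; BP_DayTimer is an actor that rotates itself to follow the sun position of the day cycle.
; On BeginPlay, the game timer manager starts a looping one-second timer, with time influence off, that reads the sun position from GameStateDefault.
; SunChanging maps that day fraction to a full pitch revolution added to ZeroRotation, keeping roll and yaw fixed.
; A binding to the day-time-changing event exists but is unconnected, so updates rely on polling.
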(event Custom|SunChanging
  (params (DayPercents :type Float%20%28single-precision%29))
  (bind _zerorotation (Variables|Default|GetZeroRotation))
  (Transformation|SetActorRotation (Math|Rotator|MakeRotator (.roll _zerorotation) (+ (.pitch _zerorotation) (* DayPercents 3.6e+02)) (.yaw _zerorotation)) true))

(event Custom|Update_Event
  (bind _asgame_state_default (Utilities|Casting|CastToGameStateDefault (Game|GetGameState)))
  (CallFunction|SunChanging (Class|GameStateDefault|GetSunPosition _asgame_state_default)))

(event EventBeginPlay
  (Class|TimerService|SetTimer (CallFunction|GetGameTimerManager) (delegate Custom|Update_Event) 1.0 true -1.0 false false))

(event Collision|EventActorBeginOverlap
  (params (OtherActor :type Actor%20Object%20Reference)))

(event EventTick
  (params (DeltaSeconds :type Float%20%28single-precision%29)))

(fn ConstructionScript)