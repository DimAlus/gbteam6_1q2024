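; BP_Saver is a utility actor that handles quick save and load through the GameState's save service.
; Save writes the QuickSave slot; Load checks that slot exists, sets it on the GameInstance, then reopens MapLand.
; A disconnected setup chain, unreachable from BeginPlay, would cache GameState, load the chosen slot and bind Save/Load to player pawn events.
; For dev maps, that chain also generates the map from a tilemap and saves it.
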(event Custom|Save
  (Class|SaveService|SaveGame (Class|GameStateDefault|GetSaveService (Variables|Default|GetGameState)) "QuickSave" (Variables|Default|GetIsDevMap)))

(event Custom|Load
  (bind _result (CallFunction|HasQuickSave))
  (if _result
    (bind _asgame_instance_default (Utilities|Casting|CastToGameInstanceDefault (Game|GetGameInstance)))
    (Variables|/Script/GBTeam6.GameInstanceDefault|SetGameSaveSlot _asgame_instance_default "QuickSave")
    (Game|OpenLevel(byName) "MapLand" false)))

(event EventBeginPlay)

(event Collision|EventActorBeginOverlap
  (params (OtherActor :type Actor%20Object%20Reference)))

(event EventTick
  (params (DeltaSeconds :type Float%20%28single-precision%29)))

(fn ConstructionScript)

(fn GenerateMapbyTilemap
  (Class|MappingService|GenerateMap (Class|GameStateDefault|GetMappingService (Variables|Default|GetGameState)) (Variables|/Script/Paper2D.PaperTileMapComponent|GetTileMap (Variables|/Script/Paper2D.PaperTileMapActor|GetRenderComponent (Variables|Default|GettileMap))) (Variables|Default|GetTileLayerName)))

(fn HasQuickSave
  (bind _returnvalue (Class|SaveService|GetSaveNames (Class|GameStateDefault|GetSaveService (Variables|Default|GetGameState)) "MapLand"))
  (for _array_element _returnvalue
    (if (Utilities|Enum|Equal(Enum) _array_element "QuickSave")
      (return true)))
  (return false))