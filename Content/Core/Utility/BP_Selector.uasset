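; BP_Selector is a selection marker actor that shows at a target actor or location for a limited time.
; It starts hidden; Init stores the target and location, shows the marker and restarts the countdown.
; While visible, Tick teleports it to the stored location, refreshed for a valid target by a short downward landscape trace so it follows on the ground.
; When the timer expires, it hides itself rather than being destroyed.
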(event EventBeginPlay
  (Rendering|SetVisibility (Variables|Default|GetDefaultSceneRoot) false true))

(event EventTick
  (params (DeltaSeconds :type Float%20%28single-precision%29))
  (bind _targetactor (Variables|Default|GetTargetActor))
  (bind _returnvalue (Transformation|GetActorLocation _targetactor))
  (if (Variables|Default|GetIsVisible)
    (bind _output_get (Variables|Default|SetCurrentTimer (- (Variables|Default|GetCurrentTimer) DeltaSeconds)))
    (if (< _output_get 0.0)
      (Rendering|SetVisibility (Variables|Default|GetDefaultSceneRoot) false true)
      (Variables|Default|SetIsVisible false)
      (else
        (Utilities|IsValid _targetactor
          (:Is%20Valid
            (bind _outhit (Collision|LineTraceForObjects _returnvalue (- _returnvalue "0.000000,0.000000,100.000000") (Variables|Default|GetLandscapeType) false 0 "None"))
            (Variables|Default|SetTargetLocation (.location _outhit)))
          (:Is%20Not%20Valid
            _))
        (Transformation|SetActorLocation (Variables|Default|GetTargetLocation) false true)))))

(fn ConstructionScript)

(fn Init
  (params (Object :type Actor%20Object%20Reference) (Location :type Vector))
  (Variables|Default|SetTargetActor Object)
  (Variables|Default|SetTargetLocation Location)
  (Variables|Default|SetIsVisible true)
  (Rendering|SetVisibility (Variables|Default|GetDefaultSceneRoot) true true)
  (Variables|Default|SetCurrentTimer (Variables|Default|GetMaxTimer)))