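; Command location point marker actor that shows a Niagara selection effect for a limited duration.
; The construction script creates a dynamic material instance and passes it to the Niagara component as a material variable.
; UpdateMaterial calls Touch to reveal the marker and restart its clock.
; Tick advances time scaled by time dilation, drives the material's Percents parameter as elapsed fraction, and hides the marker once Duration elapses.
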(event Custom|UpdateMaterial
  (CallFunction|Touch))

(event EventBeginPlay)

(event Collision|EventActorBeginOverlap
  (params (OtherActor :type Actor%20Object%20Reference)))

(event EventDestroyed)

(event EventTick
  (params (DeltaSeconds :type Float%20%28single-precision%29))
  (bind _duration (Variables|Default|GetDuration))
  (bind _output_get (Variables|Default|SetCurrentTime (+ (Variables|Default|GetCurrentTime) (* DeltaSeconds (Class|Typing|GetCurrentTimeDilation)))))
  (if (< _output_get _duration)
    (Rendering|Material|SetScalarParameterValue (Variables|Default|GetMat) "Percents" (/ _output_get _duration) :!class /Script/Engine.MaterialInstanceDynamic)
    (elif (not (Variables|Default|GetHidden))
      (CallFunction|Hide))))

(fn ConstructionScript
  (bind _ns_selection (Variables|Default|GetNS_Selection))
  (bind _returnvalue (Rendering|Material|CreateDynamicMaterialInstance "/Game/Core/Utility/CommandLocationPoint/MI_CommandLocationPoint.MI_CommandLocationPoint" "None" "None" :!class /Script/Engine.KismetMaterialLibrary))
  (bind _output_get (Variables|Default|SetMat _returnvalue))
  (Class|NiagaraComponent|SetVariableMaterial _ns_selection "DynamicMaterial" _output_get)
  (Rendering|Material|SetScalarParameterValue (Variables|Default|GetMat) "Percents" 1.0 :!class /Script/Engine.MaterialInstanceDynamic)
  (Transformation|AttachComponentToComponent _ns_selection (Variables|Default|GetDefaultSceneRoot) "None" "KeepRelative" "KeepRelative" "KeepRelative" true))

(fn Touch
  (Variables|Default|SetHidden false)
  (Variables|Default|SetCurrentTime 0.0)
  (Rendering|SetVisibility (Variables|Default|GetDefaultSceneRoot) true true))

(fn Hide
  (Variables|Default|SetHidden true)
  (Rendering|SetVisibility (Variables|Default|GetDefaultSceneRoot) false true))