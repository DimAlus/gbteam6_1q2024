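; Default player pawn for a building strategy game, handling building placement, quick save/load, the game-over panel and debug console commands.
; On BeginPlay it spawns a selector, binds those events and starts a pause-proof timer feeding camera and selected-object locations to MPC_Location.
; Placement uses a timer to move the spawned building under the cursor through the mapping service until installed or cancelled.
; Console events cheat resources, workers, human raids and day time; older selection and command logic is disconnected.
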(event Custom|UpdateCameraLocationMaterialParameter
  (bind _currentselectedcore (Variables|Default|GetCurrentSelectedCore))
  (bind _returnvalue (Class|PlayerPawnDefault|GetCameraLocation))
  (Rendering|Material|SetVectorParameterValue "/Game/MaterialLibrary/Opacity/MPC_Location.MPC_Location" "CameraLocation" (Math|Conversions|ToLinearColor(Vector) _returnvalue) :!class /Script/Engine.KismetMaterialLibrary)
  (Utilities|IsValid _currentselectedcore
    (:Is%20Valid
      (bind _returnvalue_2 (Class|GameObjectCore|GetOwner _currentselectedcore))
      (Rendering|Material|SetVectorParameterValue "/Game/MaterialLibrary/Opacity/MPC_Location.MPC_Location" "Location" (Math|Conversions|ToLinearColor(Vector) (Transformation|GetActorLocation _returnvalue_2)) :!class /Script/Engine.KismetMaterialLibrary))))

(event Custom|OnSave_Event
  ;[1 1 1] SaveLoadEnd game
  (bind _asgame_instance_default (Utilities|Casting|CastToGameInstanceDefault (Game|GetGameInstance)))
  (Class|GameInstanceDefault|SaveGame _asgame_instance_default "QuickSave"))

(event Custom|OnLoad_Event
  ;[1 1 1] SaveLoadEnd game
  (bind _asgame_instance_default (Utilities|Casting|CastToGameInstanceDefault (Game|GetGameInstance)))
  (Class|GameInstanceDefault|LoadGame _asgame_instance_default "QuickSave"))

(event Custom|OnGameOver
  ;[1 1 1] SaveLoadEnd game
  (bind _returnvalue (UserInterface|CreateWidget "/Game/UI/GameOverPanel/WBP_GameOverPanel.WBP_GameOverPanel_C" (Variables|Default|GetPlayerController)))
  (UserInterface|Viewport|AddtoViewport _returnvalue 100))

(event EventTick
  (params (DeltaSeconds :type Float%20%28single-precision%29))
  (|CallParentFunction DeltaSeconds))

(event EventBeginPlay
  (|CallParentFunction)
  (Utilities|FlowControl|Sequence
    (:then_0
      (bind _returnvalue (Game|SpawnActorfromClass "/Game/Core/Utility/BP_Selector.BP_Selector_C" (Math|Transform|MakeTransform "0, 0, 0") "Undefined" "MultiplyWithRoot" 0 0))
      (Variables|Default|SetSelector _returnvalue))
    (:then_1
      (bind _asgame_state_default (Utilities|Casting|CastToGameStateDefault (Game|GetGameState)))
      (EventDispatchers|BindEventtoOnGameOver _asgame_state_default (EventDispatchers|CreateEvent :!event Custom|OnGameOver)))
    (:then_2
      (EventDispatchers|BindEventtoOnQuickSave (EventDispatchers|CreateEvent :!event Custom|OnSave_Event))
      (EventDispatchers|BindEventtoOnQuickLoad (EventDispatchers|CreateEvent :!event Custom|OnLoad_Event)))
    (:then_3
      (Class|TimerService|SetTimer (CallFunction|GetGameTimerManager) (delegate Custom|UpdateCameraLocationMaterialParameter) 0.001 true -1.0 false true))))

(event Input|KeyboardEvents|F12
  (params (Key :type Key%20Structure :default "None"))
  ;[0.1458 0.1458 0.1458] Temp inputs
  (:Pressed
    (Development|ExecuteConsoleCommand "shot showui" (Variables|Default|GetPlayerController))
    (Audio|PlaySound2D "/Engine/VREditor/Sounds/UI/Click_on_Button.Click_on_Button" 1.0 1.0 0.0 0 0)))

(event EventHumanRaids
  (params (isEnable :type Boolean))
  (if isEnable
    (bind _returnvalue (Actor|GetActorOfClass "/Game/Core/Utility/BP_HumanSpawner.BP_HumanSpawner_C"))
    (Utilities|Time|UnpauseTimerbyHandle (Variables|/Game/Core/Utility/BP_HumanSpawner.BP_HumanSpawner_C|GetSpawnTimerHandle _returnvalue))
    (else
      (bind _returnvalue_2 (Actor|GetActorOfClass "/Game/Core/Utility/BP_HumanSpawner.BP_HumanSpawner_C"))
      (Utilities|Time|PauseTimerbyHandle (Variables|/Game/Core/Utility/BP_HumanSpawner.BP_HumanSpawner_C|GetSpawnTimerHandle _returnvalue_2)))))

(event EventCallHumanRaid
  (bind _returnvalue (Actor|GetActorOfClass "/Game/Core/Utility/BP_HumanSpawner.BP_HumanSpawner_C"))
  (Default|SpawnNewWave _returnvalue))

(event EventAddResource
  (params (resource :type EResource%20Enum :default "None") (count :type Integer))
  (bind _currentselectedcore (Variables|Default|GetCurrentSelectedCore))
  (Utilities|IsValid _currentselectedcore
    (:Is%20Valid
      (bind _returnvalue (Class|GameObjectCore|GetComponent _currentselectedcore "Inventory"))
      (bind _asinventory_base_component (Utilities|Casting|CastToInventoryBaseComponent _returnvalue)
        (:then
          (Class|InventoryBaseComponent|ChangeInventory _asinventory_base_component (Utilities|Array|MakeArray (Utilities|Struct|MakePrice resource count 0 "None")) false))
        (:CastFailed
          (bind _asgame_state_default (Utilities|Casting|CastToGameStateDefault (Game|GetGameState) :!label _label))
          (Class|GameStateDefault|AddPlayerResource _asgame_state_default resource count))))
    (:Is%20Not%20Valid
      (goto _label))))

(event EventSetTime
  (params (time :type Float%20%28single-precision%29))
  (bind _asgame_state_default (Utilities|Casting|CastToGameStateDefault (Game|GetGameState)))
  (Class|GameStateDefault|SetCurrentDayTime _asgame_state_default time))

(event EventMakeWorkers
  (params (WorkersAmount :type Integer))
  (for _index (range 1 WorkersAmount)
    (Game|SpawnActorfromClass "/Game/GameObjects/Pawns/Forest/BP_Forestling.BP_Forestling_C" (Math|Conversions|ToTransform(Vector) (Transformation|GetActorLocation)) "Undefined" "MultiplyWithRoot" 0 false 0)))

(event EventGiveWood
  (params (WoodAmount :type Integer))
  (bind _returnvalue (Actor|GetActorOfClass "/Game/GameObjects/Buildings/Forest/PersonHouse/BP_House_Forester.BP_House_Forester_C"))
  (bind _returnvalue_2 (Class|GameObjectInterface|GetCore _returnvalue))
  (bind _returnvalue_3 (Class|GameObjectCore|GetComponent _returnvalue_2 "Inventory"))
  (bind _asinventory_base_component (Utilities|Casting|CastToInventoryBaseComponent _returnvalue_3))
  (Class|InventoryBaseComponent|ChangeInventory _asinventory_base_component (Utilities|Array|MakeArray (Utilities|Struct|MakePrice "Wood" WoodAmount 0 "None")) false))

(event EventGiveSpirit
  (params (SpiritAmount :type Integer))
  (bind _returnvalue (Actor|GetActorOfClass "/Game/GameObjects/Buildings/Forest/PersonHouse/BP_House_Forester.BP_House_Forester_C"))
  (bind _returnvalue_2 (Class|GameObjectInterface|GetCore _returnvalue))
  (bind _returnvalue_3 (Class|GameObjectCore|GetComponent _returnvalue_2 "Inventory"))
  (bind _asinventory_base_component (Utilities|Casting|CastToInventoryBaseComponent _returnvalue_3))
  (Class|InventoryBaseComponent|ChangeInventory _asinventory_base_component (Utilities|Array|MakeArray (Utilities|Struct|MakePrice "Spirit" SpiritAmount 0 "None")) false))

(event EventSetTimeChanging
  (params (isChanged :type Boolean))
  (bind _asgame_state_default (Utilities|Casting|CastToGameStateDefault (Game|GetGameState)))
  (Class|GameStateDefault|SetDayChangingEnable _asgame_state_default isChanged))

(event EventEnableHumanRaids
  (bind _returnvalue (Actor|GetActorOfClass "/Game/Core/Utility/BP_HumanSpawner.BP_HumanSpawner_C"))
  (Utilities|Time|UnpauseTimerbyHandle (Variables|/Game/Core/Utility/BP_HumanSpawner.BP_HumanSpawner_C|GetSpawnTimerHandle _returnvalue)))

(event EventDisableHumanRaids
  (bind _returnvalue (Actor|GetActorOfClass "/Game/Core/Utility/BP_HumanSpawner.BP_HumanSpawner_C"))
  (Utilities|Time|PauseTimerbyHandle (Variables|/Game/Core/Utility/BP_HumanSpawner.BP_HumanSpawner_C|GetSpawnTimerHandle _returnvalue)))

(fn ConstructionScript)

(fn MoveSelectedBuilding
  (if (Variables|Default|GethaveSelectedBuilding)
    (Class|MappingService|SetLocatedCoreLocation (CallFunction|GetMappingService) (.location (Class|PlayerPawnDefault|GetHitUnderMouseCursor "ECC_Visibility")))
    (else
      (Class|TimerService|InvalidateTimer (CallFunction|GetGameTimerManager) (Variables|Default|GetMoveSelectedBuildingTimer)))))

(fn CreateBuilding
  (params (ActorClass :type Actor%20Class%20Reference))
  (if (Variables|Default|GethaveSelectedBuilding)
    (CreatingBuilding|CancelBuilding))
  (bind _returnvalue (Game|SpawnActorfromClass ActorClass (Math|Transform|MakeTransform "0, 0, 0" "0, 0, 0" "1.000000,1.000000,1.000000") "Undefined" "MultiplyWithRoot" 0 0))
  (bind _asgame_object_interface (Utilities|Casting|CastToGameObjectInterface _returnvalue)
    (:then
      (bind _returnvalue_2 (Class|GameObjectInterface|GetCore _asgame_object_interface))
      (Class|MappingService|SetLocatedCore (CallFunction|GetMappingService) _returnvalue_2)
      (Variables|Default|SethaveSelectedBuilding true)
      (bind _returnvalue_3 (Class|TimerService|SetTimer (CallFunction|GetGameTimerManager) (EventDispatchers|CreateEvent :!event MoveSelectedBuilding) 0.01 true -1.0 false false))
      (Variables|Default|SetMoveSelectedBuildingTimer _returnvalue_3))
    (:CastFailed
      (Actor|DestroyActor _returnvalue))))

(fn CancelBuilding
  (bind _mappingservice (CallFunction|GetMappingService))
  (bind _returnvalue (Class|MappingService|GetLocatedCore _mappingservice))
  (Utilities|IsValid _returnvalue
    (:Is%20Valid
      (bind _returnvalue_2 (Class|GameObjectCore|GetOwner _returnvalue))
      (Actor|DestroyActor _returnvalue_2))
    (:Is%20Not%20Valid
      _))
  (Class|MappingService|SetLocatedCore _mappingservice)
  (Variables|Default|SethaveSelectedBuilding false)
  (Class|TimerService|InvalidateTimer (CallFunction|GetGameTimerManager) (Variables|Default|GetMoveSelectedBuildingTimer)))

(fn ApplyBuilding
  (Utilities|FlowControl|Sequence
    (:then_0
      (bind _returnvalue (Class|MappingService|InstallLocatedCore (CallFunction|GetMappingService)))
      (if _returnvalue
        (Variables|Default|SethaveSelectedBuilding false)
        (Class|TimerService|InvalidateTimer (CallFunction|GetGameTimerManager) (Variables|Default|GetMoveSelectedBuildingTimer))))))

(fn UnsetSelectedActor)

(fn SetSelectedActor
  (params (TargetToSelect :type Actor%20Object%20Reference)))

(fn HandleAltSelect)

(fn OnDeadSelectedActor
  (CallFunction|UnsetSelectedActor))