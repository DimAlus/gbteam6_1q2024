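; Forest tower building that a Forestling AI can occupy as a ranged attack position.
; An entrance overlap checks for the Forestling social tag, Combat state and this tower as ObjectOfInterest, then passes through a Gate.
; The Gate sets the RangedAttack blackboard flag, teleports the unit to SpawnPlace and closes, limiting entry to one at a time.
; When an AI leaves InsideVolume, the flag clears and the Gate reopens.
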(event OnComponentBeginOverlap(EntranceVolume)
  (params (OverlappedComponent :type Primitive%20Component%20Object%20Reference) (OtherActor :type Actor%20Object%20Reference) (OtherComp :type Primitive%20Component%20Object%20Reference) (OtherBodyIndex :type Integer) (bFromSweep :type Boolean) (SweepResult :type Hit%20Result%20Structure%20%28by%20ref%29))
  (bind _returnvalue (AI|GetAIController OtherActor))
  (bind _blackboard (Variables|/Script/AIModule.AIController|GetBlackboard _returnvalue))
  (bind _returnvalue_2 (Class|GameObjectInterface|GetCore(Message) OtherActor))
  (Utilities|IsValid _returnvalue_2
    (:Is%20Valid
      (bind _returnvalue_3 (Class|GameObjectCore|GetComponent _returnvalue_2 "Social"))
      (bind _associal_base_component (Utilities|Casting|CastToSocialBaseComponent _returnvalue_3))
      (bind _returnvalue_4 (Class|SocialBaseComponent|GetSocialTags _associal_base_component))
      (if (Utilities|Array|ContainsItem _returnvalue_4 "Forestling")
        (if (== (AI|Components|Blackboard|GetValueasObject _blackboard (Utilities|Name|MakeLiteralName "ObjectOfInterest")) self)
          (if (== (Utilities|Enum|LiteralenumEAIState "Combat") (Class|BlackboardComponent|GetValueasEnum _blackboard (Utilities|Name|MakeLiteralName "AIState")))
            (Utilities|FlowControl|Gate false :!label _label
              (:Exit
                (AI|Components|Blackboard|SetValueasBool _blackboard (Utilities|Name|MakeLiteralName "RangedAttack") true)
                (Transformation|SetActorLocation OtherActor (Transformation|GetWorldLocation (Variables|Default|GetSpawnPlace)) false true)
                (goto _label Close)))))))))

(event OnComponentEndOverlap(InsideVolume)
  (params (OverlappedComponent :type Primitive%20Component%20Object%20Reference) (OtherActor :type Actor%20Object%20Reference) (OtherComp :type Primitive%20Component%20Object%20Reference) (OtherBodyIndex :type Integer))
  (bind _returnvalue (AI|GetAIController OtherActor))
  (Utilities|IsValid _returnvalue
    (:Is%20Valid
      (AI|Components|Blackboard|SetValueasBool (Variables|/Script/AIModule.AIController|GetBlackboard _returnvalue) (Utilities|Name|MakeLiteralName "RangedAttack") false)
      (Utilities|FlowControl|Gate false) ; enters at Open
    )))

(event EventBeginPlay
  (|CallParentFunction))

(fn ConstructionScript)