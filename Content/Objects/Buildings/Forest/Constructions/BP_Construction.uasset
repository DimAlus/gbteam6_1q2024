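; Forest building construction that moves through unplaced, placed and built looks, pulling meshes and materials from DT_GameObjectInitData by ObjectName.
; It listens to its core's Generator component for level changes, with RenewBuilding mapping levels to placed or built visuals.
; TurnAround rotates it 90 degrees only below level 1.
; Health death swaps the mesh for a physics-simulated geometry collection, adds a random impulse, then finalises death after a delay.
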(event Custom|ObjectDestruction
  (bind _returnvalue (Math|Random|RandomFloatinRange 0.0 2e+01))
  (Class|HealthBaseComponent|NotDestroyNow (stale EventBeginPlay _ashealth_base_component))
  (CallFunction|PrepareConstructionDestroy)
  (Utilities|FlowControl|Delay 0.2)
  (Physics|AddImpulse (Variables|Default|GetConstruction_GeometryCollection) (Math|Vector|MakeVector _returnvalue _returnvalue _returnvalue) "None" true)
  (Utilities|FlowControl|Delay 2.0)
  (Class|HealthBaseComponent|PleaseDead (stale EventBeginPlay _ashealth_base_component))
  (Utilities|IsValid (stale EventBeginPlay _ashealth_base_component)
    (:Is%20Valid
      (Class|HealthBaseComponent|PleaseDead (stale EventBeginPlay _ashealth_base_component)))))

(event EventBeginPlay
  (CallFunction|PrepareConstruction)
  (CallFunction|PrepareNotPlaced)
  (Utilities|FlowControl|DelayUntilNextTick)
  (bind _asgenerator_base_component (CallFunction|GetGeneratorComponent))
  (EventDispatchers|BindEventtoOnObjectLevelChanged _asgenerator_base_component (EventDispatchers|CreateEvent :!event RenewBuilding))
  (bind _returnvalue (Class|GameObjectInterface|GetCore))
  (bind _returnvalue_2 (Class|GameObjectCore|GetComponent _returnvalue "Health"))
  (bind _ashealth_base_component (Utilities|Casting|CastToHealthBaseComponent _returnvalue_2))
  (EventDispatchers|BindEventtoOnDeath _ashealth_base_component (delegate Custom|ObjectDestruction)))

(event EventTurnAround
  (bind _asgenerator_base_component (CallFunction|GetGeneratorComponent))
  (if (< (Class|GeneratorBaseComponent|GetLevel _asgenerator_base_component) 1)
    (Transformation|AddWorldRotation (Variables|Default|GetConstruction_GeometryCollection) "0.000000,90.000000,0.000000" false false)))

(fn ConstructionScript)

(fn GetGeneratorComponent
  (bind _asgame_object_interface (Utilities|Casting|CastToGameObjectInterface self)
    (:then
      (bind _returnvalue (Class|GameObjectInterface|GetCore _asgame_object_interface))
      (bind _returnvalue_2 (Class|GameObjectCore|GetComponent _returnvalue "Generator"))
      (bind _asgenerator_base_component (Utilities|Casting|CastToGeneratorBaseComponent _returnvalue_2)
        (:then
          (return _asgenerator_base_component))
        (:CastFailed
          _)))
    (:CastFailed
      _))
  (return 0))

(fn PrepareConstruction
  (Rendering|Material|SetMaterial (Variables|Default|GetObjectMesh) 0 "/Game/MaterialLibrary/Tile/M_TileEnabled.M_TileEnabled"))

(fn PrepareConstructionDestroy
  (bind _objectmesh (Variables|Default|GetObjectMesh))
  (bind _construction_geometrycollection (Variables|Default|GetConstruction_GeometryCollection))
  (Rendering|SetVisibility _objectmesh false false)
  (Collision|SetCollisionEnabled _objectmesh "NoCollision")
  (Rendering|SetVisibility _construction_geometrycollection true false)
  (Physics|SetSimulatePhysics _construction_geometrycollection true)
  (Collision|SetCollisionEnabled _construction_geometrycollection "PhysicsOnly")
  (return))

(fn PrepareNotPlaced
  (bind _objectmesh (Variables|Default|GetObjectMesh))
  (bind _returnvalue (Utilities|GetDataTableRow "/Game/Table/DT_GameObjectInitData.DT_GameObjectInitData" (Variables|Default|GetObjectName))
    (:then
      (Components|StaticMesh|SetStaticMesh _objectmesh (.ConstructionFullMesh (Utilities|Struct|BreakBuildingConstruction (.BuildingConstruction (Utilities|Struct|BreakGameObjectInitializer (.GameObjectInitializer (Utilities|Struct|BreakGameObjectInitData _returnvalue)))))))
      (Rendering|Material|SetMaterial _objectmesh 0 "/Game/MaterialLibrary/Tile/M_TileDefault.M_TileDefault"))))

(fn PreparePlaced
  (bind _objectmesh (Variables|Default|GetObjectMesh))
  (bind _returnvalue (Utilities|GetDataTableRow "/Game/Table/DT_GameObjectInitData.DT_GameObjectInitData" (Variables|Default|GetObjectName))
    (:then
      (Components|StaticMesh|SetStaticMesh _objectmesh (.ConstructionBaseMesh (Utilities|Struct|BreakBuildingConstruction (.BuildingConstruction (Utilities|Struct|BreakGameObjectInitializer (.GameObjectInitializer (Utilities|Struct|BreakGameObjectInitData _returnvalue)))))))
      (Rendering|Material|SetMaterial _objectmesh 0 (.ConstructionMaterial (Utilities|Struct|BreakBuildingConstruction (.BuildingConstruction (Utilities|Struct|BreakGameObjectInitializer (.GameObjectInitializer (Utilities|Struct|BreakGameObjectInitData _returnvalue))))))))))

(fn PrepareBuilded
  (bind _objectmesh (Variables|Default|GetObjectMesh))
  (bind _returnvalue (Utilities|GetDataTableRow "/Game/Table/DT_GameObjectInitData.DT_GameObjectInitData" (Variables|Default|GetObjectName))
    (:then
      (Components|StaticMesh|SetStaticMesh _objectmesh (.ConstructionFullMesh (Utilities|Struct|BreakBuildingConstruction (.BuildingConstruction (Utilities|Struct|BreakGameObjectInitializer (.GameObjectInitializer (Utilities|Struct|BreakGameObjectInitData _returnvalue)))))))
      (Rendering|Material|SetMaterial _objectmesh 0 (.ConstructionFullMaterial (Utilities|Struct|BreakBuildingConstruction (.BuildingConstruction (Utilities|Struct|BreakGameObjectInitializer (.GameObjectInitializer (Utilities|Struct|BreakGameObjectInitData _returnvalue)))))))
      (return))))

(fn RenewBuilding
  (params (CurrentLevel :type Integer))
  (if (== CurrentLevel 1)
    (CallFunction|PreparePlaced)
    (elif (== CurrentLevel 2)
      (CallFunction|PrepareBuilded))))