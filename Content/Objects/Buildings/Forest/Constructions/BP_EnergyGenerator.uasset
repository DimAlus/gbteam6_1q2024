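; BP_EnergyGenerator is a forest building construction for an energy generator, extending a parent construction Blueprint with its visual effects.
; It overrides the parent's state hooks, calling the parent logic first in each.
; The unbuilt state turns off the energy effect component and point light, and the built state turns both on.
; Preparing for destruction removes both components.
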(fn ConstructionScript)

(fn PrepareNotBuilded
  (|CallParentFunction)
  (Components|Activation|SetActive (Variables|Default|GetNS_EnegryGenerator) false true)
  (Rendering|SetVisibility (Variables|Default|GetPointLight) false false))

(fn PrepareBuilded
  (params (GeneratorName :type String) (Generator :type Generator%20Element%20Info%20Structure%20%28by%20ref%29))
  (|CallParentFunction "" Generator)
  (Components|Activation|SetActive (Variables|Default|GetNS_EnegryGenerator) true true)
  (Rendering|SetVisibility (Variables|Default|GetPointLight) true false)
  (return))

(fn PrepareConstructionDestroy
  (|CallParentFunction)
  (Components|DestroyComponent (Variables|Default|GetNS_EnegryGenerator)))