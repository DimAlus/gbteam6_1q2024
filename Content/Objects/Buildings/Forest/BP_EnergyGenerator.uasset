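; Forest energy generator building that shows its powered state and breaks apart when destroyed.
; It pulls Generator and Health components from its Core; the Niagara effect and point light stay off until it is built or the generator reports success.
; On death it holds off destruction, removes the effect, turns on geometry collection physics with a random impulse, then finalizes death after a short delay.
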(event Custom|CustomEvent
  (params (Generator :type Generator%20Structure%20%28by%20ref%29))
  (Components|Activation|SetActive (Variables|Default|GetNS_EnegryGenerator) true true)
  (Rendering|SetVisibility (Variables|Default|GetPointLight) true false))

(event Custom|ObjectDestruction
  (bind _returnvalue (Math|Random|RandomFloatinRange 0.0 2e+01))
  (bind _energygenerator_geometrycollection (Variables|Default|GetEnergyGenerator_GeometryCollection))
  (Class|HealthBaseComponent|NotDestroyNow (stale EventBeginPlay _ashealth_base_component))
  (Components|DestroyComponent (Variables|Default|GetNS_EnegryGenerator))
  (Physics|SetSimulatePhysics _energygenerator_geometrycollection true)
  (Collision|SetCollisionEnabled _energygenerator_geometrycollection "QueryAndPhysics")
  (Physics|AddImpulse (Variables|Default|GetEnergyGenerator_GeometryCollection) (Math|Vector|MakeVector _returnvalue _returnvalue _returnvalue) "None" true)
  (Utilities|FlowControl|Delay 3.0)
  (Class|HealthBaseComponent|PleaseDead (stale EventBeginPlay _ashealth_base_component)))

(event EventBeginPlay
  (bind _energygenerator_geometrycollection (Variables|Default|GetEnergyGenerator_GeometryCollection))
  (Physics|SetSimulatePhysics _energygenerator_geometrycollection false)
  (Collision|SetCollisionEnabled _energygenerator_geometrycollection "NoCollision")
  (Utilities|FlowControl|DelayUntilNextTick)
  (bind _asgenerator_base_component (CallFunction|GetGeneratorComponent))
  (bind _returnvalue (Class|GeneratorBaseComponent|GetIsBuilded _asgenerator_base_component))
  (if _returnvalue
    _
    (else
      (Components|Activation|SetActive (Variables|Default|GetNS_EnegryGenerator) false true)
      (Rendering|SetVisibility (Variables|Default|GetPointLight) false false)))
  (EventDispatchers|BindEventtoOnGeneratorSuccess _asgenerator_base_component (delegate Custom|CustomEvent))
  (bind _returnvalue_2 (Class|GameObjectInterface|GetCore))
  (bind _returnvalue_3 (Class|GameObjectCore|GetComponent _returnvalue_2 "Health"))
  (bind _ashealth_base_component (Utilities|Casting|CastToHealthBaseComponent _returnvalue_3))
  (EventDispatchers|BindEventtoOnDeath _ashealth_base_component (delegate Custom|ObjectDestruction)))

(fn ConstructionScript)

(fn GetGeneratorComponent
  (bind _asgame_object_interface (Utilities|Casting|CastToGameObjectInterface self)
    (:then
      (bind _returnvalue (Class|GameObjectInterface|GetCore _asgame_object_interface))
      (bind _returnvalue_2 (Class|GameObjectCore|GetComponent _returnvalue "Generator"))
      (bind _asgenerator_base_component (Utilities|Casting|CastToGeneratorBaseComponent _returnvalue_2)))
    (:CastFailed
      _))
  (return _asgenerator_base_component))