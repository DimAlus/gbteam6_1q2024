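; Shoremaiden forest house building whose mesh visually grows as its construction progresses.
; Once its core is created, it starts a near-per-frame looping timer that polls the Generator component's PASSIVE thread.
; While that thread runs Construction, power over work size sets a uniform scale and picks the staged mesh and material by the first border above that progress.
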(event Custom|OnCreatingAfter_Event
  (Utilities|Time|SetTimerbyEvent (delegate Custom|CheckGeneration) 0.001 true))

(event Custom|CheckGeneration
  (bind _scales (Variables|Default|GetScales))
  (bind _objectmesh (Variables|Default|GetObjectMesh))
  (bind _returnvalue (Class|GameObjectInterface|GetCore))
  (bind _returnvalue_2 (Class|GameObjectCore|GetComponent _returnvalue "Generator"))
  (bind _asgenerator_default_component (Utilities|Casting|CastToGeneratorDefaultComponent _returnvalue_2))
  (bind (_exists _returnvalue_3) (Class|GeneratorBaseComponent|GetThread _asgenerator_default_component "PASSIVE"))
  (if _exists
    (if (Utilities|Enum|Equal(Enum) (.GeneratorName (Utilities|Struct|BreakGeneratorThread _returnvalue_3)) "Construction")
      (bind (_exists_2 _returnvalue_4) (Class|GeneratorBaseComponent|GetGenerator _asgenerator_default_component (.GeneratorName (Utilities|Struct|BreakGeneratorThread _returnvalue_3))))
      (if _exists_2
        (Transformation|SetWorldScale3D (Variables|Default|GetObjectMesh) (Math|Conversions|ToVector(Float) (Math|Float|Lerp (.x _scales) (.y _scales) (/ (.Power (Utilities|Struct|BreakGeneratorThread _returnvalue_3)) (.worksize (Utilities|Struct|BreakGeneratorElementInfo _returnvalue_4))))))
        (bind (_array_element _array_index) (Utilities|Array|ForEachLoopwithBreak (Variables|Default|GetMeshBorders) :!label _label)
          (:LoopBody
            (if (> _array_element (/ (.Power (Utilities|Struct|BreakGeneratorThread _returnvalue_3)) (.worksize (Utilities|Struct|BreakGeneratorElementInfo _returnvalue_4))))
              (Components|StaticMesh|SetStaticMesh _objectmesh (Utilities|Array|Get(acopy) (Variables|Default|GetMeshes) _array_index))
              (Rendering|Material|SetMaterial _objectmesh 0 (Utilities|Array|Get(acopy) (Variables|Default|GetMaterials) _array_index))
              (goto _label Break))))))))

(event EventBeginPlay
  (|CallParentFunction)
  (bind _returnvalue (Class|GameObjectInterface|GetCore))
  (if (Class|GameObjectCore|GetIsCreated _returnvalue)
    (CallFunction|OnCreatingAfterEvent)
    (else
      (EventDispatchers|AssignOnCreatingAfter _returnvalue (delegate Custom|OnCreatingAfter_Event)))))

(fn ConstructionScript)