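; Demo Forestling pawn that endlessly performs a tennis-style serve with a stone ammo projectile.
; On BeginPlay it loops two montages, a toss followed by an overhead attack, each chained on completion.
; The toss notify spawns a stone at the left hand socket and lobs it upward.
; The attack notify overrides that stone's projectile velocity to launch it along the pawn's forward direction.
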(event EventBeginPlay
  (bind _returnvalue (Transformation|GetActorRotation))
  (bind _mesh (Variables|Character|GetMesh))
  (bind _returnvalue_2 (Math|Vector|GetForwardVector _returnvalue))
  (Animation|Montage|PlayMontage _mesh "/Game/Objects/Pawns/Forest/Forestling/Animation/AM_Forestling_Toss.AM_Forestling_Toss" :!label _label
    (:OnCompleted
      (Animation|Montage|PlayMontage _mesh "/Game/Objects/Pawns/Forest/Forestling/Animation/AM_Forestling_AttackTop.AM_Forestling_AttackTop"
        (:OnCompleted
          (goto _label))
        (:OnNotifyBegin
          (Variables|/Script/Engine.MovementComponent|SetVelocity (Variables|/Game/Objects/ThirdParty/Weapon/Ammo/BP_Ammo_Stone.BP_Ammo_Stone_C|GetProjectileMovement (stale _returnvalue_3)) (* _returnvalue_2 5e+02)))))
    (:OnNotifyBegin
      (bind _returnvalue_3 (Game|SpawnActorfromClass "/Game/Objects/ThirdParty/Weapon/Ammo/BP_Ammo_Stone.BP_Ammo_Stone_C" (Math|Transform|MakeTransform (Transformation|GetSocketLocation (Variables|Character|GetMesh) "LeftHandSocket_Ball")) "Undefined" "MultiplyWithRoot" 0 0))
      (Variables|/Script/Engine.MovementComponent|SetVelocity (Variables|/Game/Objects/ThirdParty/Weapon/Ammo/BP_Ammo_Stone.BP_Ammo_Stone_C|GetProjectileMovement _returnvalue_3) (+ (* _returnvalue_2 5e+01) "0.000000,-30.000000,600.000000")))))

(fn ConstructionScript)