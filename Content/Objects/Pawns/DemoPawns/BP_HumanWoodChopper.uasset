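; Demo human pawn that endlessly plays a tree-chopping animation with an axe in hand.
; On BeginPlay it hides its spotlight, attaches a spawned axe to the right-hand socket and replays the chop montage on completion, randomizing play rate each loop.
; It binds to the core Health component's death event, but the handler is empty; the axe is destroyed with the pawn.
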(event Custom|OnDeath)

(event EventDestroyed
  (Actor|DestroyActor (Variables|Default|GetWeaponActor)))

(event EventBeginPlay
  (|CallParentFunction)
  (Rendering|SetVisibility (Variables|Default|GetSpotLight) false false)
  (bind _returnvalue (Class|GameObjectInterface|GetCore))
  (bind _returnvalue_2 (Class|GameObjectCore|GetComponent _returnvalue "Health"))
  (bind _ashealth_default_component (Utilities|Casting|CastToHealthDefaultComponent _returnvalue_2))
  (EventDispatchers|BindEventtoOnDeath _ashealth_default_component (delegate Custom|OnDeath))
  (bind _returnvalue_3 (Game|SpawnActorfromClass "/Game/Objects/ThirdParty/Weapon/BP_Axe_.BP_Axe__C" (Math|Transform|MakeTransform "0, 0, 0") "Undefined" "MultiplyWithRoot" 0 0))
  (Transformation|AttachComponentToComponent _returnvalue_3 (Variables|Character|GetMesh) "RightHandSocket_Axe" "SnapToTarget" "SnapToTarget" "SnapToTarget" true)
  (Variables|Default|SetWeaponActor _returnvalue_3)
  (Animation|Montage|PlayMontage (Variables|Character|GetMesh) "/Game/Objects/Pawns/Human/ThirdParty/HumanWarrior/Animation/AM_HumanWarrior_TreeChopping.AM_HumanWarrior_TreeChopping" (Math|Random|RandomFloatinRange 0.6 1.5) :!label _label
    (:OnCompleted
      (goto _label))))

(fn ConstructionScript)