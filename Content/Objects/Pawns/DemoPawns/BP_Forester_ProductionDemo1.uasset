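; Production demo Forester pawn that walks to its house's workplace, sits down and endlessly crafts Forestlings.
; BeginPlay finds the ForesterHouse by tag through the GameState social service, moves there with AIMoveTo and switches to the docked AnimBP.
; MakeForestling chains staff montages to reveal a static construct's arms and horns, swaps it for a BP_Forestling with a blink effect, then repeats.
; A hardcoded false branch disables the looping research animation and Niagara effect.
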(event Custom|MakeForestling
  (bind _returnvalue (Transformation|GetActorRotation))
  (bind _returnvalue_2 (Transformation|GetActorLocation))
  (bind _returnvalue_3 (Math|Vector|GetForwardVector _returnvalue))
  (bind (_x _y _z) (Math|Vector|BreakVector _returnvalue_2))
  (bind _returnvalue_4 (* _returnvalue_3 8e+01))
  (bind _returnvalue_5 (- _z 8e+01))
  (bind _returnvalue_6 (Math|Vector|MakeVector _x _y _returnvalue_5))
  (bind _returnvalue_7 (+ _returnvalue_4 _returnvalue_6))
  (Animation|Montage|PlayMontage (Variables|Character|GetMesh) "/Game/Objects/Pawns/Forest/Forester/Animation/AM_Forester_SitGrabStaff_01.AM_Forester_SitGrabStaff_01"
    (:OnCompleted
      (bind _returnvalue_8 (Game|SpawnActorfromClass "/Game/Objects/Pawns/Forest/BP_ForestlingStaticConstruct.BP_ForestlingStaticConstruct_C" (Math|Transform|MakeTransform _returnvalue_7) "Undefined" "MultiplyWithRoot" 0 0))
      (Animation|Montage|PlayMontage (Variables|Character|GetMesh) "/Game/Objects/Pawns/Forest/Forester/Animation/AM_Forester_SitGrabStaff_01.AM_Forester_SitGrabStaff_01"
        (:OnCompleted
          (Rendering|SetVisibility (Variables|/Game/Objects/Pawns/Forest/BP_ForestlingStaticConstruct.BP_ForestlingStaticConstruct_C|GetLeftArm _returnvalue_8) true false)
          (Animation|Montage|PlayMontage (Variables|Character|GetMesh) "/Game/Objects/Pawns/Forest/Forester/Animation/AM_Forester_SitGrabStaff_01.AM_Forester_SitGrabStaff_01"
            (:OnCompleted
              (Rendering|SetVisibility (Variables|/Game/Objects/Pawns/Forest/BP_ForestlingStaticConstruct.BP_ForestlingStaticConstruct_C|GetRightArm _returnvalue_8) true false)
              (Animation|Montage|PlayMontage (Variables|Character|GetMesh) "/Game/Objects/Pawns/Forest/Forester/Animation/AM_Forester_SitGrabStaff_01.AM_Forester_SitGrabStaff_01"
                (:OnCompleted
                  (Rendering|SetVisibility (Variables|/Game/Objects/Pawns/Forest/BP_ForestlingStaticConstruct.BP_ForestlingStaticConstruct_C|GetLeftHorn _returnvalue_8) true false)
                  (Animation|Montage|PlayMontage (Variables|Character|GetMesh) "/Game/Objects/Pawns/Forest/Forester/Animation/AM_Forester_SitGrabStaff_01.AM_Forester_SitGrabStaff_01"
                    (:OnCompleted
                      (Rendering|SetVisibility (Variables|/Game/Objects/Pawns/Forest/BP_ForestlingStaticConstruct.BP_ForestlingStaticConstruct_C|GetRightHorn _returnvalue_8) true false)
                      (bind _returnvalue_9 (Game|SpawnActorfromClass "/Game/Objects/Pawns/BP_Forestling.BP_Forestling_C" (Math|Transform|MakeTransform "0, 0, 0") "Undefined" "MultiplyWithRoot" 0 0))
                      (Transformation|SetActorLocation _returnvalue_9 _returnvalue_7 false false)
                      (Niagara|SpawnSystematLocation "/Game/FX/ThirdParty/BlinkAndDashVFX/VFX_Niagara/NS_Curse_Blink.NS_Curse_Blink" _returnvalue_7)
                      (Actor|DestroyActor _returnvalue_8)
                      (Utilities|FlowControl|Delay 1.0)
                      (CallFunction|MakeForestling))))))))))))

(event EventBeginPlay
  (bind _returnvalue (Transformation|GetActorRotation))
  (bind _returnvalue_2 (Transformation|GetActorLocation))
  (bind _researchniagara (Variables|Default|GetResearchNiagara))
  (bind _returnvalue_3 (Math|Vector|GetForwardVector _returnvalue))
  (bind (_x _y _z) (Math|Vector|BreakVector _returnvalue_2))
  (bind _returnvalue_4 (* _returnvalue_3 8e+01))
  (bind _returnvalue_5 (- _z 8e+01))
  (bind _returnvalue_6 (Math|Vector|MakeVector _x _y _returnvalue_5))
  (bind _returnvalue_7 (+ _returnvalue_4 _returnvalue_6))
  (Transformation|AttachComponentToComponent _researchniagara (Variables|Character|GetMesh) "ForesterResearchSocket" "SnapToTarget" "KeepWorld" "SnapToTarget" false)
  (Components|Activation|SetActive _researchniagara false true)
  (Utilities|FlowControl|Delay 2.0 :!pinned true) ; Timer before start logic
  ;[0.2083 0.2083 0.2083] Move to start position
  (Variables|/Script/Engine.CharacterMovementComponent|SetbOrientRotationToMovement (Variables|Character|GetCharacterMovement) false)
  (Utilities|FlowControl|Delay 0.2)
  (bind _asbp_game_state (Utilities|Casting|CastToBP_GameState (Game|GetGameState)))
  (bind _returnvalue_8 (Class|SocialService|GetObjectsbyTag (Class|GameStateDefault|GetSocialService _asbp_game_state) "ForesterHouse"))
  (if (Utilities|Set|IsNotEmpty _returnvalue_8)
    (bind _result (Utilities|Set|ToArray _returnvalue_8))
    (bind _returnvalue_9 (Class|GameObjectCore|GetOwner (Utilities|Array|Get(acopy) _result)))
    (bind _asbpi_dwelling (Utilities|Casting|CastToBPI_Building _returnvalue_9))
    (bind _workplacetransform (Default|GetWorkPlace _asbpi_dwelling))
    (AI|AIMoveTo self (.Location (Math|Transform|BreakTransform _workplacetransform)) 0 5.0 false
      (:OnSuccess
        (AI|SetFocalPoint (AI|GetAIController self) (+ (.Location (Math|Transform|BreakTransform _workplacetransform)) (* (Math|Vector|GetForwardVector (.Rotation (Math|Transform|BreakTransform _workplacetransform))) 1e+03)))
        ;[1 1 1] Set docked anim BP
        (Class|SkeletalMeshComponent|SetAnimClass (Variables|Character|GetMesh) "/Game/Objects/Pawns/Forest/Forester/Animation/ABP_Forester_Docked.ABP_Forester_Docked_C")
        ;[1 1 1] Sit down
        (Animation|Montage|PlayMontage (Variables|Character|GetMesh) "/Game/Objects/Pawns/Forest/Forester/Animation/AM_Forester_SitToStand_Reverse.AM_Forester_SitToStand_Reverse"
          (:OnCompleted
            _)
          (:OnInterrupted
            _))
        (Utilities|FlowControl|Delay 2.0)
        (if false
          (Components|Activation|SetActive (Variables|Default|GetResearchNiagara) true true)
          (Animation|Montage|PlayMontage (Variables|Character|GetMesh) "/Game/Objects/Pawns/Forest/Forester/Animation/AM_Forester_SitResearch_01.AM_Forester_SitResearch_01" :!label _label
            (:OnCompleted
              (goto _label)))
          (else
            (Animation|Montage|PlayMontage (Variables|Character|GetMesh) "/Game/Objects/Pawns/Forest/Forester/Animation/AM_Forester_SitGrabStaff_01.AM_Forester_SitGrabStaff_01"
              (:OnCompleted
                (bind _returnvalue_10 (Game|SpawnActorfromClass "/Game/Objects/Pawns/Forest/BP_ForestlingStaticConstruct.BP_ForestlingStaticConstruct_C" (Math|Transform|MakeTransform _returnvalue_7) "Undefined" "MultiplyWithRoot" 0 0))
                (Animation|Montage|PlayMontage (Variables|Character|GetMesh) "/Game/Objects/Pawns/Forest/Forester/Animation/AM_Forester_SitGrabStaff_01.AM_Forester_SitGrabStaff_01"
                  (:OnCompleted
                    (Rendering|SetVisibility (Variables|/Game/Objects/Pawns/Forest/BP_ForestlingStaticConstruct.BP_ForestlingStaticConstruct_C|GetLeftArm _returnvalue_10) true false)
                    (Animation|Montage|PlayMontage (Variables|Character|GetMesh) "/Game/Objects/Pawns/Forest/Forester/Animation/AM_Forester_SitGrabStaff_01.AM_Forester_SitGrabStaff_01"
                      (:OnCompleted
                        (Rendering|SetVisibility (Variables|/Game/Objects/Pawns/Forest/BP_ForestlingStaticConstruct.BP_ForestlingStaticConstruct_C|GetRightArm _returnvalue_10) true false)
                        (Animation|Montage|PlayMontage (Variables|Character|GetMesh) "/Game/Objects/Pawns/Forest/Forester/Animation/AM_Forester_SitGrabStaff_01.AM_Forester_SitGrabStaff_01"
                          (:OnCompleted
                            (Rendering|SetVisibility (Variables|/Game/Objects/Pawns/Forest/BP_ForestlingStaticConstruct.BP_ForestlingStaticConstruct_C|GetLeftHorn _returnvalue_10) true false)
                            (Animation|Montage|PlayMontage (Variables|Character|GetMesh) "/Game/Objects/Pawns/Forest/Forester/Animation/AM_Forester_SitGrabStaff_01.AM_Forester_SitGrabStaff_01"
                              (:OnCompleted
                                (Rendering|SetVisibility (Variables|/Game/Objects/Pawns/Forest/BP_ForestlingStaticConstruct.BP_ForestlingStaticConstruct_C|GetRightHorn _returnvalue_10) true false)
                                (bind _returnvalue_11 (Game|SpawnActorfromClass "/Game/Objects/Pawns/BP_Forestling.BP_Forestling_C" (Math|Transform|MakeTransform "0, 0, 0") "Undefined" "MultiplyWithRoot" 0 0))
                                (Transformation|SetActorLocation _returnvalue_11 _returnvalue_7 false false)
                                (Niagara|SpawnSystematLocation "/Game/FX/ThirdParty/BlinkAndDashVFX/VFX_Niagara/NS_Curse_Blink.NS_Curse_Blink" _returnvalue_7)
                                (Actor|DestroyActor _returnvalue_10)
                                (Utilities|FlowControl|Delay 1.0)
                                (CallFunction|MakeForestling)))))))))))))))))

(fn ConstructionScript)