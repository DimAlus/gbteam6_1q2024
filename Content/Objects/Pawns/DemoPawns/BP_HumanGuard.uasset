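; Human guard pawn that carries a sword and can be sent after a target by its AI.
; On BeginPlay it hides its spotlight, binds an empty death handler to the core Health component, and attaches a spawned sword, destroyed along with the pawn.
; ToArms queries the game state's social service for a random EnergyGenerator, falling back to a Forester, and writes its owner to the blackboard's TargetActor.
; Torch-spawning logic exists but is disconnected.
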(event Custom|OnDeath)

(event Custom|ToArms
  (bind _asgame_state_default (Utilities|Casting|CastToGameStateDefault (Game|GetGameState)))
  (bind _returnvalue (Class|SocialService|GetObjectsbyTag (Class|GameStateDefault|GetSocialService _asgame_state_default) "EnergyGenerator"))
  (if (Utilities|Set|IsNotEmpty _returnvalue)
    (bind _result (Utilities|Set|ToArray _returnvalue))
    (bind _returnvalue_2 (Class|GameObjectCore|GetOwner (.OutItem (Utilities|Array|Random _result))))
    (bind _asaic_default (Utilities|Casting|CastToAIC_Default (AI|GetAIController self)))
    (AI|Components|Blackboard|SetValueasObject (Variables|/Script/AIModule.AIController|GetBlackboard _asaic_default) (Utilities|Name|MakeLiteralName "TargetActor") _returnvalue_2)
    (else
      (bind _returnvalue_3 (Class|SocialService|GetObjectsbyTag (Class|GameStateDefault|GetSocialService _asgame_state_default) "Forester"))
      (if (Utilities|Set|IsNotEmpty _returnvalue_3)
        (bind _result_2 (Utilities|Set|ToArray _returnvalue_3))
        (bind _returnvalue_4 (Class|GameObjectCore|GetOwner (.OutItem (Utilities|Array|Random _result_2))))
        (bind _asaic_default_2 (Utilities|Casting|CastToAIC_Default (AI|GetAIController self)))
        (AI|Components|Blackboard|SetValueasObject (Variables|/Script/AIModule.AIController|GetBlackboard _asaic_default_2) (Utilities|Name|MakeLiteralName "TargetActor") _returnvalue_4)))))

(event EventDestroyed
  (Actor|DestroyActor (Variables|Default|GetWeaponActor)))

(event EventBeginPlay
  (|CallParentFunction)
  (Rendering|SetVisibility (Variables|Default|GetSpotLight) false false)
  (bind _returnvalue (Class|GameObjectInterface|GetCore))
  (bind _returnvalue_2 (Class|GameObjectCore|GetComponent _returnvalue "Health"))
  (bind _ashealth_default_component (Utilities|Casting|CastToHealthDefaultComponent _returnvalue_2))
  (EventDispatchers|BindEventtoOnDeath _ashealth_default_component (delegate Custom|OnDeath))
  (Utilities|FlowControl|Sequence
    (:then_0
      (bind _returnvalue_3 (Game|SpawnActorfromClass "/Game/Objects/ThirdParty/Weapon/BP_Sword_.BP_Sword__C" (Math|Transform|MakeTransform "0, 0, 0") "Undefined" "MultiplyWithRoot" 0 0))
      (Transformation|AttachComponentToComponent _returnvalue_3 (Variables|Character|GetMesh) "RightHandSocket_Sword" "SnapToTarget" "SnapToTarget" "SnapToTarget" true)
      (Variables|Default|SetWeaponActor _returnvalue_3))))

(fn ConstructionScript)