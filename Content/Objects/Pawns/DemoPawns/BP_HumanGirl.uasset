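; Demo refugee girl pawn that, after a startup delay, lights up, walks to a Forester-tagged target, prays, then shows a quest panel.
; Accepting switches to the happy AnimBP, slows her and loops roaming between random interest-tag targets with happy montages.
; Declining switches to the scared AnimBP, speeds her up and sends her to a Human-tagged target.
; Targets are the first match from the game state's social tag service.
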(event Custom|OnDeath)

(event Custom|ApplyAcceptBehaviour
  (bind _returnvalue (Math|Random|RandomInteger 2))
  (bind _happyanimmontages (Variables|Default|GetHappyAnimMontages))
  (bind _mesh (Variables|Character|GetMesh))
  (bind _mesh_2 (Variables|Character|GetMesh))
  (bind _charactermovement (Variables|Character|GetCharacterMovement))
  (bind _output (Utilities|Array|Get(acopy) _happyanimmontages _returnvalue))
  (Components|Animation|SetAnimationMode _mesh_2 "AnimationBlueprint" true)
  (Class|SkeletalMeshComponent|SetAnimClass _mesh_2 "/Game/Objects/Pawns/Human/ThirdParty/HumanGirl/Animation/ABP_HumanGirl_Happy.ABP_HumanGirl_Happy_C")
  (Variables|/Script/Engine.CharacterMovementComponent|SetMaxWalkSpeed _charactermovement (+ (Variables|/Script/Engine.CharacterMovementComponent|GetMaxWalkSpeed _charactermovement) -1e+02))
  (bind _returnvalue_2 (CallFunction|GetMovementTargetbyTag (.OutItem (Utilities|Array|Random (Variables|Default|GetInterestedTags)))))
  (Utilities|IsValid _returnvalue_2
    (:Is%20Valid
      (AI|AIMoveTo self "0, 0, 0" _returnvalue_2 1e+02 false
        (:OnSuccess
          _)
        (:OnFail
          _))
      (if (Math|Random|RandomBool)
        (Animation|Montage|PlayMontage _mesh _output
          (:OnCompleted
            _)
          (:OnInterrupted
            _)))
      (Animation|Montage|PlayMontage _mesh _output
        (:OnCompleted
          _)
        (:OnInterrupted
          _))
      (if (Math|Random|RandomBool)
        (CallFunction|DanceAgain)
        (else
          (CallFunction|HappyRoaming))))
    (:Is%20Not%20Valid
      (CallFunction|HappyRoaming))))

(event Custom|ApplyDeclineBehaviour
  (bind _charactermovement (Variables|Character|GetCharacterMovement))
  (bind _mesh (Variables|Character|GetMesh))
  (Components|Animation|SetAnimationMode _mesh "AnimationBlueprint" true)
  (Class|SkeletalMeshComponent|SetAnimClass _mesh "/Game/Objects/Pawns/Human/ThirdParty/HumanGirl/Animation/ABP_HumanGirl_Scared.ABP_HumanGirl_Scared_C")
  (Variables|/Script/Engine.CharacterMovementComponent|SetMaxWalkSpeed _charactermovement (+ (Variables|/Script/Engine.CharacterMovementComponent|GetMaxWalkSpeed _charactermovement) 1e+02))
  (bind _returnvalue (CallFunction|GetMovementTargetbyTag "Human"))
  (AI|AIMoveTo self "0, 0, 0" _returnvalue 1e+02 false))

(event Custom|HappyRoaming
  (bind _returnvalue (Math|Random|RandomInteger 2))
  (bind _happyanimmontages (Variables|Default|GetHappyAnimMontages))
  (bind _mesh (Variables|Character|GetMesh))
  (bind _output (Utilities|Array|Get(acopy) _happyanimmontages _returnvalue))
  (bind _returnvalue_2 (CallFunction|GetMovementTargetbyTag (.OutItem (Utilities|Array|Random (Variables|Default|GetInterestedTags)))))
  (Utilities|IsValid _returnvalue_2
    (:Is%20Valid
      (AI|AIMoveTo self "0, 0, 0" _returnvalue_2 1e+02 false
        (:OnSuccess
          _)
        (:OnFail
          _))
      (if (Math|Random|RandomBool)
        (Animation|Montage|PlayMontage _mesh _output
          (:OnCompleted
            _)
          (:OnInterrupted
            _)))
      (Animation|Montage|PlayMontage _mesh _output
        (:OnCompleted
          _)
        (:OnInterrupted
          _))
      (if (Math|Random|RandomBool)
        (CallFunction|DanceAgain)
        (else
          (CallFunction|HappyRoaming))))
    (:Is%20Not%20Valid
      (CallFunction|HappyRoaming))))

(event Custom|DanceAgain
  (bind _returnvalue (Math|Random|RandomInteger 2))
  (bind _happyanimmontages (Variables|Default|GetHappyAnimMontages))
  (bind _mesh (Variables|Character|GetMesh))
  (bind _output (Utilities|Array|Get(acopy) _happyanimmontages _returnvalue))
  (if (Math|Random|RandomBool)
    (Animation|Montage|PlayMontage _mesh _output
      (:OnCompleted
        _)
      (:OnInterrupted
        _)))
  (Animation|Montage|PlayMontage _mesh _output
    (:OnCompleted
      _)
    (:OnInterrupted
      _))
  (if (Math|Random|RandomBool)
    (CallFunction|DanceAgain)
    (else
      (CallFunction|HappyRoaming))))

(event EventDestroyed
  (Actor|DestroyActor (Variables|Default|GetWeaponActor)))

(event EventBeginPlay
  (|CallParentFunction)
  (Utilities|FlowControl|Delay 6e+01 :!pinned true) ; Time before start quest
  (Rendering|SetVisibility (Variables|Default|GetSpotLight) true false)
  (bind _returnvalue (Class|GameObjectInterface|GetCore))
  (bind _returnvalue_2 (Class|GameObjectCore|GetComponent _returnvalue "Health"))
  (bind _ashealth_base_component (Utilities|Casting|CastToHealthBaseComponent _returnvalue_2))
  (EventDispatchers|BindEventtoOnDeath _ashealth_base_component (delegate Custom|OnDeath))
  (bind _returnvalue_3 (CallFunction|GetMovementTargetbyTag "Forester"))
  (AI|AIMoveTo self "0, 0, 0" _returnvalue_3 1e+02 false
    (:OnSuccess
      (Animation|Montage|PlayMontage (Variables|Character|GetMesh) "/Game/Objects/Pawns/Human/ThirdParty/HumanGirl/Animation/AM_HumanGirl_Praying.AM_HumanGirl_Praying" (Math|Random|RandomFloatinRange 0.6 1.5)
        (:OnCompleted
          (bind _returnvalue_4 (UserInterface|CreateWidget "/Game/UI/Demo/WBP_QuestPanel_GirlRefugee.WBP_QuestPanel_GirlRefugee_C" (Game|GetPlayerController 0)))
          (UserInterface|Viewport|AddtoViewport _returnvalue_4 0)
          (EventDispatchers|BindEventtoOnAccept _returnvalue_4 (delegate Custom|ApplyAcceptBehaviour))
          (EventDispatchers|BindEventtoOnDecline _returnvalue_4 (delegate Custom|ApplyDeclineBehaviour)))))))

(fn ConstructionScript)

(fn GetMovementTargetbyTag
  (params (SocialTag :type ESocialTag%20Enum :default "None"))
  (bind _asgame_state_default (Utilities|Casting|CastToGameStateDefault (Game|GetGameState))
    (:then
      (bind _returnvalue (Class|SocialService|GetObjectsbyTag (Class|GameStateDefault|GetSocialService _asgame_state_default) SocialTag))
      (if (Utilities|Set|IsNotEmpty _returnvalue)
        (bind _result (Utilities|Set|ToArray _returnvalue))
        (bind _returnvalue_2 (Class|GameObjectCore|GetOwner (Utilities|Array|Get(acopy) _result)))
        (return _returnvalue_2)))
    (:CastFailed
      (return _returnvalue_2))))