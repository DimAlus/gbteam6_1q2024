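; Demo Meadowman pawn that plays a scripted happiness animation sequence shortly after BeginPlay.
; It spawns a bottle, attaches it to the left-hand socket and plays a drink montage, destroying the bottle when that completes.
; Chained montage completion callbacks then play a victory montage and, after a short pause, a disappointed montage that repeats once.
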(event EventBeginPlay
  (Utilities|FlowControl|Delay 2.0)
  (bind _returnvalue (Game|SpawnActorfromClass "/Game/Objects/ThirdParty/Props/Potions/BP_Bottle.BP_Bottle_C" (Math|Transform|MakeTransform (Transformation|GetSocketLocation (Variables|Character|GetMesh) "LeftHandSocket_Bottle")) "Undefined" "MultiplyWithRoot" 0 0))
  (Transformation|AttachComponentToComponent _returnvalue (Variables|Character|GetMesh) "LeftHandSocket_Bottle" "SnapToTarget" "SnapToTarget" "SnapToTarget" true)
  (Animation|Montage|PlayMontage (Variables|Character|GetMesh) "/Game/Objects/Pawns/Forest/Meadowman/Animation/AM_Meadowman_Drink.AM_Meadowman_Drink"
    (:OnCompleted
      (Actor|DestroyActor _returnvalue)
      (Animation|Montage|PlayMontage (Variables|Character|GetMesh) "/Game/Objects/Pawns/Forest/Meadowman/Animation/AM_Meadowman_Victory.AM_Meadowman_Victory"
        (:OnCompleted
          (Utilities|FlowControl|Delay 1.0)
          (Animation|Montage|PlayMontage (Variables|Character|GetMesh) "/Game/Objects/Pawns/Forest/Meadowman/Animation/AM_Meadowman_Disappointed.AM_Meadowman_Disappointed"
            (:OnCompleted
              (Animation|Montage|PlayMontage (Variables|Character|GetMesh) "/Game/Objects/Pawns/Forest/Meadowman/Animation/AM_Meadowman_Disappointed.AM_Meadowman_Disappointed"))))))))

(fn ConstructionScript)