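; Shoremaiden pawn, an AI healer who sleeps until the raiders' cage is destroyed, then wakes and joins the Friendly team.
; Her skill moves into range if needed, spends Spirit, and heals the target on a cast montage notify.
; At workplaces, looping timers drive spirit-generation cast effects until the blackboard WorkPlace clears.
; Taking damage temporarily hides her and turns her Neutral as optional immortality.
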(event Custom|WakeUp
  (params (DestroyedActor :type Actor%20Object%20Reference))
  (AI|Components|Blackboard|SetValueasEnum (Variables|/Script/AIModule.AIController|GetBlackboard (AI|GetAIController self)) (Utilities|Name|MakeLiteralName "AIState") (Utilities|Enum|LiteralenumEAIState "Default"))
  (bind _returnvalue (Class|GameObjectInterface|GetCore))
  (bind _returnvalue_2 (Class|GameObjectCore|GetComponent _returnvalue "Social"))
  (bind _associal_base_component (Utilities|Casting|CastToSocialBaseComponent _returnvalue_2))
  (Class|SocialBaseComponent|SetSocialTeam _associal_base_component "Friendly"))

(event Custom|HealDamage
  (params (DamagedActor :type Actor%20Object%20Reference) (Damage :type Float%20%28single-precision%29) (DamageType :type Damage%20Type%20Object%20Reference) (InstigatedBy :type Controller%20Object%20Reference) (DamageCauser :type Actor%20Object%20Reference))
  (bind _returnvalue (Class|GameObjectInterface|GetCore(Message) self))
  (bind _returnvalue_2 (Class|GameObjectCore|GetComponent _returnvalue "Health"))
  (bind _ashealth_default_component (Utilities|Casting|CastToHealthDefaultComponent _returnvalue_2))
  (Class|HealthDefaultComponent|ChangeHealth _ashealth_default_component Damage))

(event Custom|CheckIsWorking
  (Utilities|IsValid (AI|Components|Blackboard|GetValueasObject (Variables|/Script/AIModule.AIController|GetBlackboard (AI|GetAIController self)) (Utilities|Name|MakeLiteralName "WorkPlace"))
    (:Is%20Not%20Valid
      (Animation|StopAnimMontage "/Game/Objects/Pawns/Forest/Shoremaiden/Animation/AM_Shoremaiden_Cast_AOE.AM_Shoremaiden_Cast_AOE")
      (Utilities|Time|ClearandInvalidateTimerbyHandle (stale EventMakeResource _returnvalue))
      (Utilities|Time|ClearandInvalidateTimerbyHandle (stale EventMakeResource _returnvalue_2))
      (CallFunction|ResetMakeResource))))

(event Custom|ResetMakeResource
  (Utilities|FlowControl|DoOnce false) ; enters at Reset
)

(event Custom|EmergencyHideOnDamage
  (params (DamagedActor :type Actor%20Object%20Reference) (Damage :type Float%20%28single-precision%29) (DamageType :type Damage%20Type%20Object%20Reference) (InstigatedBy :type Controller%20Object%20Reference) (DamageCauser :type Actor%20Object%20Reference))
  (bind _returnvalue (Transformation|GetActorLocation))
  (bind _returnvalue_2 (Class|GameObjectInterface|GetCore))
  (Utilities|IsValid _returnvalue_2
    (:Is%20Valid
      (bind _returnvalue_3 (Class|GameObjectCore|GetComponent _returnvalue_2 "Social"))
      (bind _associal_base_component (Utilities|Casting|CastToSocialBaseComponent _returnvalue_3))
      (Class|SocialBaseComponent|SetSocialTeam _associal_base_component "Neutral")
      (Rendering|SetActorHiddenInGame true)
      (Niagara|SpawnSystematLocation "/Game/FX/NS_Nature_Cast.NS_Nature_Cast" _returnvalue)
      (Utilities|FlowControl|Delay 5.0)
      (Niagara|SpawnSystematLocation "/Game/FX/NS_Nature_Heal_Impact.NS_Nature_Heal_Impact" _returnvalue)
      (Rendering|SetActorHiddenInGame false)
      (Class|SocialBaseComponent|SetSocialTeam _associal_base_component "Friendly"))))

(event Custom|DoCast
  (Animation|Montage|PlayMontage (Variables|Character|GetMesh) "/Game/Objects/Pawns/Forest/Shoremaiden/Animation/AM_Shoremaiden_Cast_AOE.AM_Shoremaiden_Cast_AOE"
    (:OnInterrupted
      _)
    (:OnNotifyBegin
      _))
  (CallFunction|SpawnSpriritGenerationFX (stale EventMakeResource _innardpoint)))

(event EventBeginPlay
  (|CallParentFunction)
  (AI|Components|Blackboard|SetValueasEnum (Variables|/Script/AIModule.AIController|GetBlackboard (AI|GetAIController self)) (Utilities|Name|MakeLiteralName "AIState") (Utilities|Enum|LiteralenumEAIState "Sleep"))
  (Utilities|FlowControl|Delay 1.0)
  (bind _returnvalue (Actor|GetActorOfClass "/Game/Enviroment/Human/Raiders/BP_Raiders_Cage.BP_Raiders_Cage_C"))
  (Game|BindEventtoOnDestroyed _returnvalue (delegate Custom|WakeUp))
  (EventDispatchers|BindEventtoOnTakeAnyDamage (delegate Custom|EmergencyHideOnDamage)) ; Optional immortality
)

(event EventUseSkill
  (params (SkillTarget :type Actor%20Object%20Reference))
  (Class|BPIAIController|SetAIState(Message) (AI|GetAIController self) "Sleep")
  (if (<= (Math|Vector|Distance(Vector) (Transformation|GetActorLocation) (Transformation|GetActorLocation SkillTarget)) 5e+02)
    (Variables|Default|SetCuurntGoToSkill false :!label _label)
    (CallFunction|ShowSkillArea false)
    (bind _canuseskill (CallFunction|TrySkillPricePay))
    (if _canuseskill
      (AI|SetFocus (AI|GetAIController self) SkillTarget)
      (Variables|/Script/Engine.CharacterMovementComponent|SetbOrientRotationToMovement (Variables|Character|GetCharacterMovement) false)
      (Animation|Montage|PlayMontage (Variables|Character|GetMesh) "/Game/Objects/Pawns/Forest/Shoremaiden/Animation/AM_Shoremaiden_Cast.AM_Shoremaiden_Cast"
        (:OnInterrupted
          _)
        (:OnNotifyBegin
          (CallFunction|HealTarget SkillTarget 4e+01)
          (Niagara|SpawnSystemAttached "/Game/FX/NS_Nature_Cast.NS_Nature_Cast" (Variables|Character|GetMesh) "RightHandSocket" "0, 0, 0" "0, 0, 0" "KeepRelativeOffset" true)
          (Niagara|SpawnSystematLocation "/Game/FX/NS_Nature_Heal_Impact.NS_Nature_Heal_Impact" (Transformation|GetActorLocation SkillTarget))
          (|CallParentFunction SkillTarget))))
    (else
      (CallFunction|ShowSkillArea true)
      (Variables|Default|SetCuurntGoToSkill true)
      (AI|AIMoveTo self "0, 0, 0" SkillTarget 5e+02 true
        (:OnSuccess
          (goto _label))
        (:OnFail
          (Variables|Default|SetCuurntGoToSkill false)
          (CallFunction|ShowSkillArea false)))))
  (AI|ClearFocus (AI|GetAIController self))
  (Variables|/Script/Engine.CharacterMovementComponent|SetbOrientRotationToMovement (Variables|Character|GetCharacterMovement) true)
  (Class|BPIAIController|SetAIStateasOriginal(Message) (AI|GetAIController self)))

(event EventFinishWorkatPlace
  (Variables|/Script/Engine.CharacterMovementComponent|SetbOrientRotationToMovement (Variables|Character|GetCharacterMovement) true))

(event EventPreparetoWorkinPlace
  (Variables|/Script/Engine.CharacterMovementComponent|SetbOrientRotationToMovement (Variables|Character|GetCharacterMovement) false)
  (Utilities|FlowControl|DelayUntilNextTick)
  (Default|CallOnPreparedtoWork))

(event EventMakeResource
  (params (WorkTime :type Float%20%28double-precision%29) (WorkPlaceObject :type Object%20Object%20Reference))
  (Utilities|FlowControl|DoOnce false
    (:Completed
      (bind (_isvalid _innardpoint) (Class|BPIBuilding|GetInnardPoint(Message) WorkPlaceObject))
      (if _isvalid
        (bind _returnvalue (Utilities|Time|SetTimerbyEvent (delegate Custom|DoCast) 1.0 true)))
      (bind _returnvalue_2 (Utilities|Time|SetTimerbyEvent (delegate Custom|CheckIsWorking) 0.1 true)))))

(fn ConstructionScript)

(fn SpawnSpriritGenerationFX
  (params (GenerationPoint :type Transform))
  (bind (_location _rotation _scale) (Math|Transform|BreakTransform GenerationPoint))
  (Niagara|SpawnSystematLocation "/Game/FX/NS_Shoremaiden_GenrateSpirit.NS_Shoremaiden_GenrateSpirit" (Transformation|GetSocketLocation (Variables|Character|GetMesh) "CastSocket") "0, 0, 0" "1.000000,1.000000,1.000000" true true "AutoRelease")
  (bind _returnvalue (Niagara|SpawnSystematLocation "/Game/FX/NS_EnegryGenerator_BIG.NS_EnegryGenerator_BIG" _location _rotation _scale true true "AutoRelease"))
  (return _returnvalue))

(fn ShowSkillArea
  (params (IsShowed :type Boolean))
  (Rendering|SetVisibility (Variables|Default|GetHealZone) (or IsShowed (Variables|Default|GetCuurntGoToSkill)) false))

(fn TrySkillPricePay
  (bind _asgame_state_default (Utilities|Casting|CastToGameStateDefault (Game|GetGameState)))
  (bind _returnvalue (Class|GameStateDefault|PopPlayerResource _asgame_state_default "Spirit" 20))
  (if _returnvalue
    (bind _asgame_state_default_2 (Utilities|Casting|CastToGameStateDefault (Game|GetGameState)))
    (bind _returnvalue_2 (Class|GameObjectInterface|GetCore))
    (Default|CallOnShowInventoryChanging _asgame_state_default_2 _returnvalue_2 (Utilities|Struct|MakePrice "Spirit" -20 0 "None"))
    (else
      (bind _asbp_player_controller (Utilities|Casting|CastToBP_PlayerController (Game|GetPlayerController 0))
        (:then
          (Default|ShowSkillConstraintWarning (Variables|/Game/Core/Player/BP_PlayerController.BP_PlayerController_C|GetWindow _asbp_player_controller)))
        (:CastFailed
          _))))
  (return _returnvalue))

(fn HealTargetPercent
  (params (Target :type Object%20Object%20Reference) (HealPercentage :type Float%20%28double-precision%29))
  (bind _returnvalue (Class|GameObjectInterface|GetCore(Message) Target))
  (bind _output_get (LocalVariables|SetTargetCore _returnvalue))
  (bind _returnvalue_2 (Class|GameObjectCore|GetComponent _output_get "Health"))
  (bind _ashealth_default_component (Utilities|Casting|CastToHealthDefaultComponent _returnvalue_2)
    (:then
      (bind _returnvalue_3 (Class|HealthBaseComponent|GetMaxHealth _ashealth_default_component))
      (Class|HealthDefaultComponent|ChangeHealth _ashealth_default_component (* _returnvalue_3 HealPercentage))
      (bind _asgame_state_default (Utilities|Casting|CastToGameStateDefault (Game|GetGameState))
        (:then
          (Default|CallOnShowInventoryChanging _asgame_state_default (LocalVariables|GetTargetCore) (Utilities|Struct|MakePrice "Heal" (Math|Float|Truncate (* _returnvalue_3 HealPercentage)) 0 "None")))
        (:CastFailed
          _))
      (return))
    (:CastFailed
      (return))))

(fn HealTarget
  (params (Target :type Object%20Object%20Reference) (HealAmount :type Float%20%28double-precision%29))
  (bind _returnvalue (Class|GameObjectInterface|GetCore(Message) Target))
  (bind _output_get (LocalVariables|SetTargetCore _returnvalue))
  (bind _returnvalue_2 (Class|GameObjectCore|GetComponent _output_get "Health"))
  (bind _ashealth_default_component (Utilities|Casting|CastToHealthDefaultComponent _returnvalue_2)
    (:then
      (Class|HealthDefaultComponent|ChangeHealth _ashealth_default_component HealAmount)
      (bind _asgame_state_default (Utilities|Casting|CastToGameStateDefault (Game|GetGameState))
        (:then
          (Default|CallOnShowInventoryChanging _asgame_state_default (LocalVariables|GetTargetCore) (Utilities|Struct|MakePrice "Heal" (Math|Float|Truncate HealAmount) 0 "None")))
        (:CastFailed
          _))
      (return))
    (:CastFailed
      (return))))