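; BP_Human_1 is a human pawn that carries an axe and drops it on death.
; On BeginPlay it binds to the death event of the Health component fetched from its Core, then spawns a BP_Axe and snaps it to the right-hand mesh socket.
; On death the weapon detaches and its static mesh simulates physics.
; When the pawn is destroyed, any remaining weapon actor is destroyed with it.
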(event Custom|OnDeath
  (bind _weaponactor (Variables|Default|GetWeaponActor))
  (Transformation|DetachFromActor _weaponactor "KeepWorld" "KeepWorld" "KeepWorld")
  (bind _asbp_weapon_base (Utilities|Casting|CastToBP_Weapon_Base _weaponactor))
  (Physics|SetSimulatePhysics (Variables|/Game/Objects/Other/BP_Weapon_Base.BP_Weapon_Base_C|GetWeaponStaticMesh _asbp_weapon_base) true))

(event EventDestroyed
  (bind _weaponactor (Variables|Default|GetWeaponActor)
    (:then
      (Actor|DestroyActor _weaponactor))
    (:else)))

(event EventBeginPlay
  (|CallParentFunction)
  (Utilities|FlowControl|Sequence
    (:then_1
      (bind _returnvalue (Class|GameObjectInterface|GetCore))
      (bind _returnvalue_2 (Class|GameObjectCore|GetComponent _returnvalue "Health"))
      (bind _ashealth_default_component (Utilities|Casting|CastToHealthDefaultComponent _returnvalue_2))
      (EventDispatchers|BindEventtoOnDeath _ashealth_default_component (delegate Custom|OnDeath))
      (bind _returnvalue_3 (Game|SpawnActorfromClass "/Game/Objects/Other/Human/BP_Axe.BP_Axe_C" (Math|Transform|MakeTransform "0, 0, 0") "Undefined" "MultiplyWithRoot" 0 0))
      (Transformation|AttachComponentToComponent _returnvalue_3 (Variables|Character|GetMesh) "RightHandSocket_Axe" "SnapToTarget" "SnapToTarget" "SnapToTarget" true)
      (Variables|Default|SetWeaponActor _returnvalue_3))))

(fn ConstructionScript)