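; Forestling pawn that works and fights, pulling tasks from the game's task manager.
; On BeginPlay it removes a static Forestling construct, teleports to the Forester house spawn and binds Health death to a delayed PleaseDead.
; It equips a socketed club for randomized melee montages and repeats a swing montage for work.
; Ranged attacks use montage notifies to toss a stone, then strike it into a homing projectile that damages on overlap.
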(event Custom|OnDeath
  ;[1 1 1] OnDeath
  (Utilities|FlowControl|Delay 1e+01)
  (Class|HealthBaseComponent|PleaseDead (stale EventBeginPlay _ashealth_default_component)))

(event Custom|ClearTask)

(event Custom|DealRangedDamage
  (params (OverlappedActor :type Actor%20Object%20Reference) (OtherActor :type Actor%20Object%20Reference))
  (if (== OtherActor (stale EventAttackRanged TargetActor))
    (bind _asactor (Utilities|Casting|CastToActor (AI|Components|Blackboard|GetValueasObject (Variables|/Script/AIModule.AIController|GetBlackboard (AI|GetAIController self)) (Utilities|Name|MakeLiteralName "ObjectOfInterest"))))
    (Game|Damage|ApplyDamage OtherActor (Variables|Default|GetDamage) 0 _asactor)))

(event Custom|UnequipWeapon
  ;[1 1 1] WeaponTasks
  (Utilities|IsValid (Variables|Default|GetWeaponActor)
    (:Is%20Valid
      (Actor|DestroyActor (Variables|Default|GetWeaponActor)))))

(event Custom|EquipWeapon
  ;[1 1 1] WeaponTasks
  (Utilities|IsValid (Variables|Default|GetWeaponActor)
    (:Is%20Not%20Valid
      (bind _returnvalue (Game|SpawnActorfromClass "/Game/Objects/ThirdParty/Weapon/BP_Club_.BP_Club__C" (Math|Transform|MakeTransform "0, 0, 0") "Undefined" "MultiplyWithRoot" 0 0))
      (bind _output_get (Variables|Default|SetWeaponActor _returnvalue))
      (Transformation|AttachComponentToComponent _output_get (Variables|Character|GetMesh) (Utilities|Name|MakeLiteralName "RightHandSocket") "SnapToTarget" "SnapToTarget" "SnapToTarget" true))))

(event EventAttackRanged
  (params (TargetActor :type Actor%20Object%20Reference))
  (bind _returnvalue (Transformation|GetActorRotation))
  (bind _mesh (Variables|Character|GetMesh))
  (bind _returnvalue_2 (Math|Vector|GetForwardVector _returnvalue))
  (Animation|Montage|PlayMontage _mesh "/Game/Objects/Pawns/Forest/Forestling/Animation/AM_Forestling_Toss.AM_Forestling_Toss"
    (:OnCompleted
      (Animation|Montage|PlayMontage _mesh "/Game/Objects/Pawns/Forest/Forestling/Animation/AM_Forestling_AttackTop.AM_Forestling_AttackTop"
        (:OnNotifyBegin
          (Variables|/Script/Engine.MovementComponent|SetVelocity (Variables|/Game/Objects/ThirdParty/Weapon/Ammo/BP_Ammo_Stone.BP_Ammo_Stone_C|GetProjectileMovement (stale _returnvalue_3)) (* _returnvalue_2 5e+02))
          (Audio|PlaySoundatLocation "/Game/Sound/Wawe/Environment/Stone_Kick/stone_kick_-_2.stone_kick_-_2" (Transformation|GetActorLocation (stale _returnvalue_3)) "0, 0, 0" 1.0 1.0 0.0 0 0 0 0)
          (Components|Activation|SetActive (Variables|/Game/Objects/ThirdParty/Weapon/Ammo/BP_Ammo_Stone.BP_Ammo_Stone_C|GetNS_ProjectileTrail (stale _returnvalue_3)) true true)
          (Utilities|IsValid TargetActor
            (:Is%20Valid
              (Variables|/Script/Engine.ProjectileMovementComponent|SetHomingTargetComponent (Variables|/Game/Objects/ThirdParty/Weapon/Ammo/BP_Ammo_Stone.BP_Ammo_Stone_C|GetProjectileMovement (stale _returnvalue_3)) (Variables|/Script/Engine.Actor|GetRootComponent TargetActor))
              (Collision|BindEventtoOnActorBeginOverlap (stale _returnvalue_3) (delegate Custom|DealRangedDamage)))))))
    (:OnNotifyBegin
      (bind _returnvalue_3 (Game|SpawnActorfromClass "/Game/Objects/ThirdParty/Weapon/Ammo/BP_Ammo_Stone.BP_Ammo_Stone_C" (Math|Transform|MakeTransform (Transformation|GetSocketLocation (Variables|Character|GetMesh) "LeftHandSocket_Ball")) "Undefined" "MultiplyWithRoot" 0 self))
      (Variables|/Game/Objects/ThirdParty/Weapon/Ammo/BP_Ammo_Stone.BP_Ammo_Stone_C|SetTargetActor _returnvalue_3 TargetActor)
      (Variables|/Script/Engine.MovementComponent|SetVelocity (Variables|/Game/Objects/ThirdParty/Weapon/Ammo/BP_Ammo_Stone.BP_Ammo_Stone_C|GetProjectileMovement _returnvalue_3) (+ (* _returnvalue_2 3e+01) "0.000000,30.000000,300.000000")))))

(event EventDestroyed
  (bind _weaponactor (Variables|Default|GetWeaponActor))
  (Utilities|IsValid _weaponactor
    (:Is%20Valid
      (Actor|DestroyActor _weaponactor))))

(event EventBeginPlay
  (|CallParentFunction)
  ;[1 1 1] TEST TP on spawn point
  (Utilities|FlowControl|Sequence
    (:then_0
      (bind _returnvalue (Actor|GetActorOfClass "/Game/Objects/Pawns/Forest/BP_ForestlingStaticConstruct.BP_ForestlingStaticConstruct_C"))
      (Utilities|IsValid _returnvalue
        (:Is%20Valid
          (Actor|DestroyActor _returnvalue))))
    (:then_1
      (bind _asbp_game_state (Utilities|Casting|CastToBP_GameState (Game|GetGameState)))
      (bind _returnvalue_2 (Class|SocialService|GetObjectsbyTag (Class|GameStateDefault|GetSocialService _asbp_game_state) "ForesterHouse"))
      (if (Utilities|Set|IsNotEmpty _returnvalue_2)
        (bind _result (Utilities|Set|ToArray _returnvalue_2))
        (bind _returnvalue_3 (Class|GameObjectCore|GetOwner (Utilities|Array|Get(acopy) _result)))
        (bind _asbp_house_forester (Utilities|Casting|CastToBP_House_Forester _returnvalue_3))
        (bind _spawnplacetransform (Default|GetSpawnPlace _asbp_house_forester))
        (Transformation|SetActorTransform (Math|Transform|MakeTransform (.Location (Math|Transform|BreakTransform _spawnplacetransform))) false true)
        (EventDispatchers|BindEventtoOnTaskComplete (delegate Custom|ClearTask))
        (bind _returnvalue_4 (Class|GameObjectInterface|GetCore))
        (bind _returnvalue_5 (Class|GameObjectCore|GetComponent _returnvalue_4 "Health"))
        (bind _ashealth_default_component (Utilities|Casting|CastToHealthDefaultComponent _returnvalue_5))
        (EventDispatchers|BindEventtoOnDeath _ashealth_default_component (delegate Custom|OnDeath))))))

(event EventAttackDefault
  (params (TargetActor :type Actor%20Object%20Reference))
  ;[1 1 1] WeaponTasks
  (if (Math|Random|RandomBool)
    (Variables|Default|SetAttackAnimMontage "/Game/Objects/Pawns/Forest/Forestling/Animation/AM_Forestling_AttackRight.AM_Forestling_AttackRight")
    (else
      (Variables|Default|SetAttackAnimMontage "/Game/Objects/Pawns/Forest/Forestling/Animation/AM_Forestling_AttackTop.AM_Forestling_AttackTop")))
  (|CallParentFunction TargetActor))

(event EventDoWorkatPlace
  (params (WorkTime :type Float%20%28double-precision%29) (WorkPlaceObject :type Object%20Object%20Reference))
  (Utilities|FlowControl|Sequence
    (:then_0
      (goto _label Reset))
    (:then_1
      (Utilities|FlowControl|DoN 3 :!label _label
        (:Exit
          (Animation|Montage|PlayMontage (Variables|Character|GetMesh) "/Game/Objects/Pawns/Forest/Forestling/Animation/AM_Forestling_AttackTop.AM_Forestling_AttackTop"
            (:OnCompleted
              (goto _label))))))))

(fn ConstructionScript)

(fn TryGetTask0
  (bind _asgame_state_default (Utilities|Casting|CastToGameStateDefault (Game|GetGameState)))
  (bind _returnvalue (Class|GameObjectInterface|GetCore))
  (bind _returnvalue_2 (Class|TaskManagerService|GetTask (Class|GameStateDefault|GetTaskManagerService _asgame_state_default) _returnvalue))
  (if _returnvalue_2
    (Default|CallOnTaskReserve)))