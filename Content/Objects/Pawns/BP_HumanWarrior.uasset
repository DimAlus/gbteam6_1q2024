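; BP_HumanWarrior is a human warrior pawn that carries a sword.
; On BeginPlay it runs the parent logic, binds an OnDeath handler to the core's Health component, then spawns BP_Sword_ snapped to the right-hand socket on its mesh.
; The sword is stored as WeaponActor and destroyed along with the pawn, while the OnDeath handler is currently empty.
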(event Custom|OnDeath)

(event EventDestroyed
  (Actor|DestroyActor (Variables|Default|GetWeaponActor)))

(event EventBeginPlay
  (|CallParentFunction)
  (Utilities|FlowControl|Sequence
    (:then_1
      (bind _returnvalue (Class|GameObjectInterface|GetCore))
      (bind _returnvalue_2 (Class|GameObjectCore|GetComponent _returnvalue "Health"))
      (bind _ashealth_default_component (Utilities|Casting|CastToHealthDefaultComponent _returnvalue_2))
      (EventDispatchers|BindEventtoOnDeath _ashealth_default_component (delegate Custom|OnDeath))
      (bind _returnvalue_3 (Game|SpawnActorfromClass "/Game/Objects/ThirdParty/Weapon/BP_Sword_.BP_Sword__C" (Math|Transform|MakeTransform "0, 0, 0") "Undefined" "MultiplyWithRoot" 0 0))
      (Transformation|AttachComponentToComponent _returnvalue_3 (Variables|Character|GetMesh) "RightHandSocket_Sword" "SnapToTarget" "SnapToTarget" "SnapToTarget" true)
      (Variables|Default|SetWeaponActor _returnvalue_3))))

(fn ConstructionScript)