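; BP_Wisp is a melee pawn that fights with a club and uses Forestling attack montages.
; Equip spawns the club on the mesh's right-hand socket, while unequip and the pawn's destruction remove it.
; AttackDefault randomly picks a right or top swing montage before handing off to the parent's attack logic.
; BeginPlay binds task-complete and Health component death events, but both handlers are empty stubs.
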(event Custom|OnDeath
  ;[1 1 1] OnDeath
)

(event Custom|ClearTask)

(event Custom|UnequipWeapon
  ;[1 1 1] WeaponTasks
  (Utilities|IsValid (Variables|Default|GetWeaponActor)
    (:Is%20Valid
      (Actor|DestroyActor (Variables|Default|GetWeaponActor)))))

(event Custom|EquipWeapon
  ;[1 1 1] WeaponTasks
  (Utilities|IsValid (Variables|Default|GetWeaponActor)
    (:Is%20Not%20Valid
      (bind _returnvalue (Game|SpawnActorfromClass "/Game/Objects/ThirdParty/Weapon/BP_Club_.BP_Club__C" (Math|Transform|MakeTransform "0, 0, 0") "Undefined" "MultiplyWithRoot" 0 0))
      (bind _output_get (Variables|Default|SetWeaponActor _returnvalue))
      (Transformation|AttachComponentToComponent _output_get (Variables|Character|GetMesh) (Utilities|Name|MakeLiteralName "RightHandSocket") "SnapToTarget" "SnapToTarget" "SnapToTarget" true))))

(event EventAttackDefault
  (params (TargetActor :type Actor%20Object%20Reference))
  ;[1 1 1] WeaponTasks
  (if (Math|Random|RandomBool)
    (Variables|Default|SetAttackAnimMontage "/Game/Objects/Pawns/Forest/Forestling/Animation/AM_Forestling_AttackRight.AM_Forestling_AttackRight")
    (else
      (Variables|Default|SetAttackAnimMontage "/Game/Objects/Pawns/Forest/Forestling/Animation/AM_Forestling_AttackTop.AM_Forestling_AttackTop")))
  (|CallParentFunction TargetActor))

(event EventDestroyed
  (bind _weaponactor (Variables|Default|GetWeaponActor))
  ;[1 1 1] OnDeath
  (Utilities|IsValid _weaponactor
    (:Is%20Valid
      (Actor|DestroyActor _weaponactor))))

(event EventBeginPlay
  (|CallParentFunction)
  (EventDispatchers|BindEventtoOnTaskComplete (delegate Custom|ClearTask))
  (bind _returnvalue (Class|GameObjectInterface|GetCore))
  (bind _returnvalue_2 (Class|GameObjectCore|GetComponent _returnvalue "Health"))
  (bind _ashealth_default_component (Utilities|Casting|CastToHealthDefaultComponent _returnvalue_2))
  (EventDispatchers|BindEventtoOnDeath _ashealth_default_component (delegate Custom|OnDeath)))

(fn ConstructionScript)