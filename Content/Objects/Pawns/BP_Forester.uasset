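; Forester pawn that works seated at a workplace, with a Forestling construct spawned in front of it to show production progress.
; Work swaps to a docked AnimBP and loops a montage, rate-scaled by work time, renewing the construct from the workplace Generator's "WORK" progress until complete.
; Finishing restores locomotion and destroys the construct.
; It seeks and reserves delivery tasks via its Tasker only when no AI-controlled Forestling is out of combat.
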(event Custom|RemoveForestlingConstruct
  (Utilities|IsValid (stale EventDoWorkatPlace _returnvalue_2)
    (:Is%20Valid
      (Actor|DestroyActor (stale EventDoWorkatPlace _returnvalue_2)))))

(event Custom|ContinueWork
  (Animation|Montage|PlayMontage (Variables|Character|GetMesh) "/Game/Objects/Pawns/Forest/Forester/Animation/AM_Forester_SitGrabStaff_01.AM_Forester_SitGrabStaff_01" (/ 1.2e+02 (stale EventDoWorkatPlace WorkTime))
    (:OnCompleted
      (bind _returnvalue (CallFunction|GetWorkProgressPercent (stale EventDoWorkatPlace WorkPlaceObject)))
      (Utilities|IsValid (stale EventDoWorkatPlace _returnvalue_2)
        (:Is%20Valid
          (Default|RenewConstruct (stale EventDoWorkatPlace _returnvalue_2) _returnvalue)
          (if (< _returnvalue 1.0)
            (CallFunction|ContinueWork)))))))

(event EventDoWorkatPlace
  (params (WorkTime :type Float%20%28double-precision%29) (WorkPlaceObject :type Object%20Object%20Reference))
  (bind _returnvalue (CallFunction|GetWorkProgressPercent WorkPlaceObject))
  (bind _returnvalue_2 (CallFunction|SpawnForestlingConstruct _returnvalue))
  (Animation|Montage|PlayMontage (Variables|Character|GetMesh) "/Game/Objects/Pawns/Forest/Forester/Animation/AM_Forester_SitGrabStaff_01.AM_Forester_SitGrabStaff_01" (/ 1.2e+02 WorkTime)
    (:OnCompleted
      (bind _returnvalue_3 (CallFunction|GetWorkProgressPercent WorkPlaceObject))
      (Utilities|IsValid _returnvalue_2
        (:Is%20Valid
          (Default|RenewConstruct _returnvalue_2 _returnvalue_3)
          (if (< _returnvalue_3 1.0)
            (CallFunction|ContinueWork)))))))

(event EventPreparetoWorkinPlace
  (bind _mesh (Variables|Character|GetMesh))
  (Variables|/Script/Engine.CharacterMovementComponent|SetbOrientRotationToMovement (Variables|Character|GetCharacterMovement) false)
  (Class|SkeletalMeshComponent|SetAnimClass _mesh "/Game/Objects/Pawns/Forest/Forester/Animation/ABP_Forester_Docked.ABP_Forester_Docked_C")
  (Animation|Montage|PlayMontage _mesh "/Game/Objects/Pawns/Forest/Forester/Animation/AM_Forester_SitToStand_Reverse.AM_Forester_SitToStand_Reverse"
    (:OnCompleted
      (Default|CallOnPreparedtoWork))))

(event EventFinishWorkatPlace
  (Variables|/Script/Engine.CharacterMovementComponent|SetbOrientRotationToMovement (Variables|Character|GetCharacterMovement) true)
  (Class|SkeletalMeshComponent|SetAnimClass (Variables|Character|GetMesh) "/Game/Objects/Pawns/Forest/Forester/Animation/ABP_Forester.ABP_Forester_C")
  (CallFunction|RemoveForestlingConstruct))

(fn ConstructionScript)

(fn SpawnForestlingConstruct
  (params (ReadinessPercent :type Float%20%28double-precision%29))
  (bind _returnvalue (Transformation|GetActorLocation))
  (bind (_x _y _z) (Math|Vector|BreakVector _returnvalue))
  (bind _returnvalue_2 (Game|SpawnActorfromClass "/Game/Objects/Pawns/Forest/BP_ForestlingStaticConstruct.BP_ForestlingStaticConstruct_C" (Math|Transform|MakeTransform (+ (* (Math|Vector|GetForwardVector (Transformation|GetActorRotation)) 8e+01) (Math|Vector|MakeVector _x _y (- _z 8e+01)))) "Undefined" "MultiplyWithRoot" 0 0))
  (return _returnvalue_2))

(fn RenewForestlingConstruct
  (params (ProductionReadinessPercent :type Float%20%28double-precision%29) (ForeslingConstuct :type BP%20Forestling%20Static%20Construct%20Object%20Reference)))

(fn GetWorkProgressPercent
  (params (WorkPlaceObject :type Object%20Object%20Reference))
  (bind _returnvalue (Class|GameObjectInterface|GetCore(Message) WorkPlaceObject))
  (bind _returnvalue_2 (Class|GameObjectCore|GetComponent _returnvalue "Generator"))
  (bind _asgenerator_base_component (Utilities|Casting|CastToGeneratorBaseComponent _returnvalue_2)
    (:then
      (bind _returnvalue_3 (Class|GeneratorBaseComponent|GetProgressPercents _asgenerator_base_component "WORK"))
      (return _returnvalue_3))
    (:CastFailed
      (return 0.0))))

(fn TryGetDeliveryTask
  (bind _asgame_instance_default (Utilities|Casting|CastToGameInstanceDefault (Game|GetGameInstance)))
  (bind _returnvalue (Class|SocialService|GetObjectsbyTag (Class|GameInstanceDefault|GetSocialService _asgame_instance_default) "Forestling"))
  (if (Utilities|Set|IsNotEmpty _returnvalue)
    (bind _result (Utilities|Set|ToArray _returnvalue))
    (bind _array_element (Utilities|Array|ForEachLoopwithBreak _result :!label _label)
      (:LoopBody
        (bind _returnvalue_2 (Class|GameObjectCore|GetOwner _array_element))
        (Utilities|IsValid (AI|GetAIController _returnvalue_2)
          (:Is%20Valid
            (if (Utilities|Enum|NotEqual(Enum) (Utilities|Enum|ByteToEnumEAIState (Class|BlackboardComponent|GetValueasEnum (Variables|/Script/AIModule.AIController|GetBlackboard (AI|GetAIController _returnvalue_2)) (Utilities|Name|MakeLiteralName "AIState"))) "Combat")
              (LocalVariables|SetHasReadyWorkers true)
              (goto _label Break)))))
      (:Completed
        (if (not (LocalVariables|GetHasReadyWorkers))
          (bind _returnvalue_3 (Class|GameObjectInterface|GetCore :!label _label_2))
          (bind _returnvalue_4 (Class|GameObjectCore|GetComponent _returnvalue_3 "Tasker"))
          (bind _astasker_base_component (Utilities|Casting|CastToTaskerBaseComponent _returnvalue_4))
          (bind _returnvalue_5 (Class|TaskerBaseComponent|FindTask _astasker_base_component))
          (if _returnvalue_5
            (Default|CallOnTaskReserve)))))
    (else
      (goto _label_2))))