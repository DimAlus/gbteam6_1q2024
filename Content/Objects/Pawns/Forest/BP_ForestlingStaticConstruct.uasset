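; Static visual of a Forestling under construction, which assembles piece by piece as its production progresses.
; RenewConstruct maps the readiness fraction to one of five stages through ChooseForestlingBuildStep.
; Each stage cumulatively reveals the base, arms and horns through chained visibility calls, with nothing hidden again.
; On destruction it spawns a curse blink Niagara effect at its location.
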(event EventBeginPlay)

(event Collision|EventActorBeginOverlap
  (params (OtherActor :type Actor%20Object%20Reference)))

(event EventTick
  (params (DeltaSeconds :type Float%20%28single-precision%29)))

(event EventDestroyed
  (Niagara|SpawnSystematLocation "/Game/FX/ThirdParty/BlinkAndDashVFX/VFX_Niagara/NS_Curse_Blink.NS_Curse_Blink" (Transformation|GetActorLocation)))

(fn ConstructionScript)

(fn RenewConstruct
  (params (ProductionReadinessPercent :type Float%20%28double-precision%29))
  (Utilities|ChooseForestlingBuildStep ProductionReadinessPercent
    (:First
      _)
    (:Second
      (Rendering|SetVisibility (Variables|Default|GetLeftArm) true false :!label _label))
    (:Third
      (Rendering|SetVisibility (Variables|Default|GetRightArm) true false :!label _label_2)
      (goto _label))
    (:Fourth
      (Rendering|SetVisibility (Variables|Default|GetLeftHorn) true false :!label _label_3)
      (goto _label_2))
    (:Fifth
      (Rendering|SetVisibility (Variables|Default|GetRightHorn) true false)
      (goto _label_3)))
  (Rendering|SetVisibility (Variables|Default|GetBase) true false))