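; Forester pawn that works in place, visibly assembling a static forestling construct.
; Preparing swaps to the docked AnimBP, stops orient-to-movement and plays a montage before signalling readiness.
; Work chains repeated staff montages, rate-scaled by work time, spawning the construct in front after the first, then revealing an arm or horn after each.
; Finishing restores the normal AnimBP and movement rotation and destroys the construct; a stand-up montage is left unwired.
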(event Custom|RemoveForestlingConstruct
  (Utilities|IsValid (stale EventDoWorkatPlace _returnvalue_3)
    (:Is%20Valid
      (Actor|DestroyActor (stale EventDoWorkatPlace _returnvalue_3)))))

(event EventDoWorkatPlace
  (params (WorkTime :type Float%20%28double-precision%29) (WorkPlaceObject :type Object%20Object%20Reference))
  (bind _returnvalue (Transformation|GetActorLocation))
  (bind _returnvalue_2 (/ 1e+01 WorkTime))
  (bind (_x _y _z) (Math|Vector|BreakVector _returnvalue))
  (Animation|Montage|PlayMontage (Variables|Character|GetMesh) "/Game/Objects/Pawns/Forest/Forester/Animation/AM_Forester_SitGrabStaff_01.AM_Forester_SitGrabStaff_01" _returnvalue_2
    (:OnCompleted
      (bind _returnvalue_3 (Game|SpawnActorfromClass "/Game/Objects/Pawns/Forest/BP_ForestlingStaticConstruct.BP_ForestlingStaticConstruct_C" (Math|Transform|MakeTransform (+ (* (Math|Vector|GetForwardVector (Transformation|GetActorRotation)) 8e+01) (Math|Vector|MakeVector _x _y (- _z 8e+01)))) "Undefined" "MultiplyWithRoot" 0 0))
      (Animation|Montage|PlayMontage (Variables|Character|GetMesh) "/Game/Objects/Pawns/Forest/Forester/Animation/AM_Forester_SitGrabStaff_01.AM_Forester_SitGrabStaff_01" _returnvalue_2
        (:OnCompleted
          (Rendering|SetVisibility (Variables|/Game/Objects/Pawns/Forest/BP_ForestlingStaticConstruct.BP_ForestlingStaticConstruct_C|GetLeftArm _returnvalue_3) true false)
          (Animation|Montage|PlayMontage (Variables|Character|GetMesh) "/Game/Objects/Pawns/Forest/Forester/Animation/AM_Forester_SitGrabStaff_01.AM_Forester_SitGrabStaff_01" _returnvalue_2
            (:OnCompleted
              (Rendering|SetVisibility (Variables|/Game/Objects/Pawns/Forest/BP_ForestlingStaticConstruct.BP_ForestlingStaticConstruct_C|GetRightArm _returnvalue_3) true false)
              (Animation|Montage|PlayMontage (Variables|Character|GetMesh) "/Game/Objects/Pawns/Forest/Forester/Animation/AM_Forester_SitGrabStaff_01.AM_Forester_SitGrabStaff_01" _returnvalue_2
                (:OnCompleted
                  (Rendering|SetVisibility (Variables|/Game/Objects/Pawns/Forest/BP_ForestlingStaticConstruct.BP_ForestlingStaticConstruct_C|GetLeftHorn _returnvalue_3) true false)
                  (Animation|Montage|PlayMontage (Variables|Character|GetMesh) "/Game/Objects/Pawns/Forest/Forester/Animation/AM_Forester_SitGrabStaff_01.AM_Forester_SitGrabStaff_01" _returnvalue_2
                    (:OnCompleted
                      (Rendering|SetVisibility (Variables|/Game/Objects/Pawns/Forest/BP_ForestlingStaticConstruct.BP_ForestlingStaticConstruct_C|GetRightHorn _returnvalue_3) true false))))))))))))

(event EventPreparetoWorkinPlace
  (bind _mesh (Variables|Character|GetMesh))
  (Variables|/Script/Engine.CharacterMovementComponent|SetbOrientRotationToMovement (Variables|Character|GetCharacterMovement) false)
  (Class|SkeletalMeshComponent|SetAnimClass _mesh "/Game/Objects/Pawns/Forest/Forester/Animation/ABP_Forester_Docked.ABP_Forester_Docked_C")
  (Animation|Montage|PlayMontage _mesh "/Game/Objects/Pawns/Forest/Forester/Animation/AM_Forester_SitToStand_Reverse.AM_Forester_SitToStand_Reverse"
    (:OnCompleted
      (Default|CallOnPreparedtoWork))))

(event EventFinishWorkatPlace
  (Variables|/Script/Engine.CharacterMovementComponent|SetbOrientRotationToMovement (Variables|Character|GetCharacterMovement) true)
  (Class|SkeletalMeshComponent|SetAnimClass (Variables|Character|GetMesh) "/Game/Objects/Pawns/Forest/Forester/Animation/ABP_Forester.ABP_Forester_C")
  (CallFunction|RemoveForestlingConstruct))

(fn ConstructionScript)