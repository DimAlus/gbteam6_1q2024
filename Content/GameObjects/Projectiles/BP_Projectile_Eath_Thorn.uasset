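; BP_Projectile_Eath_Thorn is an earth thorn projectile that appears as a circular patch of animated vines on the ground.
; On initialization it snaps to the ground with a downward trace and scales its cylinder from the projectile data's radius.
; It scatters vine skeletal meshes by area density, randomizing placement and scale plus angle, duration and mirroring in ABP_Vine.
; Spawned vines are destroyed with the actor.
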(event Custom|Inited
  (bind _returnvalue (Transformation|GetActorLocation))
  (bind _outhit (Collision|LineTraceByChannel (+ _returnvalue "0.000000,0.000000,100.000000") (+ _returnvalue "0.000000,0.000000,-1000.000000") "TraceTypeQuery1" false 0 "None"))
  (Transformation|SetActorLocation (.Location (Collision|BreakHitResult _outhit)) false true)
  (bind _returnvalue_2 (Class|Projectile|GetProjectileData))
  (bind _output_get (Variables|Default|SetRadius (.Radius (Utilities|Struct|BreakSkillProjectileData _returnvalue_2))))
  (Transformation|SetWorldScale3D (Variables|Default|GetCylinder) (Math|Vector|MakeVector (* _output_get 0.02) (* _output_get 0.02) 0.5))
  (bind _output_get_2 (Variables|Default|SetSpace (* _output_get _output_get 3.1456 0.0001)))
  (for _index (range 0 (Math|Float|Round (* _output_get_2 (Variables|Default|GetVinesPerMeter))))
    (CallFunction|CreateVine (Math|Vector|RotateVectorAroundAxis (Math|Vector|MakeVector (Math|Random|RandomFloatinRange 0.0 (Variables|Default|GetRadius)) 0.0 0.0) (Math|Random|RandomFloatinRange 0.0 3.6e+02) "0.000000,0.000000,1.000000"))))

(event EventBeginPlay
  (|CallParentFunction)
  (EventDispatchers|BindEventtoOnInitialized (delegate Custom|Inited)))

(event EventDestroyed
  (Utilities|FlowControl|Sequence
    (:then_0
      (for _array_element (Variables|Default|GetSpawnedTentacles)
        (Components|DestroyComponent _array_element)))
    (:then_1
      (|CallParentFunction))))

(fn ConstructionScript)

(fn CreateVine
  (params (Location :type Vector))
  (bind _returnvalue (Game|AddComponentbyClass "/Script/Engine.SkeletalMeshComponent" false (Math|Transform|MakeTransform Location "0, 0, 0" (Math|Conversions|ToVector(Float) (Math|Random|RandomFloatinRange 0.8 1.2)))))
  (Utilities|Array|Add (Variables|Default|GetSpawnedTentacles) _returnvalue)
  (Variables|/Script/Engine.SkeletalMeshComponent|SetSkeletalMeshAsset _returnvalue "/Game/FX/Mesh/SKM_Vine.SKM_Vine")
  (Components|SkeletalMesh|SetAnimInstanceClass _returnvalue "/Game/FX/Animation/ABP_Vine.ABP_Vine_C")
  ;[0.15 0.15 0.15 0.5] Comment
  (bind _asabp_vine (Utilities|Casting|CastToABP_Vine (Components|SkeletalMesh|GetAnimInstance _returnvalue)))
  (Variables|/Game/FX/Animation/ABP_Vine.ABP_Vine_C|SetAngle _asabp_vine (* (Math|Random|RandomFloat) 2.0 3.1456))
  (Variables|/Game/FX/Animation/ABP_Vine.ABP_Vine_C|SetDuration _asabp_vine (Math|Random|RandomFloatinRange 1.0 2.0))
  (if (Math|Random|RandomBool)
    (Variables|/Game/FX/Animation/ABP_Vine.ABP_Vine_C|SetYMultiplier _asabp_vine 1.0)
    (else
      (Variables|/Game/FX/Animation/ABP_Vine.ABP_Vine_C|SetYMultiplier _asabp_vine -1.0)))
  (Variables|/Game/FX/Animation/ABP_Vine.ABP_Vine_C|SetInited _asabp_vine true))