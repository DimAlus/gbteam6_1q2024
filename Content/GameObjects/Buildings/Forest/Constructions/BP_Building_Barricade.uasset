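; BP_Building_Barricade is a Forest construction building that shows an arrow mesh while it is at level zero.
; After creation it calls the parent handler, gets the Generator component from Core and makes SMBuildingArrow visible if that generator's level is 0.
; On a level change it calls the parent handler and hides the arrow once the level rises above zero.
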(event Custom|OnObjectLevelChanged_Event
  (params (CurrentLevel :type Integer))
  (|CallParentFunction CurrentLevel)
  (if (> CurrentLevel 0)
    (Rendering|SetVisibility (Variables|Default|GetSM_BuildingArrow) false false)))

(event EventOnCreatingAfterEvent
  (|CallParentFunction)
  (bind _returnvalue (Class|GameObjectCore|GetComponent (Variables|Default|GetCore) "Generator"))
  (bind _asgenerator_base_component (Utilities|Casting|CastToGeneratorBaseComponent _returnvalue))
  (if (== (Class|GeneratorBaseComponent|GetLevel _asgenerator_base_component) 0)
    (Rendering|SetVisibility (Variables|Default|GetSM_BuildingArrow) true false)))

(fn ConstructionScript)