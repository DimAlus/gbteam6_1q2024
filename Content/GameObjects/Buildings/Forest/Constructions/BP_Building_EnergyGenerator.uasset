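; BP_Building_EnergyGenerator is a forest construction building for an energy generator, handling its visual effects across build states.
; Its prepare functions switch the NSEnegryGenerator effect and PointLight off while not placed and on once built.
; On construction destruction, both components are destroyed.
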(fn ConstructionScript)

(fn PrepareNotPlaced
  (Components|Activation|SetActive (Variables|Default|GetNS_EnegryGenerator) false true)
  (Rendering|SetVisibility (Variables|Default|GetPointLight) false false))

(fn PrepareBuilded
  (Components|Activation|SetActive (Variables|Default|GetNS_EnegryGenerator) true true)
  (Rendering|SetVisibility (Variables|Default|GetPointLight) true false)
  (return))

(fn PrepareConstructionDestroy
  (Components|DestroyComponent (Variables|Default|GetNS_EnegryGenerator)))