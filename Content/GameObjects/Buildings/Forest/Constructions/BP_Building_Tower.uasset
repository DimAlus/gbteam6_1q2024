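; Forest tower building whose top mesh turns solid once its generator succeeds and is removed when the building tries to die.
; On BeginPlay it binds to the Generator and Health components on its core, which drive enabling query and physics collision on the tower top or destroying that component.
; It overrides GetLocationByType to return the AttachLocation transform for Attach requests, deferring other types to the parent.
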(event Custom|SetPlaneActive
  (params (GeneratorName :type String) (Generator :type Generator%20Element%20Info%20Structure%20%28by%20ref%29))
  (Collision|SetCollisionEnabled (Variables|Default|GetSM_TowerTop) "QueryAndPhysics"))

(event Custom|DestroyPlane
  (params (Value :type Integer))
  (Components|DestroyComponent (Variables|Default|GetSM_TowerTop)))

(event EventBeginPlay
  (|CallParentFunction)
  (Utilities|FlowControl|Sequence
    (:then_0
      (bind _returnvalue (Class|GameObjectInterface|GetCore))
      (bind _returnvalue_2 (Class|GameObjectCore|GetComponent _returnvalue "Generator"))
      (bind _asgenerator_base_component (Utilities|Casting|CastToGeneratorBaseComponent _returnvalue_2))
      (EventDispatchers|BindEventtoOnGeneratorSuccess _asgenerator_base_component (delegate Custom|SetPlaneActive)))
    (:then_1
      (bind _returnvalue_3 (Class|GameObjectInterface|GetCore))
      (bind _returnvalue_4 (Class|GameObjectCore|GetComponent _returnvalue_3 "Health"))
      (bind _ashealth_base_component (Utilities|Casting|CastToHealthBaseComponent _returnvalue_4))
      (EventDispatchers|BindEventtoOnTryDead _ashealth_base_component (delegate Custom|DestroyPlane)))))

(fn ConstructionScript)

(fn GetLocationbyType
  (params (LocationType :type ELocationType%20Enum :default "None"))
  (if (Utilities|Enum|Equal(Enum) LocationType "Attach")
    (return true (Math|Conversions|ToTransform(Vector) (Transformation|GetWorldLocation (Variables|Default|GetAttachLocation))))
    (else
      (bind (_found _returnvalue) (|CallParentFunction LocationType))
      (return _found _returnvalue))))