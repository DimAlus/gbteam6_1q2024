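; Forester house building that produces units through its core's Generator component and gathers them into its own formation group.
; While a "Forestling" generator runs, it shows a construct actor at SpawnPoint, removed on success or failure.
; Spawned actors are teleported to SpawnPoint and their cores join the group.
; The group is created after a short delay beside the house and repositioned to the core's group-service location when AI group data changes.
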(event Custom|OnGroupDataChanging_Event
  (bind _groupservice (CallFunction|GetGroupService))
  (bind _returnvalue (Class|GroupService|GetCoreLocation _groupservice (Variables|Default|GetCore)))
  (Class|GroupService|SetGroupData _groupservice (Variables|Default|GetFormationGroup) (Utilities|Struct|MakeGroupData "None" _returnvalue 0.0)))

(event Custom|OnGeneratorBegin
  (params (GeneratorName :type String) (Generator :type Generator%20Element%20Info%20Structure%20%28by%20ref%29))
  (if (Utilities|String|StartsWith GeneratorName "Forestling")
    (CallFunction|SpawnForestlingConstruct)
    (bind _returnvalue (Class|GameObjectInterface|GetCore))
    (bind _returnvalue_2 (Class|GameObjectCore|GetComponent _returnvalue "Generator"))
    (bind _asgenerator_base_component (Utilities|Casting|CastToGeneratorBaseComponent _returnvalue_2))
    (Default|Init (Variables|Default|GetForestlingConstruct) _asgenerator_base_component GeneratorName)))

(event Custom|OnGeneratorEnd
  (params (GeneratorName :type String) (Generator :type Generator%20Element%20Info%20Structure%20%28by%20ref%29))
  (if (Utilities|String|StartsWith GeneratorName "Forestling")
    (CallFunction|RemoveForestlingConstruct)))

(event Custom|OnSpawnActor
  (params (Actor :type Actor%20Object%20Reference) (StringValue :type String))
  (bind _spawnpoint (Variables|Default|GetSpawnPoint))
  (Transformation|SetActorRotation Actor (Transformation|GetWorldRotation _spawnpoint) true)
  (Transformation|SetActorLocation Actor (Transformation|GetWorldLocation _spawnpoint) false true)
  (bind _returnvalue (Class|GameObjectInterface|GetCore(Message) Actor))
  (Utilities|IsValid _returnvalue
    (:Is%20Valid
      (Class|GroupService|AddCoretoGroup (CallFunction|GetGroupService) (Variables|Default|GetFormationGroup) _returnvalue))))

(event EventOnCreatingAfterEvent
  (bind _core (Variables|Default|GetCore))
  (|CallParentFunction)
  (Utilities|FlowControl|Sequence
    (:then_0
      (bind _returnvalue (Class|GameObjectCore|GetComponent _core "Generator"))
      (bind _asgenerator_base_component (Utilities|Casting|CastToGeneratorBaseComponent _returnvalue))
      (EventDispatchers|BindEventtoOnGenerationBegin _asgenerator_base_component (EventDispatchers|CreateEvent :!event Custom|OnGeneratorBegin))
      (EventDispatchers|AssignOnGeneratorSuccess _asgenerator_base_component (EventDispatchers|CreateEvent :!event Custom|OnGeneratorEnd))
      (EventDispatchers|BindEventtoOnGeneratorFail _asgenerator_base_component (EventDispatchers|CreateEvent :!event Custom|OnGeneratorEnd))
      (EventDispatchers|BindEventtoOnSpawnActor _asgenerator_base_component (EventDispatchers|CreateEvent :!event Custom|OnSpawnActor)))
    (:then_1
      (bind _returnvalue_2 (Class|GameObjectCore|GetComponent _core "AI"))
      (bind _asaibase_component (Utilities|Casting|CastToAIBaseComponent _returnvalue_2))
      (EventDispatchers|BindEventtoOnGroupDataChanging _asaibase_component (EventDispatchers|CreateEvent :!event Custom|OnGroupDataChanging_Event)))
    (:then_2
      (Utilities|FlowControl|Delay 0.2)
      (bind _returnvalue_3 (Class|GroupService|CreateConstantGroup (CallFunction|GetGroupService) (Utilities|Array|MakeArray) (Utilities|Struct|MakeGroupData "None" (+ (Transformation|GetActorLocation) "500.000000,0.000000,0.000000") (.yaw (Transformation|GetActorRotation)))))
      (Variables|Default|SetFormationGroup _returnvalue_3))))

(fn ConstructionScript)

(fn SpawnForestlingConstruct
  (bind _spawnpoint (Variables|Default|GetSpawnPoint))
  (Utilities|IsValid (Variables|Default|GetForestlingConstruct)
    (:Is%20Not%20Valid
      (bind _returnvalue (Game|SpawnActorfromClass "/Game/GameObjects/Pawns/Forest/BP_ForestlingStaticConstruct.BP_ForestlingStaticConstruct_C" (Math|Transform|MakeTransform (Transformation|GetWorldLocation _spawnpoint) (Transformation|GetWorldRotation _spawnpoint)) "Undefined" "MultiplyWithRoot" 0 0))
      (Variables|Default|SetForestlingConstruct _returnvalue))))

(fn RemoveForestlingConstruct
  (bind _forestlingconstruct (Variables|Default|GetForestlingConstruct))
  (Utilities|IsValid _forestlingconstruct
    (:Is%20Valid
      (Actor|DestroyActor _forestlingconstruct))))