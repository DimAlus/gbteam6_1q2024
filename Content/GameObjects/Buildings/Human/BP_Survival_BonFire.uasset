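; Human survival bonfire building whose point light pulses in brightness during play.
; Each tick accumulates time and turns it into a looping linear triangle wave over LightTime, which adds up to LightBorders on top of the base LightIntencivity.
; Random flicker and light-position jitter nodes remain in the graph but are disconnected and never run.
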(event EventBeginPlay
  (Rendering|Components|Light|SetIntensity (Variables|Default|GetPointLight) (Variables|Default|GetLightIntencivity)))

(event Collision|EventActorBeginOverlap
  (params (OtherActor :type Actor%20Object%20Reference)))

(event EventTick
  (params (DeltaSeconds :type Float%20%28single-precision%29))
  (bind _lighttime (Variables|Default|GetLightTime))
  (bind _output_get (Variables|Default|SetLightCurrentTime (+ (Variables|Default|GetLightCurrentTime) DeltaSeconds)))
  (Rendering|Components|Light|SetIntensity (Variables|Default|GetPointLight) (+ (Variables|Default|GetLightIntencivity) (* (Variables|Default|GetLightBorders) (Math|Float|Absolute(Float) (- 1.0 (* (/ (Math|Float|%(Float) _output_get _lighttime) _lighttime) 2.0)))))))

(fn ConstructionScript)