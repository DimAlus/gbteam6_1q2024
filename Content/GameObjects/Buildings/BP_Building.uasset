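; Building actor that shows a health bar and an attack range zone, and hides behind a destruction effect on death.
; Generator component level and construction-stage events swap static or skeletal meshes from per-level data; a collision toggle for unbuilt level 0 is marked not working.
; Zone radius comes from the Auto skill's target finder, overridable by AI attacher actions, and drives a dynamic ring material.
; Selection changes update zone visibility and health bar mouse state.
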(event Custom|OnObjectLevelChanged_Event
  (params (CurrentLevel :type Integer))
  (bind _collisionbody (Variables|Default|GetCollisionBody))
  (bind _meshdatasbylevel (Variables|Default|GetMeshDatasByLevel))
  (bind (_value _returnvalue) (Utilities|Map|Find _meshdatasbylevel CurrentLevel))
  (Utilities|FlowControl|Sequence
    (:then_0
      (if _returnvalue
        (if (Utilities|Array|IsNotEmpty (.meshdatas _value))
          (CallFunction|ApplyMeshData (Utilities|Array|Get(acopy) (.meshdatas _value) (Utilities|Array|LastIndex (.meshdatas _value)))))))
    (:then_1
      ;[0.15 0.15 0.15 0.5] Not Worked!
      (if (> CurrentLevel 0)
        (Collision|SetCollisionEnabled _collisionbody (Variables|Default|GetDefaultCollisionEnabled) :!label _label)
        (else
          (bind _returnvalue_2 (Class|GameObjectCore|GetComponent (Variables|Default|GetCore) "Generator"))
          (bind _asgenerator_base_component (Utilities|Casting|CastToGeneratorBaseComponent _returnvalue_2))
          (bind _returnvalue_3 (Class|GeneratorBaseComponent|NeedBuilding _asgenerator_base_component))
          (if _returnvalue_3
            (Collision|SetCollisionEnabled _collisionbody "NoCollision")
            (else
              (goto _label))))))))

(event Custom|OnConstructionStageChanged_Event
  (params (CurrentLevel :type Integer) (Progress :type Float%20%28single-precision%29) (Stage :type Integer))
  (bind _returnvalue (+ CurrentLevel 1))
  (bind _meshdatasbylevel (Variables|Default|GetMeshDatasByLevel))
  (bind (_value _returnvalue_2) (Utilities|Map|Find _meshdatasbylevel _returnvalue))
  (if _returnvalue_2
    (if (Utilities|Array|IsNotEmpty (.meshdatas _value))
      (CallFunction|ApplyMeshData (Utilities|Array|Get(acopy) (.meshdatas _value) (Math|Integer|Min(Integer) Stage (Utilities|Array|LastIndex (.meshdatas _value))))))))

(event EventOnCreatingAfterEvent
  (|CallParentFunction)
  (Utilities|FlowControl|Sequence
    (:then_0
      (Variables|Default|SetDefaultCollisionEnabled (Collision|GetCollisionEnabled (Variables|Default|GetCollisionBody))))
    (:then_1
      (bind _returnvalue (Class|GameObjectCore|GetComponent (Variables|Default|GetCore) "Generator"))
      (bind _asgenerator_base_component (Utilities|Casting|CastToGeneratorBaseComponent _returnvalue))
      (EventDispatchers|AssignOnObjectLevelChanged _asgenerator_base_component (EventDispatchers|CreateEvent :!event Custom|OnObjectLevelChanged_Event))
      (EventDispatchers|AssignOnConstructionStageChanged _asgenerator_base_component (EventDispatchers|CreateEvent :!event Custom|OnConstructionStageChanged_Event))
      (CallFunction|OnObjectLevelChangedEvent (Class|GeneratorBaseComponent|GetLevel _asgenerator_base_component)))
    (:then_2
      (CallFunction|UpdateZoneRadius)
      (Rendering|SetVisibility (Variables|Default|GetAttackZone) false true))))

(event EventBeginPlay
  (bind _healthbar (Variables|Default|GetHealthBar))
  (|CallParentFunction)
  (bind _aswbp_object_short_staticstic (Utilities|Casting|CastToWBP_ObjectShortStaticstic (UserInterface|GetWidget _healthbar)))
  (bind _returnvalue (Class|GameObjectInterface|GetCore))
  (Default|Init _aswbp_object_short_staticstic _returnvalue _healthbar))

(event EventOnSelectionChangingEvent
  (|CallParentFunction)
  (bind _asplayer_pawn_default (Utilities|Casting|CastToPlayerPawnDefault (Game|Player|GetPlayerPawn 0)))
  (bind _returnvalue (Class|GameObjectCore|GetComponent (Variables|Default|GetCore) "AI"))
  (bind _asaibase_component (Utilities|Casting|CastToAIBaseComponent _returnvalue))
  (bind _returnvalue_2 (Class|AIBaseComponent|GetSelection _asaibase_component))
  (Utilities|FlowControl|Sequence
    (:then_0
      (bind _aswbp_object_short_staticstic (Utilities|Casting|CastToWBP_ObjectShortStaticstic (UserInterface|GetWidget (Variables|Default|GetHealthBar))))
      (Default|SetMouseTurned _aswbp_object_short_staticstic (.MouseTurn (Utilities|Struct|BreakObjectSelection _returnvalue_2))))
    (:then_1
      (Rendering|SetVisibility (Variables|Default|GetAttackZone) (or (and (== (Variables|Default|GetCore) (Variables|/Script/GBTeam6.PlayerPawnDefault|GetCurrentSelectedCore _asplayer_pawn_default)) (.Selection (Utilities|Struct|BreakObjectSelection _returnvalue_2))) (.ShowZone (Utilities|Struct|BreakObjectSelection _returnvalue_2))) true))))

(event EventOnDeadEvent
  (Niagara|SpawnSystematLocation "/Game/FX/VFX/BuildingDestroy/NS_BuildingDestroy.NS_BuildingDestroy" (Transformation|GetActorLocation))
  (Rendering|SetVisibility (Variables|Default|GetSceneBase) false true))

(fn ConstructionScript
  (bind _attackzone (Variables|Default|GetAttackZone))
  (bind _returnvalue (Transformation|GetWorldScale _attackzone))
  (bind _returnvalue_2 (Rendering|Material|CreateDynamicMaterialInstance "/Game/MaterialLibrary/AttackZone/MI_BuildingZoneRadius.MI_BuildingZoneRadius" "None" "None" :!class /Script/Engine.KismetMaterialLibrary))
  (bind _output_get (Variables|Default|SetMatAttackZone _returnvalue_2))
  (Rendering|Material|SetMaterial (Variables|Default|GetAttackZone) 0 _output_get)
  (CallFunction|SetZoneRadius (* (Math|Float|Min(Float) (.x _returnvalue) (.y _returnvalue)) 5e+01)))

(fn ApplyMeshData
  (params (data :type BPS%20Mesh%20Data%20Structure))
  (bind (_staticmesh _skeletalmesh _scale _material) (Utilities|Struct|BreakBPS_MeshData data))
  (bind _objectmesh (Variables|Default|GetObjectMesh))
  (bind _object_skeletal_mesh (Variables|Default|GetObject%20Skeletal%20Mesh))
  (Utilities|FlowControl|Sequence
    (:then_0
      (Utilities|IsValid _staticmesh
        (:Is%20Valid
          (Rendering|SetVisibility _objectmesh true false)
          (Components|StaticMesh|SetStaticMesh _objectmesh _staticmesh)
          (Transformation|SetWorldScale3D _objectmesh _scale)
          (for (_array_element _array_index) _material
            (Rendering|Material|SetMaterial _objectmesh _array_index _array_element)))
        (:Is%20Not%20Valid
          (Rendering|SetVisibility _objectmesh false false))))
    (:then_1
      (Utilities|IsValid _skeletalmesh
        (:Is%20Valid
          (Rendering|SetVisibility _object_skeletal_mesh true false)
          (Components|SkeletalMesh|SetSkeletalMeshAsset _object_skeletal_mesh _skeletalmesh)
          (Transformation|SetWorldScale3D _object_skeletal_mesh _scale)
          (for (_array_element_2 _array_index_2) _material
            (Rendering|Material|SetMaterial _object_skeletal_mesh _array_index_2 _array_element_2)))
        (:Is%20Not%20Valid
          (Rendering|SetVisibility _object_skeletal_mesh false false))))))

(fn SetCustomDepthStencil0
  (params (Value :type Integer)))

(fn SetCustomDepthStencil
  (params (Value :type Integer))
  (|CallParentFunction Value)
  (Rendering|SetCustomDepthStencilValue (Variables|Default|GetObject%20Skeletal%20Mesh) Value))

(fn UpdateZoneRadius
  (Utilities|FlowControl|Sequence
    (:then_0
      (CallFunction|SetZoneRadius 0.0))
    (:then_1
      (bind _returnvalue (Class|GameObjectCore|GetComponent (Variables|Default|GetCore) "SkillHeaver"))
      (bind _asskill_heaver_base_component (Utilities|Casting|CastToSkillHeaverBaseComponent _returnvalue))
      (bind (_skillfound _returnvalue_2) (Class|SkillHeaverBaseComponent|GetSkillData _asskill_heaver_base_component "Auto"))
      (if _skillfound
        (bind _returnvalue_3 (Class|SocialService|GetFinderRadius (CallFunction|GetSocialService) (Utilities|Struct|BreakSkillProjectileData (Utilities|Array|Get(acopy) (Utilities|Struct|BreakSkill _returnvalue_2)))))
        (CallFunction|SetZoneRadius _returnvalue_3)))
    (:then_2
      (bind _returnvalue_4 (Class|GameObjectCore|GetComponent (Variables|Default|GetCore) "AI"))
      (bind _asaibase_component (Utilities|Casting|CastToAIBaseComponent _returnvalue_4))
      (bind _returnvalue_5 (Class|AIBaseComponent|GetAttacherActions _asaibase_component))
      (for _array_element _returnvalue_5
        (if (.ReturnValue (Utilities|Map|Find (.OverridedSkills (Utilities|Struct|BreakGameObjectAction _array_element)) "Auto"))
          (bind _returnvalue_6 (Class|SocialService|GetFinderRadius (CallFunction|GetSocialService) (Utilities|Struct|BreakSkillProjectileData (Utilities|Array|Get(acopy) (Utilities|Struct|BreakSkill (.Value (Utilities|Map|Find (.OverridedSkills (Utilities|Struct|BreakGameObjectAction _array_element)) "Auto")))))))
          (CallFunction|SetZoneRadius _returnvalue_6))))))

(fn SetZoneRadius
  (params (radius :type Float%20%28double-precision%29))
  (bind _returnvalue (* radius 0.02))
  (bind _matattackzone (Variables|Default|GetMatAttackZone))
  (bind _attackzone (Variables|Default|GetAttackZone))
  (Transformation|SetWorldScale3D _attackzone (Math|Vector|MakeVector _returnvalue _returnvalue (.z (Transformation|GetWorldScale _attackzone))))
  (Rendering|Material|SetScalarParameterValue _matattackzone "RadiusOuter" radius :!class /Script/Engine.MaterialInstanceDynamic)
  (Rendering|Material|SetScalarParameterValue _matattackzone "RadiusInner" (- radius (Variables|Default|GetAttackZoneRadius)) :!class /Script/Engine.MaterialInstanceDynamic))