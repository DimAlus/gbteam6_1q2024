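; Stone ammo actor for the weapon system that plays a stone kick sound and removes itself shortly after spawning.
; On BeginPlay it switches off its Niagara projectile trail and starts two timed branches.
; A gate opens after a short delay, so later collision overlaps with TargetActor play the sound and destroy the stone.
; A longer fallback delay does the same without any overlap.
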(event OnComponentBeginOverlap(Collision)
  (params (OverlappedComponent :type Primitive%20Component%20Object%20Reference) (OtherActor :type Actor%20Object%20Reference) (OtherComp :type Primitive%20Component%20Object%20Reference) (OtherBodyIndex :type Integer) (bFromSweep :type Boolean) (SweepResult :type Hit%20Result%20Structure%20%28by%20ref%29))
  (Utilities|FlowControl|Gate true
    (:Exit
      (if (== OtherActor (Variables|Default|GetTargetActor))
        (Audio|PlaySoundatLocation "/Game/Sound/Wawe/Environment/Stone_Kick/stone_kick_-_6.stone_kick_-_6" (Transformation|GetActorLocation) "0, 0, 0" 1.0 1.0 0.0 0 0 0 0)
        (Utilities|FlowControl|DelayUntilNextTick)
        (Actor|DestroyActor)))))

(event EventBeginPlay
  (Components|Activation|SetActive (Variables|Default|GetNS_ProjectileTrail) false true)
  (Utilities|FlowControl|Sequence
    (:then_0
      (Utilities|FlowControl|Delay 1.0)
      (Utilities|FlowControl|Gate true) ; enters at Open
    )
    (:then_1
      (Utilities|FlowControl|Delay 2.5)
      (Audio|PlaySoundatLocation "/Game/Sound/Wawe/Environment/Stone_Kick/stone_kick_-_6.stone_kick_-_6" (Transformation|GetActorLocation) "0, 0, 0" 1.0 1.0 0.0 0 0 0 0)
      (Utilities|FlowControl|DelayUntilNextTick)
      (Actor|DestroyActor))))

(fn ConstructionScript)