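; Shoremaiden forest pawn that stays on no social team until no cages remain, then becomes friendly.
; After creation it sets its Social component's team to None and starts a short looping game timer that ignores time influence.
; The timer polls the social service for Cage-tagged objects; once none are found, it cancels itself and switches the team to Friendly.
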(event Custom|CheckCageExists_Event
  (bind _returnvalue (Class|SocialService|GetObjectsbyTag (CallFunction|GetSocialService) "Cage"))
  (if (Utilities|Set|IsEmpty _returnvalue)
    (Class|TimerService|InvalidateTimer (CallFunction|GetGameTimerManager) (Variables|Default|GetCheckCage%20Timer%20Handler))
    (bind _returnvalue_2 (Class|GameObjectCore|GetComponent (Variables|Default|GetCore) "Social"))
    (bind _associal_base_component (Utilities|Casting|CastToSocialBaseComponent _returnvalue_2))
    (Class|SocialBaseComponent|SetSocialTeam _associal_base_component "Friendly")))

(event EventOnCreatingAfterEvent
  (|CallParentFunction)
  (bind _returnvalue (Class|GameObjectCore|GetComponent (Variables|Default|GetCore) "Social"))
  (bind _associal_base_component (Utilities|Casting|CastToSocialBaseComponent _returnvalue))
  (Class|SocialBaseComponent|SetSocialTeam _associal_base_component "None")
  (bind _returnvalue_2 (Class|TimerService|SetTimer (CallFunction|GetGameTimerManager) (EventDispatchers|CreateEvent :!event Custom|CheckCageExists_Event) 0.2 true -1.0 false false))
  (Variables|Default|SetCheckCage%20Timer%20Handler _returnvalue_2))

(fn ConstructionScript)