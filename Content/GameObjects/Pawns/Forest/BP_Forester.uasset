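; Forester pawn that animates its Tasker component's tasks and enables work on creation.
; Before a task, it pauses processing, swaps to the docked anim class and resumes after a reversed sit-to-stand montage; completion restores the normal class.
; The first Receiving or Delivery registration sets the ForesterDeliver tutorial tag, then unbinds.
; Older workplace, resource-making and forestling logic is mostly empty events and disconnected nodes, partly marked Remove.
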(event Custom|ShowDeliveryDialog
  (EventDispatchers|UnbindEventfromOnTaskRegistry (stale EventOnCreatingAfterEvent _astasker_base_component) (delegate Custom|OnTaskRegistry_Event))
  (bind _asgame_instance_default (Utilities|Casting|CastToGameInstanceDefault (Game|GetGameInstance)))
  (Class|GameEventsService|UpdateTag (Class|GameInstanceDefault|GetGameEventsService _asgame_instance_default) "Tutor" "ForesterDeliver" true))

(event Custom|ContinueMakingSocial
  ;[0.3542 0.3542 0.3542] Remove
)

(event Custom|CheckNewGenerator
  (params (GeneratorName :type String) (Generator :type Generator%20Element%20Info%20Structure%20%28by%20ref%29))
  ;[0.3542 0.3542 0.3542] Remove
)

(event Custom|OnTaskStart
  (params (TaskType :type EGameTaskType%20Enum :default "Receiving"))
  (Animation|Montage|PlayMontage (Variables|Character|GetMesh) "/Game/GameObjects/Pawns/Forest/Forester/Animation/AM_Forester_SitGrabStaff_01.AM_Forester_SitGrabStaff_01"))

(event Custom|BreakResourceMaking
  ;[0.3542 0.3542 0.3542] Remove
)

(event Custom|CheckWorkPlace
  ;[0.3542 0.3542 0.3542] Remove
  (Utilities|IsValid (AI|Components|Blackboard|GetValueasObject (Variables|/Script/AIModule.AIController|GetBlackboard (AI|GetAIController self)) (Utilities|Name|MakeLiteralName "WorkPlace"))
    (:Is%20Not%20Valid
      (CallFunction|BreakResourceMaking)
      (bind _returnvalue (Class|GameObjectInterface|GetCore(Message) (stale EventMakeResource WorkPlaceObject)))
      (bind _returnvalue_2 (Class|GameObjectCore|GetComponent _returnvalue "Generator"))
      (bind _asgenerator_base_component (Utilities|Casting|CastToGeneratorBaseComponent _returnvalue_2))
      (EventDispatchers|UnbindEventfromOnGeneratorChanging _asgenerator_base_component (delegate Custom|CheckNewGenerator))
      (Utilities|FlowControl|DoOnce false) ; enters at Reset
    )))

(event Custom|OnTaskStartBefore
  (params (TaskType :type EGameTaskType%20Enum :default "Receiving"))
  (bind _mesh (Variables|Character|GetMesh))
  (bind _returnvalue (Class|GameObjectInterface|GetCore))
  (bind _returnvalue_2 (Class|GameObjectCore|GetComponent _returnvalue "Tasker"))
  (bind _astasker_base_component (Utilities|Casting|CastToTaskerBaseComponent _returnvalue_2))
  (Class|TaskerBaseComponent|NotTaskProcessStartNow _astasker_base_component)
  (Components|SkeletalMesh|SetAnimInstanceClass _mesh "/Game/GameObjects/Pawns/Forest/Forester/Animation/ABP_Forester_Docked.ABP_Forester_Docked_C")
  (Animation|Montage|PlayMontage _mesh "/Game/GameObjects/Pawns/Forest/Forester/Animation/AM_Forester_SitToStand_Reverse.AM_Forester_SitToStand_Reverse"
    (:OnCompleted
      (Class|TaskerBaseComponent|TaskProcessStartContinue _astasker_base_component))))

(event Custom|OnTaskCompleted
  (Animation|StopAnimMontage "/Game/GameObjects/Pawns/Forest/Forester/Animation/AM_Forester_SitResearch_01.AM_Forester_SitResearch_01")
  (Components|SkeletalMesh|SetAnimInstanceClass (Variables|Character|GetMesh) "/Game/GameObjects/Pawns/Forest/Forester/Animation/ABP_Forester.ABP_Forester_C"))

(event Custom|OnTaskRegistry_Event
  (params (TaskType :type EGameTaskType%20Enum :default "Receiving"))
  (if (or (Utilities|Enum|Equal(Enum) TaskType "Receiving") (Utilities|Enum|Equal(Enum) TaskType "Delivery"))
    (CallFunction|ShowDeliveryDialog)))

(event EventPreparetoWorkinPlace
  ;[0.3542 0.3542 0.3542] Remove
)

(event EventFinishWorkatPlace
  ;[0.3542 0.3542 0.3542] Remove
)

(event EventOnCreatingAfterEvent
  (|CallParentFunction)
  (bind _returnvalue (Class|GameObjectInterface|GetCore))
  (Utilities|FlowControl|Sequence
    (:then_0
      (bind _returnvalue_2 (Class|GameObjectCore|GetComponent _returnvalue "Tasker"))
      (bind _astasker_base_component (Utilities|Casting|CastToTaskerBaseComponent _returnvalue_2))
      (EventDispatchers|BindEventtoOnTaskProcessStarted _astasker_base_component (EventDispatchers|CreateEvent :!event Custom|OnTaskStart))
      (EventDispatchers|BindEventtoOnTaskProcessCompleted _astasker_base_component (EventDispatchers|CreateEvent :!event Custom|OnTaskCompleted))
      (EventDispatchers|BindEventtoOnTaskProcessBefore _astasker_base_component (EventDispatchers|CreateEvent :!event Custom|OnTaskStartBefore))
      (EventDispatchers|AssignOnTaskRegistry _astasker_base_component (delegate Custom|OnTaskRegistry_Event)))
    (:then_1
      (CallFunction|SetCanWork true))))

(event EventMakeResource
  (params (WorkTime :type Float%20%28double-precision%29) (WorkPlaceObject :type Object%20Object%20Reference))
  ;[0.3542 0.3542 0.3542] Remove
)

(event EventMakeSocialTagObject
  (params (WorkTime :type Float%20%28double-precision%29) (WorkPlaceObject :type Object%20Object%20Reference))
  ;[0.3542 0.3542 0.3542] Remove
)

(fn ConstructionScript)