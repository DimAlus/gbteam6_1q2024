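; Forestling pawn Blueprint that plays work animation at a build site and exposes its power and sleep-pose helpers.
; BuildObject gets the workplace's generator component and replays the top-attack montage while it stays at level 1 and the AI blackboard's IsCommanded is false.
; TryGetPowerStatus forwards the PowerConsumptionComponent's status.
; CorrectSleepPosition shifts the mesh height when sleep starts or ends.
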(event EventBeginPlay
  (|CallParentFunction))

(event EventBuildObject
  (params (WorkTime :type Float%20%28double-precision%29) (WorkPlaceObject :type Object%20Object%20Reference))
  (bind _self self)
  (bind _returnvalue (AI|GetAIController _self))
  (Utilities|IsValid WorkPlaceObject
    (:Is%20Valid
      (bind _returnvalue_2 (Class|GameObjectInterface|GetCore(Message) WorkPlaceObject))
      (bind _returnvalue_3 (Class|GameObjectCore|GetComponent _returnvalue_2 "Generator"))
      (bind _asgenerator_base_component (Utilities|Casting|CastToGeneratorBaseComponent _returnvalue_3))
      (Utilities|IsValid _returnvalue :!label _label
        (:Is%20Valid
          (Utilities|IsValid _asgenerator_base_component
            (:Is%20Valid
              (if (and (== (Class|GeneratorBaseComponent|GetLevel _asgenerator_base_component) 1) (not (ScalableFloat|GetValueasBool (Variables|/Script/AIModule.AIController|GetBlackboard _returnvalue) (Utilities|Name|MakeLiteralName "IsCommanded"))))
                (Animation|Montage|PlayMontage (Variables|Character|GetMesh) "/Game/GameObjects/Pawns/Forest/Forestling/Animation/AM_Forestling_AttackTop.AM_Forestling_AttackTop"
                  (:OnCompleted
                    (goto _label))
                  (:OnInterrupted
                    (goto _label)))))))))))

(fn ConstructionScript)

(fn TryGetPowerStatus
  (bind (_lowpowered _poweredoff _powerlevel) (Default|GetPowerStatus (Variables|Default|GetPowerConsumptionComponent)))
  (return true _lowpowered _poweredoff _powerlevel))

(fn CorrectSleepPosition
  (params (StartSleep :type Boolean))
  (bind _mesh (Variables|Character|GetMesh))
  (bind _mesh_2 (Variables|Character|GetMesh))
  (bind _relativelocation (Variables|/Script/Engine.SceneComponent|GetRelativeLocation _mesh_2))
  (bind _relativelocation_2 (Variables|/Script/Engine.SceneComponent|GetRelativeLocation _mesh))
  (if StartSleep
    (Transformation|SetRelativeLocation _mesh_2 (Math|Vector|MakeVector (.x _relativelocation) (.y _relativelocation) -89.0) false true)
    (else
      (Transformation|SetRelativeLocation _mesh (Math|Vector|MakeVector (.x _relativelocation_2) (.y _relativelocation_2) -97.0) false true))))