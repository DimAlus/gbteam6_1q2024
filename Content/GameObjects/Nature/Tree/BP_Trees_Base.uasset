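; Base tree Blueprint that randomizes and grounds a set of tree mesh components, with an optional editor footprint preview.
; The construction script can build a centered grid of flattened cubes as the preview.
; Initialize gives each supplied tree a mesh picked via TreesWeights, with its matching scale slightly varied, random yaw and XY jitter based on preview cell size.
; It then snaps each tree to a downward visibility trace hit.
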(event EventBeginPlay
  (CallFunction|Initialize))

(fn ConstructionScript
  (bind _countpreview (Variables|Default|Debug|GetCountPreview))
  (bind _sizepreview (Variables|Default|Debug|GetSizePreview))
  (bind _previewborder (Variables|Default|Debug|GetPreviewBorder))
  (bind _sizepreview_2 (Variables|Default|Debug|GetSizePreview))
  (bind _sizepreview_3 (Variables|Default|Debug|GetSizePreview))
  (bind _previewborder_2 (Variables|Default|Debug|GetPreviewBorder))
  (bind _countpreview_2 (Variables|Default|Debug|GetCountPreview))
  (bind _returnvalue (Math|Conversions|ToFloat(Integer) _countpreview_2))
  (bind _returnvalue_2 (- _countpreview 1))
  (bind _returnvalue_3 (* _previewborder _sizepreview_2))
  (bind _returnvalue_4 (Utilities|Operators|Subtract 1.0 _previewborder _previewborder))
  (bind _returnvalue_5 (/ _returnvalue 2.0))
  (bind _returnvalue_6 (+ _returnvalue_5 _previewborder_2 -0.5))
  (bind _returnvalue_7 (* _returnvalue_6 _sizepreview_3 -1.0))
  (if (Variables|Default|Debug|GetShowPreview)
    (for _index (range 0 _returnvalue_2)
      (for _index_2 (range 0 _returnvalue_2)
        (bind _returnvalue_8 (AddComponent|AddStaticMeshComponent false (Math|Transform|MakeTransform (Math|Vector|MakeVector (+ (* _index _sizepreview_2) _returnvalue_3) (+ (* _index_2 _sizepreview_2) _returnvalue_3) 0.0) "0, 0, 0" (Math|Vector|MakeVector (* _sizepreview 0.01 _returnvalue_4) (* _sizepreview 0.01 _returnvalue_4) 0.1))))
        (Components|StaticMesh|SetStaticMesh _returnvalue_8 "/Engine/BasicShapes/Cube.Cube")
        (Transformation|AddRelativeLocation _returnvalue_8 (Math|Vector|MakeVector _returnvalue_7 _returnvalue_7 0.0) false true)))))

(fn Initialize
  (params (Trees :type Array%20of%20Static%20Mesh%20Component%20Object%20References))
  (for _array_element Trees
    (CallFunction|RandomizeMesh _array_element)
    (bind _outhit (Collision|LineTraceByChannel (+ (Transformation|GetWorldLocation _array_element) "0.000000,0.000000,5000.000000") (+ (Transformation|GetWorldLocation _array_element) "0.000000,0.000000,-1000.000000") "TraceTypeQuery1" false 0 "None"))
    (Transformation|SetWorldLocation _array_element (.Location (Collision|BreakHitResult _outhit)) false true)))

(fn RandomizeMesh
  (params (Mesh :type Static%20Mesh%20Component%20Object%20Reference))
  (bind _sizepreview (Variables|Default|Debug|GetSizePreview))
  (bind _returnvalue (* _sizepreview 0.3))
  (bind _returnvalue_2 (* _returnvalue -1.0))
  (Utilities|FlowControl|Sequence
    (:then_0
      (bind _index (CallFunction|RandomIndex (LocalVariables|GetTreesWeights)))
      (bind _output_get (LocalVariables|SetIndex _index))
      (Components|StaticMesh|SetStaticMesh Mesh (Utilities|Array|Get(acopy) (LocalVariables|GetTreesMeshes) _output_get)))
    (:then_1
      (Transformation|SetWorldScale3D Mesh (* (Utilities|Array|Get(acopy) (LocalVariables|GetTreesScales) (LocalVariables|GetIndex)) (Math|Random|RandomFloatinRange 0.9 1.1))))
    (:then_2
      (Transformation|SetWorldRotation Mesh (Math|Rotator|MakeRotator 0.0 0.0 (Math|Random|RandomFloatinRange 0.0 3.6e+02)) false false))
    (:then_3
      (Transformation|SetWorldLocation Mesh (+ (Transformation|GetWorldLocation Mesh) (Math|Vector|MakeVector (Math|Random|RandomFloatinRange _returnvalue_2 _returnvalue) (Math|Random|RandomFloatinRange _returnvalue_2 _returnvalue) 0.0)) false true))))