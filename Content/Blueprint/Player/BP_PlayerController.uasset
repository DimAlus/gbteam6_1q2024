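; Player controller that creates the in-game HUD window on non-menu maps and handles basic game input.
; After a short BeginPlay delay it binds to GameStateDefault events, which add selector widgets to the window's container and show pages in its quest panel.
; Right click calls the right-button handler and Space toggles pause.
; Debug keys toggle window visibility, or open a test quest panel and call all human guards to arms.
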(event Custom|AddSelectorWidget
  (params (TimeLimit :type Float%20%28single-precision%29) (IsObjectSelector :type Boolean) (SelectedObject :type Actor%20Object%20Reference) (Location :type Vector))
  (bind _returnvalue (UserInterface|CreateWidget "/Game/Blueprint/UI/WBP_Selector.WBP_Selector_C"))
  (Default|Init _returnvalue IsObjectSelector SelectedObject Location TimeLimit)
  (Widget|Panel|AddChild (Variables|/Game/Blueprint/UI/WBP_GameWindow.WBP_GameWindow_C|GetContainer (Variables|Default|GetWindow)) _returnvalue))

(event Custom|ShowPages1
  (params (Pages :type Array%20of%20Quest%20Page%20Structures))
  (Default|ShowPages (Variables|/Game/Blueprint/UI/WBP_GameWindow.WBP_GameWindow_C|GetQuestPanel (Variables|Default|GetWindow)) Pages))

(event EventBeginPlay
  (Utilities|FlowControl|Delay 0.4)
  (bind _asgame_state_default (Utilities|Casting|CastToGameStateDefault (Game|GetGameState)))
  (if (not (Variables|/Script/GBTeam6.GameStateDefault|GetisMenuMap _asgame_state_default))
    (bind _returnvalue (UserInterface|CreateWidget "/Game/Blueprint/UI/WBP_GameWindow.WBP_GameWindow_C"))
    (UserInterface|Viewport|AddtoPlayerScreen _returnvalue)
    (Variables|Default|SetWindow _returnvalue)
    (bind _asgame_state_default_2 (Utilities|Casting|CastToGameStateDefault (Game|GetGameState)))
    (EventDispatchers|BindEventtoAddSelectedWidget _asgame_state_default_2 (delegate Custom|AddSelectorWidget))
    (EventDispatchers|BindEventtoOnShowPages _asgame_state_default_2 (delegate Custom|ShowPages1))))

(event EventTick
  (params (DeltaSeconds :type Float%20%28single-precision%29)))

(event Input|MouseEvents|RightMouseButton
  (params (Key :type Key%20Structure))
  (:Pressed
    (Default|CallRightButtonPressed)))

(event Input|KeyboardEvents|SpaceBar
  (params (Key :type Key%20Structure))
  (:Pressed
    (bind _output_get (Variables|Default|SetisPause (not (Variables|Default|GetisPause))))
    (Game|SetGamePaused _output_get)))

(event Input|KeyboardEvents|V
  (params (Key :type Key%20Structure))
  (bind _window (Variables|Default|GetWindow))
  ;[1 1 1] Debug and test
  (:Pressed
    (Utilities|FlowControl|FlipFlop
      (:A
        (Widget|SetVisibility _window "Hidden"))
      (:B
        (Widget|SetVisibility _window "Visible")))))

(event Input|KeyboardEvents|C
  (params (Key :type Key%20Structure))
  ;[1 1 1] Debug and test
  (:Pressed
    (bind _returnvalue (UserInterface|CreateWidget "/Game/Blueprint/UI/Demo/WBP_QuestPanel_HumanSeeksDaughter.WBP_QuestPanel_HumanSeeksDaughter_C" self))
    (UserInterface|Viewport|AddtoViewport _returnvalue 0)
    (Utilities|FlowControl|Sequence
      (:then_1
        (bind _outactors (Actor|GetAllActorsOfClass "/Game/Temp/Actors/Pawns/Demo/BP_HumanGuard.BP_HumanGuard_C"))
        (if (Utilities|Array|IsNotEmpty _outactors)
          (for _array_element _outactors
            (Default|ToArms _array_element)))))))

(fn ConstructionScript)

(fn SelectObject
  (params (NewParam :type Boolean)))