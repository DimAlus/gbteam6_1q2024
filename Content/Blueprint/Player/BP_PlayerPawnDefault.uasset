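; Default player pawn for strategy-style play, handling object selection, move orders and building placement.
; Select confirms a pending building and shows the selected game object in the controller's window, while Command cancels placement and sends AI-controlled selected pawns to the point of interest.
; A looping timer moves the spawned preview under the cursor through its Mapping component, updating build validity.
; Debug keys drive save/load, level opening, task inspection and quitting.
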(event EventTick
  (params (DeltaSeconds :type Float%20%28single-precision%29))
  (Rendering|Debug|DrawDebugSphere (.Location (Collision|BreakHitResult (Class|PlayerPawnDefault|GetHitUnderMouseCursor "ECC_WorldStatic"))) 1e+02 12 "(R=1.000000,G=0.080851,B=0.868892,A=1.000000)" 0.0))

(event EventOnSelect
  (|CallParentFunction)
  (Utilities|FlowControl|Sequence
    (:then_0
      (CallFunction|ApplyBuilding))
    (:then_1
      (bind _asbp_player_controller (Utilities|Casting|CastToBP_PlayerController (Pawn|GetController)))
      (bind _asgame_object_interface (Utilities|Casting|CastToGameObjectInterface (Variables|Default|GetSelectedActor)))
      (Default|SelectObject (Variables|/Game/Blueprint/Player/BP_PlayerController.BP_PlayerController_C|GetWindow _asbp_player_controller) _asgame_object_interface))))

(event EventOnCommand
  (|CallParentFunction)
  (Utilities|FlowControl|Sequence
    (:then_0
      (CallFunction|CancelBuilding))
    (:then_1
      (bind _selectedactor (Variables|Default|GetSelectedActor)
        (:then
          (bind _aspawn (Utilities|Casting|CastToPawn _selectedactor))
          (bind _asaic_default (Utilities|Casting|CastToAIC_Default (AI|GetAIController _aspawn)))
          (Default|CommandMove _asaic_default (Variables|Default|GetPointOfInterest)))
        (:else)))))

(event Input|KeyboardEvents|5
  (params (Key :type Key%20Structure :default "None"))
  (:Pressed
    (bind _asgame_mode_default (Utilities|Casting|CastToGameModeDefault (Game|GetGameMode)))
    (Development|PrintString (Variables|/Script/GBTeam6.GameModeDefault|GetSaveSlotName _asgame_mode_default))))

(event Input|KeyboardEvents|6
  (params (Key :type Key%20Structure :default "None"))
  (:Pressed
    (bind _asgame_mode_default (Utilities|Casting|CastToGameModeDefault (Game|GetGameMode)))
    (Variables|/Script/GBTeam6.GameModeDefault|SetSaveSlotName _asgame_mode_default "Test")))

(event Input|KeyboardEvents|7
  (params (Key :type Key%20Structure :default "None"))
  (:Pressed
    (Game|OpenLevel(byName) "Map/PlayMap/MapLand")))

(event Input|KeyboardEvents|Escape
  (params (Key :type Key%20Structure :default "None"))
  (:Pressed
    (Game|QuitGame 0 "Quit" false)))

(event Input|KeyboardEvents|9
  (params (Key :type Key%20Structure :default "None"))
  (:Pressed
    (Default|CallOnSave)))

(event Input|KeyboardEvents|0
  (params (Key :type Key%20Structure :default "None"))
  (:Pressed
    (Default|CallOnLoad)))

(event Input|KeyboardEvents|G
  (params (Key :type Key%20Structure :default "None"))
  (:Pressed
    (bind _asgame_state_default (Utilities|Casting|CastToGameStateDefault (Game|GetGameState)))
    (Class|TaskManagerService|RefreshNeeds (Class|GameStateDefault|GetTaskManagerService _asgame_state_default))))

(event Input|KeyboardEvents|L
  (params (Key :type Key%20Structure :default "None"))
  (:Pressed
    (bind _asgame_state_default (Utilities|Casting|CastToGameStateDefault (Game|GetGameState)))
    (Class|TaskManagerService|ShowGameTasksDebug (Class|GameStateDefault|GetTaskManagerService _asgame_state_default))
    (bind _returnvalue (Class|TaskManagerService|GetGameTasksDebug (Class|GameStateDefault|GetTaskManagerService _asgame_state_default)))
    (for _array_element _returnvalue
      (Development|PrintString (Utilities|GetDisplayName (.From (Utilities|Struct|BreakGameTask _array_element))) true true "(R=0.000000,G=1.000000,B=0.064711,A=1.000000)" 1e+01))))

(fn ConstructionScript)

(fn MoveSelectedBuilding
  (if (Variables|Default|GethaveSelectedBuilding)
    (bind _returnvalue (Class|GameObjectInterface|GetCore (Variables|Default|GetSelectedBuilding)))
    (bind _returnvalue_2 (Class|GameObjectCore|GetComponent _returnvalue "Mapping"))
    (bind _asmapping_base_component (Utilities|Casting|CastToMappingBaseComponent _returnvalue_2))
    (Class|MappingBaseComponent|SetOwnerLocation _asmapping_base_component (.location (Class|PlayerPawnDefault|GetHitUnderMouseCursor "ECC_Visibility")) true)
    (else
      (Utilities|Time|ClearandInvalidateTimerbyHandle (Variables|Default|GetMoveSelectedBuildingTimer)))))

(fn CreateBuilding
  (params (ActorClass :type Actor%20Class%20Reference))
  (if (Variables|Default|GethaveSelectedBuilding)
    (CallFunction|CancelBuilding))
  (bind _returnvalue (Game|SpawnActorfromClass ActorClass (Math|Transform|MakeTransform "0, 0, 0" "0, 0, 0" "1.000000,1.000000,1.000000") "Undefined" "MultiplyWithRoot" 0 0))
  (bind _asgame_object_interface (Utilities|Casting|CastToGameObjectInterface _returnvalue)
    (:then
      (Variables|Default|SetSelectedBuilding _asgame_object_interface)
      (Variables|Default|SethaveSelectedBuilding true)
      (bind _returnvalue_2 (Utilities|Time|SetTimerbyFunctionName 0 "MoveSelectedBuilding" 0.1 true))
      (Variables|Default|SetMoveSelectedBuildingTimer _returnvalue_2)
      (bind _component (CallFunction|GetComponentbyGameObject (Variables|Default|GetSelectedBuilding) "Mapping"))
      (bind _asmapping_base_component (Utilities|Casting|CastToMappingBaseComponent _component)
        (:then
          (Class|MappingBaseComponent|SetPreviewVisibility _asmapping_base_component true))
        (:CastFailed
          (CallFunction|CancelBuilding))))
    (:CastFailed
      (Actor|DestroyActor _returnvalue))))

(fn CancelBuilding
  (if (Variables|Default|GethaveSelectedBuilding)
    (Variables|Default|SethaveSelectedBuilding false)
    (bind _returnvalue (Class|GameObjectInterface|GetCore (Variables|Default|GetSelectedBuilding)))
    (bind _returnvalue_2 (Class|GameObjectCore|GetOwner _returnvalue))
    (Actor|DestroyActor _returnvalue_2)))

(fn ApplyBuilding
  (if (Variables|Default|GethaveSelectedBuilding)
    (bind _component (CallFunction|GetComponentbyGameObject (Variables|Default|GetSelectedBuilding) "Mapping"))
    (bind _asmapping_base_component (Utilities|Casting|CastToMappingBaseComponent _component)
      (:then
        (bind _returnvalue (Class|MappingBaseComponent|SetIsBuilded _asmapping_base_component true))
        (if _returnvalue
          (Variables|Default|SethaveSelectedBuilding false)
          (Class|MappingBaseComponent|SetPreviewVisibility _asmapping_base_component false)))
      (:CastFailed
        (CallFunction|CancelBuilding)))))