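; BPFL_Lib is a Blueprint function library of shared lookup helpers for resources, config, components and team relations.
; Resource data comes from scanning DTResourceData by resource type, also matching class for Actor resources, with Void or Disabled default rows as fallbacks.
; Config values are read by row name with a caller-supplied default.
; Components resolve through a GameObject's core, and team relations through the GameState's social service.
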(fn GetResourceData
  (params (Resource :type EResource%20Enum :default "Actor") (ActorClass :type Actor%20Class%20Reference))
  (bind _dt_resourcedata (LocalVariables|GetDT_ResourceData))
  (bind _outrownames (DataTable|GetDataTableRowNames _dt_resourcedata))
  (for _array_element _outrownames
    (bind _returnvalue (Utilities|GetDataTableRow _dt_resourcedata _array_element)
      (:then
        (if (Utilities|Enum|Equal(Enum) (.Resource (Utilities|Struct|BreakBPS_ResourseData _returnvalue)) Resource)
          (if (Utilities|Enum|Equal(Enum) (.Resource (Utilities|Struct|BreakBPS_ResourseData _returnvalue)) "Actor")
            (if (== (.ActorClass (Utilities|Struct|BreakBPS_ResourseData _returnvalue)) ActorClass)
              (return _returnvalue))
            (else
              (return _returnvalue)))))))
  (bind _resourcedata (CallFunction|GetResourceDataDefault true))
  (return _resourcedata))

(fn GetResourceDataDefault
  (params (IsVoid :type Boolean))
  (bind _dt_resourcedata (LocalVariables|GetDT_ResourceData))
  (if IsVoid
    (bind _returnvalue (Utilities|GetDataTableRow _dt_resourcedata "Void")
      (:then
        (return _returnvalue))
      (:RowNotFound
        _))
    (else
      (bind _returnvalue_2 (Utilities|GetDataTableRow _dt_resourcedata "Disabled")
        (:then
          (return _returnvalue_2))
        (:RowNotFound
          _))))
  (return (Utilities|Struct|MakeBPS_ResourseData "Actor" 0 0)))

(fn GetComponentbyGameObject
  (params (GameObject :type Game%20Object%20Interface%20Interface) (ComponentType :type EGameComponentType%20Enum :default "Health"))
  (Utilities|IsValid (Utilities|ToObject(Interface) GameObject)
    (:Is%20Valid
      (bind _returnvalue (Class|GameObjectInterface|GetCore GameObject))
      (bind _returnvalue_2 (Class|GameObjectCore|GetComponent _returnvalue ComponentType))
      (return _returnvalue_2))
    (:Is%20Not%20Valid
      (return 0))))

(fn GetConfig
  (params (ConfigName :type String) (Default :type Config%20Structure))
  (bind _returnvalue (Utilities|GetDataTableRow (LocalVariables|GetTable) (Utilities|String|StringToName ConfigName))
    (:then
      (return (.Value (Utilities|Struct|BreakTRConfig _returnvalue))))
    (:RowNotFound
      (return Default))))

(fn GetRelationsBetweenTeams
  (params (TeamFrom :type ESocialTeam%20Enum :default "None") (TeamTo :type ESocialTeam%20Enum :default "None"))
  (bind _asgame_state_default (Utilities|Casting|CastToGameStateDefault (Game|GetGameState))
    (:then
      (bind _returnvalue (Class|SocialService|GetRelationsBetweenTeams (Class|GameStateDefault|GetSocialService _asgame_state_default) TeamFrom TeamTo))
      (return _returnvalue))
    (:CastFailed
      (return "None"))))