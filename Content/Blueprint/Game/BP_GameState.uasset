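; Game state Blueprint that applies configured audio volumes at level start and handles game over.
; Shortly after BeginPlay, it reads master, music, effects and voice values from config, then overrides and pushes a sound mix for each sound class.
; It also binds a game-over event that opens StartMap, and flags any level other than MapLand as a menu map.
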(event Custom|GameOver
  (Game|OpenLevel(byName) "StartMap"))

(event EventBeginPlay
  (|CallParentFunction)
  (Utilities|FlowControl|Delay 0.2)
  (Utilities|FlowControl|Sequence
    (:then_0
      (bind _config (Class|GameStateDefault|GetConfig "SoundValue"))
      (Audio|SetSoundMixClassOverride "/Game/Sound/SoundClass/Mix_MasterSound.Mix_MasterSound" "/Game/Sound/SoundClass/MasterSound.MasterSound" (.FloatValue (Utilities|Struct|BreakConfig _config)) 1.0 0.0 true)
      (Audio|PushSoundMixModifier "/Game/Sound/SoundClass/Mix_MasterSound.Mix_MasterSound"))
    (:then_1
      (bind _config_2 (Class|GameStateDefault|GetConfig "MusicValue"))
      (Audio|SetSoundMixClassOverride "/Game/Sound/SoundClass/Mix_MusicSound.Mix_MusicSound" "/Game/Sound/SoundClass/MusicSound.MusicSound" (.FloatValue (Utilities|Struct|BreakConfig _config_2)) 1.0 0.0 true)
      (Audio|PushSoundMixModifier "/Game/Sound/SoundClass/Mix_MusicSound.Mix_MusicSound"))
    (:then_2
      (bind _config_3 (Class|GameStateDefault|GetConfig "EffectValue"))
      (Audio|SetSoundMixClassOverride "/Game/Sound/SoundClass/Mix_EffectsSound.Mix_EffectsSound" "/Game/Sound/SoundClass/EffectsSound.EffectsSound" (.FloatValue (Utilities|Struct|BreakConfig _config_3)) 1.0 0.0 true)
      (Audio|PushSoundMixModifier "/Game/Sound/SoundClass/Mix_EffectsSound.Mix_EffectsSound"))
    (:then_3
      (bind _config_4 (Class|GameStateDefault|GetConfig "VoiceValue"))
      (Audio|SetSoundMixClassOverride "/Game/Sound/SoundClass/Mix_VoiceSound.Mix_VoiceSound" "/Game/Sound/SoundClass/VoiceSound.VoiceSound" (.FloatValue (Utilities|Struct|BreakConfig _config_4)) 1.0 0.0 true)
      (Audio|PushSoundMixModifier "/Game/Sound/SoundClass/Mix_VoiceSound.Mix_VoiceSound"))
    (:then_4
      (EventDispatchers|BindEventtoOnGameOver (delegate Custom|GameOver)))
    (:then_5
      (bind _returnvalue (Game|GetCurrentLevelName true))
      (Variables|Default|SetisMenuMap (not (Utilities|Enum|Equal(Enum) _returnvalue "MapLand"))))))

(fn ConstructionScript)