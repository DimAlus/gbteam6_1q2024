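; BP_TreeFoliage is a tree foliage actor that registers its placement with a mapping component.
; Its construction script fetches the Mapping component, casts it to MappingBaseComponent and sets the owner location to the actor's location, with the can-build update turned off.
; The event graph holds only disabled default events, so it adds no runtime logic.
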(event EventBeginPlay
  (|CallParentFunction) ; This node is disabled and will not be called.\nDrag off pins to build functionality.
)

(event Collision|EventActorBeginOverlap
  (params (OtherActor :type Actor%20Object%20Reference))
  (|CallParentFunction OtherActor) ; This node is disabled and will not be called.\nDrag off pins to build functionality.
)

(event EventTick
  (params (DeltaSeconds :type Float%20%28single-precision%29))
  (|CallParentFunction DeltaSeconds) ; This node is disabled and will not be called.\nDrag off pins to build functionality.
)

(fn ConstructionScript
  (|CallParentFunction)
  (bind _returnvalue (Class|GameObjectInterface|GetComponent "Mapping"))
  (bind _asmapping_base_component (Utilities|Casting|CastToMappingBaseComponent _returnvalue))
  (Class|MappingBaseComponent|SetOwnerLocation _asmapping_base_component (Transformation|GetActorLocation) false))