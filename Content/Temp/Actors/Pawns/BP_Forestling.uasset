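; Forestling AI pawn that hauls resources between actors' inventories and can fight with a club.
; It runs a behavior tree and, while idle, polls the game state's task manager every second to reserve a task.
; Tasks pop resources at the source and push them at the destination, attempting a reversed delivery if the push fails.
; It also spawns socket-attached clubs, randomizes attack montages and destroys itself on death.
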(event Custom|OnDeath
  (bind _weaponactor (Variables|Default|GetWeaponActor))
  (Utilities|IsValid _weaponactor
    (:Is%20Valid
      (Actor|DestroyActor _weaponactor))
    (:Is%20Not%20Valid
      _))
  (Actor|DestroyActor))

(event Custom|ClearTask
  (Variables|Default|SetActiveTask (Utilities|Struct|MakeGameTask 0 "None"))
  (bind _asgame_state_default (Utilities|Casting|CastToGameStateDefault (Game|GetGameState)))
  (Class|TaskManagerService|CompleteTask (Class|GameStateDefault|GetTaskManagerService _asgame_state_default) self))

(event Custom|GetGameTask
  (Utilities|IsValid (.TaskPerformer (Utilities|Struct|BreakGameTask (Variables|Default|GetActiveTask)))
    (:Is%20Not%20Valid
      (bind _asgame_state_default (Utilities|Casting|CastToGameStateDefault (Game|GetGameState)))
      (bind (_tasktoreserve _returnvalue) (Class|TaskManagerService|ReserveTask (Class|GameStateDefault|GetTaskManagerService _asgame_state_default) self))
      (if _returnvalue
        (Variables|Default|SetActiveTask _tasktoreserve)))))

(event Custom|UnequipWeapon
  (Utilities|IsValid (Variables|Default|GetWeaponActor)
    (:Is%20Valid
      (Actor|DestroyActor (Variables|Default|GetWeaponActor)))))

(event Custom|EquipWeapon
  (Utilities|IsValid (Variables|Default|GetWeaponActor)
    (:Is%20Not%20Valid
      (bind _returnvalue (Game|SpawnActorfromClass "/Game/Temp/Actors/Weapons/BP_Club.BP_Club_C" (Math|Transform|MakeTransform "0, 0, 0") "Undefined" "MultiplyWithRoot" 0 0))
      (bind _output_get (Variables|Default|SetWeaponActor _returnvalue))
      (Transformation|AttachComponentToComponent _output_get (Variables|Character|GetMesh) (Utilities|Name|MakeLiteralName "RightHandSocket") "SnapToTarget" "SnapToTarget" "SnapToTarget" true))))

(event Custom|DeliverTo
  (AI|AIMoveTo self "0, 0, 0" (.To (Utilities|Struct|BreakGameTask (Variables|Default|GetActiveTask))) 5.0 false
    (:OnSuccess
      (bind _returnvalue (Class|GameObjectInterface|GetCore(Message) (.To (Utilities|Struct|BreakGameTask (Variables|Default|GetActiveTask)))))
      (bind _returnvalue_2 (Class|GameObjectCore|GetComponent _returnvalue "Inventory"))
      (bind _asinventory_base_component (Utilities|Casting|CastToInventoryBaseComponent _returnvalue_2))
      (bind _returnvalue_3 (Class|InventoryBaseComponent|Push _asinventory_base_component (Utilities|Array|MakeArray (Utilities|Struct|MakePrice (.ResType (Utilities|Struct|BreakGameTask (Variables|Default|GetActiveTask))) (.ResAmount (Utilities|Struct|BreakGameTask (Variables|Default|GetActiveTask)))))))
      (if _returnvalue_3
        (Default|CallOnTaskComplete)
        (else
          (Default|CallOnTaskComplete)
          (Variables|Default|SetActiveTask (Utilities|Struct|MakeGameTask (.TaskPerformer (Utilities|Struct|BreakGameTask (Variables|Default|GetActiveTask))) (.ResType (Utilities|Struct|BreakGameTask (Variables|Default|GetActiveTask))) (.ResAmount (Utilities|Struct|BreakGameTask (Variables|Default|GetActiveTask))) (.To (Utilities|Struct|BreakGameTask (Variables|Default|GetActiveTask))) (.From (Utilities|Struct|BreakGameTask (Variables|Default|GetActiveTask)))))
          (CallFunction|Deliverto))))))

(event EventBeginPlay
  (Utilities|FlowControl|DelayUntilNextTick)
  (AI|RunBehaviorTree (AI|GetAIController self) "/Game/AI/BehaviourTree/BT_Forestling.BT_Forestling")
  (EventDispatchers|BindEventtoOnTaskComplete (delegate Custom|ClearTask))
  (Utilities|Time|SetTimerbyEvent (delegate Custom|GetGameTask) 1.0 true)
  (bind _returnvalue (Class|GameObjectInterface|GetCore))
  (bind _returnvalue_2 (Class|GameObjectCore|GetComponent _returnvalue "Health"))
  (bind _ashealth_default_component (Utilities|Casting|CastToHealthDefaultComponent _returnvalue_2))
  (EventDispatchers|BindEventtoOnDeath _ashealth_default_component (delegate Custom|OnDeath)))

(event EventAttackDefault
  (params (TargetActor :type Actor%20Object%20Reference))
  (if (Math|Random|RandomBool)
    (Variables|Default|SetAttackAnimMontage "/Game/Temp/Character/Forestling/Animation/AM_Forestling_AttackRight.AM_Forestling_AttackRight")
    (else
      (Variables|Default|SetAttackAnimMontage "/Game/Temp/Character/Forestling/Animation/AM_Forestling_AttackTop.AM_Forestling_AttackTop")))
  (|CallParentFunction TargetActor))

(event EventDoTask
  (|CallParentFunction)
  (AI|AIMoveTo self "0, 0, 0" (.From (Utilities|Struct|BreakGameTask (Variables|Default|GetActiveTask))) 5.0 false
    (:OnSuccess
      (bind _returnvalue (Class|GameObjectInterface|GetCore(Message) (.From (Utilities|Struct|BreakGameTask (Variables|Default|GetActiveTask)))))
      (bind _returnvalue_2 (Class|GameObjectCore|GetComponent _returnvalue "Inventory"))
      (bind _asinventory_base_component (Utilities|Casting|CastToInventoryBaseComponent _returnvalue_2))
      (bind _returnvalue_3 (Class|InventoryBaseComponent|Pop _asinventory_base_component (Utilities|Array|MakeArray (Utilities|Struct|MakePrice (.ResType (Utilities|Struct|BreakGameTask (Variables|Default|GetActiveTask))) (.ResAmount (Utilities|Struct|BreakGameTask (Variables|Default|GetActiveTask)))))))
      (if _returnvalue_3
        (AI|AIMoveTo self "0, 0, 0" (.To (Utilities|Struct|BreakGameTask (Variables|Default|GetActiveTask))) 5.0 false
          (:OnSuccess
            (bind _returnvalue_4 (Class|GameObjectInterface|GetCore(Message) (.To (Utilities|Struct|BreakGameTask (Variables|Default|GetActiveTask)))))
            (bind _returnvalue_5 (Class|GameObjectCore|GetComponent _returnvalue_4 "Inventory"))
            (bind _asinventory_base_component_2 (Utilities|Casting|CastToInventoryBaseComponent _returnvalue_5))
            (bind _returnvalue_6 (Class|InventoryBaseComponent|Push _asinventory_base_component_2 (Utilities|Array|MakeArray (Utilities|Struct|MakePrice (.ResType (Utilities|Struct|BreakGameTask (Variables|Default|GetActiveTask))) (.ResAmount (Utilities|Struct|BreakGameTask (Variables|Default|GetActiveTask)))))))
            (if _returnvalue_6
              (Default|CallOnTaskComplete)
              (else
                (Default|CallOnTaskComplete)
                (Variables|Default|SetActiveTask (Utilities|Struct|MakeGameTask (.TaskPerformer (Utilities|Struct|BreakGameTask (Variables|Default|GetActiveTask))) (.ResType (Utilities|Struct|BreakGameTask (Variables|Default|GetActiveTask))) (.ResAmount (Utilities|Struct|BreakGameTask (Variables|Default|GetActiveTask))) (.To (Utilities|Struct|BreakGameTask (Variables|Default|GetActiveTask))) (.From (Utilities|Struct|BreakGameTask (Variables|Default|GetActiveTask)))))
                (CallFunction|Deliverto)))))
        (else
          (Default|CallOnTaskComplete))))))

(fn ConstructionScript)

(fn HasTask
  (Utilities|IsValid (.TaskPerformer (Utilities|Struct|BreakGameTask (Variables|Default|GetActiveTask)))
    (:Is%20Valid
      (return true))
    (:Is%20Not%20Valid
      (return false))))