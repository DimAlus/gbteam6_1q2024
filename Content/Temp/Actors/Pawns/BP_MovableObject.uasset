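; Movable pawn that can attack and die, announcing its spawn, hit and death through the game state's message service as tagged messages.
; On begin play it sends the spawn message and binds to the death event of the Health component obtained from its Core.
; AttackDefault plays an attack montage and applies damage on the Hit notify, then sends the hit message.
; DeathSequence sends the death message, without a sender.
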(event EventBeginPlay
  (Utilities|FlowControl|Sequence
    (:then_0
      (bind _asgame_state_default (Utilities|Casting|CastToGameStateDefault (Game|GetGameState)))
      (bind _returnvalue (Class|GameObjectInterface|GetCore))
      (Class|MessageService|Send (Class|GameStateDefault|GetMessageService _asgame_state_default) (Utilities|Set|MakeSet "GOASpawn") _returnvalue))
    (:then_1
      (bind _returnvalue_2 (Class|GameObjectInterface|GetCore))
      (bind _returnvalue_3 (Class|GameObjectCore|GetComponent _returnvalue_2 "Health"))
      (bind _ashealth_base_component (Utilities|Casting|CastToHealthBaseComponent _returnvalue_3))
      (EventDispatchers|BindEventtoOnDeath _ashealth_base_component (EventDispatchers|CreateEvent :!event DeathSequence)))))

(event EventAttackDefault
  (params (TargetActor :type Actor%20Object%20Reference))
  (bind _notifyname (Animation|Montage|PlayMontage (Variables|Character|GetMesh) (Variables|Default|GetAttackAnimMontage))
    (:OnNotifyBegin
      (if (== _notifyname (Utilities|Name|MakeLiteralName "Hit"))
        (Game|Damage|ApplyDamage TargetActor (Variables|Default|GetDamage) 0 0)
        (bind _asgame_state_default (Utilities|Casting|CastToGameStateDefault (Game|GetGameState)))
        (bind _returnvalue (Class|GameObjectInterface|GetCore))
        (Class|MessageService|Send (Class|GameStateDefault|GetMessageService _asgame_state_default) (Utilities|Set|MakeSet "GOAHit") _returnvalue)))))

(fn ConstructionScript)

(fn DeathSequence
  (Class|MessageService|Send (Class|GameStateDefault|GetMessageService (Variables|Default|GetGameState)) (Utilities|Set|MakeSet "GOADeath")))