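; BP_Wisp is an AI worker pawn that hauls resources between inventories and can also fight with a club.
; While passive, it polls the game state's task manager every second for a task.
; DoTask chains AI moves from source to destination, transferring through its core's inventory, confirming receive and delivery, and pushing items back when a push fails.
; Weapon events spawn or destroy the hand-socketed club, and attacks pick one of two montages at random.
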(event Custom|OnDeath
  ;[1 1 1] OnDeath
)

(event Custom|ClearTask)

(event Custom|GetGameTask
  ;[1 1 1] Check new task
  (bind _state (CallFunction|GetAIState))
  (if (Utilities|Enum|Equal(Enum) _state "Passive")
    (CallFunction|TryGetTask)))

(event Custom|UnequipWeapon
  ;[1 1 1] WeaponTasks
  (Utilities|IsValid (Variables|Default|GetWeaponActor)
    (:Is%20Valid
      (Actor|DestroyActor (Variables|Default|GetWeaponActor)))))

(event Custom|EquipWeapon
  ;[1 1 1] WeaponTasks
  (Utilities|IsValid (Variables|Default|GetWeaponActor)
    (:Is%20Not%20Valid
      (bind _returnvalue (Game|SpawnActorfromClass "/Game/Temp/Actors/Weapons/BP_Club.BP_Club_C" (Math|Transform|MakeTransform "0, 0, 0") "Undefined" "MultiplyWithRoot" 0 0))
      (bind _output_get (Variables|Default|SetWeaponActor _returnvalue))
      (Transformation|AttachComponentToComponent _output_get (Variables|Character|GetMesh) (Utilities|Name|MakeLiteralName "RightHandSocket") "SnapToTarget" "SnapToTarget" "SnapToTarget" true))))

(event EventAttackDefault
  (params (TargetActor :type Actor%20Object%20Reference))
  ;[1 1 1] WeaponTasks
  (if (Math|Random|RandomBool)
    (Variables|Default|SetAttackAnimMontage "/Game/Temp/Character/Forestling/Animation/AM_Forestling_AttackRight.AM_Forestling_AttackRight")
    (else
      (Variables|Default|SetAttackAnimMontage "/Game/Temp/Character/Forestling/Animation/AM_Forestling_AttackTop.AM_Forestling_AttackTop")))
  (|CallParentFunction TargetActor))

(event EventDoTask
  (bind _task (CallFunction|GetTask))
  (bind _task_2 (CallFunction|GetTask))
  (bind _price (Utilities|Struct|MakePrice (.restype _task) (.resamount _task)))
  (bind _price_2 (Utilities|Struct|MakePrice (.restype _task_2) (.resamount _task_2)))
  (bind _array (Utilities|Array|MakeArray _price))
  (bind _array_2 (Utilities|Array|MakeArray _price_2))
  (|CallParentFunction)
  (if (CallFunction|HasTask)
    ;[1 1 1] GoToSource
    (bind _returnvalue (Class|GameObjectCore|GetOwner (.from (CallFunction|GetTask))))
    (AI|AIMoveTo self "0, 0, 0" _returnvalue 5.0 false
      (:OnSuccess
        (if (CallFunction|HasTask)
          (bind _returnvalue_2 (Class|GameObjectCore|GetComponent (.from _task) "Inventory"))
          (bind _asinventory_base_component (Utilities|Casting|CastToInventoryBaseComponent _returnvalue_2)
            (:then
              (bind _returnvalue_3 (Class|InventoryBaseComponent|Pop _asinventory_base_component _array))
              (bind _asgame_state_default (Utilities|Casting|CastToGameStateDefault (Game|GetGameState)))
              (bind _returnvalue_4 (Class|GameObjectInterface|GetCore))
              (if _returnvalue_3
                ;;[1 1 1] push to my inventory
                (bind _returnvalue_5 (Class|GameObjectCore|GetComponent _returnvalue_4 "Inventory"))
                (bind _asinventory_base_component_2 (Utilities|Casting|CastToInventoryBaseComponent _returnvalue_5))
                (bind _returnvalue_6 (Class|InventoryBaseComponent|Push _asinventory_base_component_2 _array))
                (if _returnvalue_6
                  (Class|TaskManagerService|ConfirmReceive (Class|GameStateDefault|GetTaskManagerService _asgame_state_default) _returnvalue_4 true)
                  (bind _returnvalue_7 (Class|GameObjectCore|GetOwner (.to (CallFunction|GetTask))))
                  (AI|AIMoveTo self "0, 0, 0" _returnvalue_7 5.0 false
                    (:OnSuccess
                      (if (CallFunction|HasTask)
                        (bind _returnvalue_8 (Class|GameObjectInterface|GetCore))
                        (bind _returnvalue_9 (Class|GameObjectCore|GetComponent _returnvalue_8 "Inventory"))
                        (bind _asinventory_base_component_3 (Utilities|Casting|CastToInventoryBaseComponent _returnvalue_9)
                          (:then
                            (bind _returnvalue_10 (Class|InventoryBaseComponent|Pop _asinventory_base_component_3 _array_2))
                            (if _returnvalue_10
                              (bind _returnvalue_11 (Class|GameObjectCore|GetComponent (.to _task_2) "Inventory"))
                              (bind _asinventory_base_component_4 (Utilities|Casting|CastToInventoryBaseComponent _returnvalue_11)
                                (:then
                                  (bind _returnvalue_12 (Class|InventoryBaseComponent|Push _asinventory_base_component_4 _array_2))
                                  (if _returnvalue_12
                                    (bind _asgame_state_default_2 (Utilities|Casting|CastToGameStateDefault (Game|GetGameState)))
                                    (bind _returnvalue_13 (Class|GameObjectInterface|GetCore))
                                    (Class|TaskManagerService|ConfirmDelivery (Class|GameStateDefault|GetTaskManagerService _asgame_state_default_2) _returnvalue_13 true)
                                    (Default|CallOnTaskComplete)
                                    (else
                                      (Class|InventoryBaseComponent|Push _asinventory_base_component_3 _array_2)
                                      (bind _returnvalue_14 (Class|GameObjectInterface|GetCore))
                                      (Class|TaskManagerService|ConfirmDelivery (Class|GameStateDefault|GetTaskManagerService _asgame_state_default_2) _returnvalue_14 false)
                                      (CallFunction|CancelTask)
                                      (Default|CallOnTaskComplete))))
                                (:CastFailed
                                  (CallFunction|CancelTask :!label _label)
                                  (Default|CallOnTaskComplete)))
                              (else
                                (goto _label))))
                          (:CastFailed
                            (goto _label)))
                        (else
                          (Default|CallOnTaskComplete :!label _label_2))))
                    (:OnFail
                      (CallFunction|CancelTask)
                      (goto _label_2)))
                  (else
                    (Class|InventoryBaseComponent|Push _asinventory_base_component _array)
                    (Class|TaskManagerService|ConfirmReceive (Class|GameStateDefault|GetTaskManagerService _asgame_state_default) _returnvalue_4 false :!label _label_3)
                    (CallFunction|CancelTask)
                    (Default|CallOnTaskComplete)))
                (else
                  (goto _label_3))))
            (:CastFailed
              (CallFunction|CancelTask)
              (Default|CallOnTaskComplete)))
          (else
            (Default|CallOnTaskComplete :!label _label_4))))
      (:OnFail
        (CallFunction|CancelTask)
        (goto _label_4)))
    (else
      (Default|CallOnTaskComplete))))

(event EventDestroyed
  (bind _weaponactor (Variables|Default|GetWeaponActor))
  ;[1 1 1] OnDeath
  (Utilities|IsValid _weaponactor
    (:Is%20Valid
      (Actor|DestroyActor _weaponactor))))

(event EventBeginPlay
  (|CallParentFunction)
  (EventDispatchers|BindEventtoOnTaskComplete (delegate Custom|ClearTask))
  (Utilities|Time|SetTimerbyEvent (delegate Custom|GetGameTask) 1.0 true)
  (bind _returnvalue (Class|GameObjectInterface|GetCore))
  (bind _returnvalue_2 (Class|GameObjectCore|GetComponent _returnvalue "Health"))
  (bind _ashealth_default_component (Utilities|Casting|CastToHealthDefaultComponent _returnvalue_2))
  (EventDispatchers|BindEventtoOnDeath _ashealth_default_component (delegate Custom|OnDeath)))

(fn ConstructionScript)

(fn TryGetTask
  (bind _asgame_state_default (Utilities|Casting|CastToGameStateDefault (Game|GetGameState)))
  (bind _returnvalue (Class|GameObjectInterface|GetCore))
  (bind _returnvalue_2 (Class|TaskManagerService|GetTask (Class|GameStateDefault|GetTaskManagerService _asgame_state_default) _returnvalue))
  (if _returnvalue_2
    (Default|CallOnTaskReserve)))