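; Wooden house building actor that uses Mapping, Generator and Inventory components retrieved from its Core.
; The Mapping component's OnBuilded event toggles generator work to match the built state and selects the first generation option.
; A fast looping timer prints on-screen debug text showing the current generator's output resource, or NoWork, plus the inventory stacks.
; The construction script initializes the Mapping component.
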(event Custom|CustomEvent
  (bind _returnvalue (Class|GameObjectInterface|GetCore))
  (Utilities|FlowControl|Sequence
    (:then_0
      (bind _returnvalue_2 (Class|GameObjectCore|GetComponent _returnvalue "Generator"))
      (bind _asgenerator_base_component (Utilities|Casting|CastToGeneratorBaseComponent _returnvalue_2))
      (bind _returnvalue_3 (Class|GeneratorBaseComponent|IsWorking _asgenerator_base_component))
      (if _returnvalue_3
        (bind _returnvalue_4 (Class|GeneratorBaseComponent|GetCurrentGenerator _asgenerator_base_component))
        (Development|PrintString (Utilities|String|EnumtoString (.resource (Utilities|Array|Get(acopy) (.Result (Utilities|Struct|BreakBarter (.barter _returnvalue_4)))))) true false "(R=0.000000,G=0.660000,B=1.000000,A=1.000000)" 0.09)
        (else
          (Development|PrintString "NoWork" true false "(R=0.000000,G=0.660000,B=1.000000,A=1.000000)" 0.09))))
    (:then_1
      (bind _returnvalue_5 (Class|GameObjectCore|GetComponent _returnvalue "Inventory"))
      (bind _asinventory_base_component (Utilities|Casting|CastToInventoryBaseComponent _returnvalue_5))
      (bind _returnvalue_6 (Class|InventoryBaseComponent|GetStacks _asinventory_base_component))
      (for _array_element _returnvalue_6
        (Development|PrintString (Utilities|String|Append (Utilities|String|EnumtoString (.resource _array_element)) ": " (Utilities|String|ToString(Integer) (.count _array_element))) true false "(R=1.000000,G=0.166862,B=0.756536,A=1.000000)" 0.09)))))

(event Custom|CustomEvent_0
  (params (IsBuilded :type Boolean))
  (bind _returnvalue (Class|GameObjectInterface|GetCore))
  (bind _returnvalue_2 (Class|GameObjectCore|GetComponent _returnvalue "Generator"))
  (bind _asgenerator_base_component (Utilities|Casting|CastToGeneratorBaseComponent _returnvalue_2))
  (Class|GeneratorBaseComponent|SetWorkEnabled _asgenerator_base_component IsBuilded)
  (Class|GeneratorBaseComponent|ChangeGenerationSelection _asgenerator_base_component 0 true))

(event EventBeginPlay
  (Utilities|FlowControl|DelayUntilNextTick)
  (Utilities|Time|SetTimerbyEvent (delegate Custom|CustomEvent) 0.1 true)
  (bind _returnvalue (Class|GameObjectInterface|GetCore))
  (bind _returnvalue_2 (Class|GameObjectCore|GetComponent _returnvalue "Mapping"))
  (bind _asmapping_base_component (Utilities|Casting|CastToMappingBaseComponent _returnvalue_2))
  (EventDispatchers|BindEventtoOnBuilded _asmapping_base_component (delegate Custom|CustomEvent_0)))

(fn ConstructionScript
  (bind _mappingcomponent (Variables|Default|GetMappingComponent))
  (Class|MappingBaseComponent|Initialize _mappingcomponent (Variables|/Script/GBTeam6.MappingBaseComponent|GetInitializer _mappingcomponent)))