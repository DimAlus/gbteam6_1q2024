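; BP_Dwelling is a dwelling building actor that exposes anchor points for spawning, storage and work.
; Three getter functions return the world transforms of its SpawnPlace, StoragePlace and WorkPlace components.
; It has no active logic of its own, as the construction script is empty and the default events are disabled.
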(event EventBeginPlay)

(event Collision|EventActorBeginOverlap
  (params (OtherActor :type Actor%20Object%20Reference)))

(event EventTick
  (params (DeltaSeconds :type Float%20%28single-precision%29)))

(fn ConstructionScript)

(fn GetSpawnPlace
  (return (Transformation|GetWorldTransform (Variables|Default|GetSpawnPlace))))

(fn GetStoragePlace
  (return (Transformation|GetWorldTransform (Variables|Default|GetStoragePlace))))

(fn GetWorkPlace
  (return (Transformation|GetWorldTransform (Variables|Default|GetWorkPlace))))