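; BP_StandingTorch is an environment torch for human buildings whose point light and Niagara fire toggle with the day/night cycle.
; One second after BeginPlay it shows both if GameStateDefault reports night, then registers with its message service for GLBDay and GLBNight.
; TakeMessage shows them on GLBDay and hides them on GLBNight, the inverse of the initial check.
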(event EventBeginPlay
  (Utilities|FlowControl|Delay 1.0)
  (bind _asgame_state_default (Utilities|Casting|CastToGameStateDefault (Game|GetGameState)))
  (Rendering|SetVisibility (Variables|Default|GetPointLight) (not (Class|GameStateDefault|IsDay _asgame_state_default)) false)
  (Class|MessageService|AddObserver (Class|GameStateDefault|GetMessageService _asgame_state_default) self (Utilities|Set|MakeSet "GLBDay" "GLBNight")))

(event EventTakeMessage
  (params (tags :type Set%20of%20EMessageTag%20Enums :default "None") (sender :type Game%20Object%20Core%20Object%20Reference))
  (bind _pointlight (Variables|Default|GetPointLight))
  (if (Utilities|Set|Contains tags "GLBDay")
    (Rendering|SetVisibility _pointlight true false)
    (elif (Utilities|Set|Contains tags "GLBNight")
      (Rendering|SetVisibility _pointlight false false))))

(fn ConstructionScript)