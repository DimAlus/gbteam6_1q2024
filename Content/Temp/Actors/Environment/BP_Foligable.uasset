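; BP_Foligable is an environment actor that can be selected and, when flagged as foliage, registers its position through a mapping component.
; Select and Deselect toggle its selected flag and switch the mesh's custom depth stencil value.
; The construction script initializes the mapping component, then, for foliage only, passes it the actor's location without updating buildability.
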(event EventSelect
  (Rendering|SetCustomDepthStencilValue (Variables|Default|GetObjectMesh) 1)
  (Variables|Default|SetIsSelected true))

(event EventDeselect
  (Rendering|SetCustomDepthStencilValue (Variables|Default|GetObjectMesh) 0)
  (Variables|Default|SetIsSelected false))

(fn ConstructionScript
  (bind _mappingcomponent (Variables|Default|GetMappingComponent))
  (Class|MappingBaseComponent|Initialize _mappingcomponent (Variables|/Script/GBTeam6.MappingBaseComponent|GetInitializer _mappingcomponent))
  (if (Variables|Default|GetIsFoliage)
    (Class|MappingBaseComponent|SetOwnerLocation (Variables|Default|GetMappingComponent) (Transformation|GetActorLocation) false)))