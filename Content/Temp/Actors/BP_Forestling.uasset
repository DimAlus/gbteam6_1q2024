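; Forestling worker pawn that hauls resources between actors on tasks from the GameState's task manager.
; It runs BT_Forestling and polls the manager on a looping timer to reserve a task.
; DoTask moves to the source, pops the resource from its inventory, then moves to the destination and pushes it there.
; Completion fires a dispatcher that clears the task and notifies the manager; HasTask reports whether one is held.
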(event Custom|DoTask
  (bind _activetask (Variables|Default|GetActiveTask))
  (bind _activetask_2 (Variables|Default|GetActiveTask))
  (bind (_taskperformer _restype _resamount _from) (Utilities|Struct|BreakGameTask _activetask))
  (bind (_taskperformer_2 _restype_2 _resamount_2 _from_2 _to) (Utilities|Struct|BreakGameTask _activetask_2))
  (if (== (.TaskPerformer (Utilities|Struct|BreakGameTask (Variables|Default|GetActiveTask))) self)
    (AI|AIMoveTo self "0, 0, 0" _from 5.0 false
      (:OnSuccess
        (bind _returnvalue (Class|GameObjectInterface|GetCore(Message) _from))
        (bind _returnvalue_2 (Class|GameObjectCore|GetComponent _returnvalue "Inventory"))
        (bind _asinventory_base_component (Utilities|Casting|CastToInventoryBaseComponent _returnvalue_2))
        (Class|InventoryBaseComponent|Pop _asinventory_base_component (Utilities|Array|MakeArray (Utilities|Struct|MakePrice _restype _resamount)))
        (AI|AIMoveTo self "0, 0, 0" _to 5.0 false
          (:OnSuccess
            (bind _returnvalue_3 (Class|GameObjectInterface|GetCore(Message) _to))
            (bind _returnvalue_4 (Class|GameObjectCore|GetComponent _returnvalue_3 "Inventory"))
            (bind _asinventory_base_component_2 (Utilities|Casting|CastToInventoryBaseComponent _returnvalue_4))
            (Class|InventoryBaseComponent|Push _asinventory_base_component_2 (Utilities|Array|MakeArray (Utilities|Struct|MakePrice _restype_2 _resamount_2)))
            (Default|CallOnTaskCompleted)))))))

(event Custom|ClearTask
  (Variables|Default|SetActiveTask (Utilities|Struct|MakeGameTask 0 "Actor"))
  (bind _asgame_state_default (Utilities|Casting|CastToGameStateDefault (Game|GetGameState)))
  (Class|TaskManagerService|CompleteTask (Class|GameStateDefault|GetTaskManagerService _asgame_state_default) self))

(event Custom|GetGameTask
  (bind _asgame_state_default (Utilities|Casting|CastToGameStateDefault (Game|GetGameState)))
  (bind (_tasktoreserve _returnvalue) (Class|TaskManagerService|ReserveTask (Class|GameStateDefault|GetTaskManagerService _asgame_state_default) self))
  (if _returnvalue
    (Variables|Default|SetActiveTask _tasktoreserve)))

(event EventBeginPlay
  (AI|RunBehaviorTree (AI|GetAIController self) "/Game/AI/BehaviourTrees/BT_Forestling.BT_Forestling")
  (EventDispatchers|BindEventtoOnTaskCompleted (delegate Custom|ClearTask))
  (Utilities|Time|SetTimerbyEvent (delegate Custom|GetGameTask) 1.0 true))

(fn ConstructionScript)

(fn HasTask
  (Utilities|IsValid (.TaskPerformer (Utilities|Struct|BreakGameTask (Variables|Default|GetActiveTask)))
    (:Is%20Valid
      (return true))
    (:Is%20Not%20Valid
      (return false))))