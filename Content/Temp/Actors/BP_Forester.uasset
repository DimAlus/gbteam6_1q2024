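; BP_Forester is an actor that repeatedly attacks a target and turns smoothly toward its direction of movement.
; Attack loops a montage while CanAttack holds, applying fixed damage on the DoDamage notify and printing the amount.
; A DoOnce binds CancelAttack to the death event of the target's health component, found through GetCoreMessage.
; CancelAttack clears CanAttack and resets that binding gate, while Tick interpolates yaw from velocity.
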(event Custom|Attack
  (params (TargetActor :type Actor%20Object%20Reference))
  (if (Variables|Default|GetCanAttack)
    (Utilities|FlowControl|Sequence
      (:then_0
        (Utilities|FlowControl|DoOnce false
          (:Completed
            (bind _returnvalue (Class|GameObjectInterface|GetCore(Message) TargetActor))
            (bind _returnvalue_2 (Class|GameObjectCore|GetComponent _returnvalue "Health"))
            (bind _ashealth_base_component (Utilities|Casting|CastToHealthBaseComponent _returnvalue_2))
            (EventDispatchers|BindEventtoOnDeath _ashealth_base_component (delegate Custom|CancelAttack)))))
      (:then_1
        (bind _notifyname (Animation|Montage|PlayMontage (Variables|Default|GetSkeletalMesh) (Variables|Default|GetAttackMontage))
          (:OnCompleted
            (if (Variables|Default|GetCanAttack)
              (CallFunction|Attack TargetActor)))
          (:OnNotifyBegin
            (if (and (== _notifyname "DoDamage") (Variables|Default|GetCanAttack))
              (bind _returnvalue_3 (Game|Damage|ApplyDamage TargetActor 1e+01 0 0))
              (Development|PrintString (Utilities|String|MakeLiteralString (Utilities|String|Append "Damage deal: Amount = " (Utilities|String|ToString(Float) _returnvalue_3)))))))))))

(event Custom|CancelAttack
  (Variables|Default|SetCanAttack false)
  (CallFunction|ResetBindSet))

(event Custom|ResetBindSet
  (Utilities|FlowControl|DoOnce false) ; enters at Reset
)

(event EventTick
  (params (DeltaSeconds :type Float%20%28single-precision%29))
  (bind _returnvalue (Transformation|GetActorRotation))
  (bind _returnvalue_2 (Transformation|GetActorRotation))
  (bind (_roll _pitch _yaw) (Math|Rotator|BreakRotator _returnvalue_2))
  (Transformation|SetActorRotation (Math|Interpolation|RInterpTo _returnvalue (Math|Rotator|Lerp(Rotator) _returnvalue (Math|Rotator|MakeRotator _roll _pitch (+ _yaw (Class|KismetAnimationLibrary|CalculateDirection (Math|Vector|Normalize (Transformation|GetVelocity)) (Transformation|GetActorRotation)))) 0.5 true) DeltaSeconds 2e+01)))

(fn ConstructionScript
  (|CallParentFunction))