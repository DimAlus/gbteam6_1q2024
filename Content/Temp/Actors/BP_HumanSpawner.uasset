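; BP_HumanSpawner is an actor that spawns waves of BP_HumanWarrior at its own location, starting at BeginPlay and repeating on a looping timer.
; GetHumansAmount scales each wave with the number of BP_EnergyGenerator actors in the level, adding a wave-count bonus in later waves.
; Each wave lowers SpawnDelay to a floor, but the timer is set only once, so its interval stays at the initial value.
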(event Custom|SpawnEvent
  (Math|Integer|IncrementInt (Variables|Default|GetWaveCount)
    (:%20%20
      (CallFunction|SpawnHuman))))

(event Custom|SpawnHuman
  (bind _humansamountnum (CallFunction|GetHumansAmount))
  (for _index (range 0 _humansamountnum)
    (Game|SpawnActorfromClass "/Game/Temp/Actors/Pawns/BP_HumanWarrior.BP_HumanWarrior_C" (Math|Transform|MakeTransform (Transformation|GetActorLocation)) "AdjustIfPossibleButDontSpawnIfColliding" "MultiplyWithRoot" 0 0))
  (bind _output_get (Variables|Default|SetSpawnDelay (- (Variables|Default|GetSpawnDelay) 5.0)))
  (if (< _output_get 1e+01)
    (Variables|Default|SetSpawnDelay 1e+01)))

(event EventBeginPlay
  (Utilities|Time|SetTimerbyEvent (delegate Custom|SpawnEvent) (Variables|Default|GetSpawnDelay) true)
  (CallFunction|SpawnHuman))

(fn ConstructionScript)

(fn GetHumansAmount
  (bind _wavecount (Variables|Default|GetWaveCount))
  (bind _returnvalue (- _wavecount 5))
  (bind _outactors (Actor|GetAllActorsOfClass "/Game/Temp/Actors/Buildings/BP_EnergyGenerator.BP_EnergyGenerator_C"))
  (bind _output_get (LocalVariables|SetBasicHumansAmount (Utilities|Array|Length _outactors)))
  (if (> _output_get 0)
    (Math|Integer|DecrementInt _output_get
      (:%20%20
        _)))
  (if (>= _returnvalue 0)
    (return (+ (LocalVariables|GetBasicHumansAmount) _returnvalue))
    (else
      (return (LocalVariables|GetBasicHumansAmount)))))