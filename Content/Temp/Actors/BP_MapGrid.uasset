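; BP_MapGrid is an actor that draws a grid of lines from thin, stretched cube meshes sharing one material.
; Its construction script runs two loops that add perpendicular bars at 100-unit spacing, with no runtime logic.
; Both loops take their count from Width and bar length from Heighgt, so the grid only lines up when square.
; Only the first set of bars has collision disabled.
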(event EventBeginPlay)

(event Collision|EventActorBeginOverlap
  (params (OtherActor :type Actor%20Object%20Reference)))

(event EventTick
  (params (DeltaSeconds :type Float%20%28single-precision%29)))

(fn ConstructionScript
  (bind _heighgt (Variables|Default|GetHeighgt))
  (bind _heighgt_2 (Variables|Default|GetHeighgt))
  (for _index (range 0 (Variables|Default|GetWidth))
    (bind _returnvalue (AddComponent|AddStaticMeshComponent false (Math|Transform|MakeTransform (Math|Vector|MakeVector (Math|Conversions|ToFloat(Integer) (* _index 100)) (Math|Conversions|ToFloat(Integer) (* _heighgt_2 50)) 0.0) "0, 0, 0" (Math|Vector|MakeVector 0.1 (Math|Conversions|ToFloat(Integer) (* _heighgt_2 1)) 0.1))))
    (Components|StaticMesh|SetStaticMesh _returnvalue "/Engine/BasicShapes/Cube.Cube")
    (Rendering|Material|SetMaterial _returnvalue 0 (Variables|Default|GetMaterial))
    (Collision|SetCollisionEnabled _returnvalue "NoCollision"))
  (for _index_2 (range 0 (Variables|Default|GetWidth))
    (bind _returnvalue_2 (AddComponent|AddStaticMeshComponent false (Math|Transform|MakeTransform (Math|Vector|MakeVector (Math|Conversions|ToFloat(Integer) (* _heighgt 50)) (Math|Conversions|ToFloat(Integer) (* _index_2 100)) 0.0) "0, 0, 0" (Math|Vector|MakeVector (Math|Conversions|ToFloat(Integer) (* _heighgt 1)) 0.1 0.09))))
    (Components|StaticMesh|SetStaticMesh _returnvalue_2 "/Engine/BasicShapes/Cube.Cube")
    (Rendering|Material|SetMaterial _returnvalue_2 0 (Variables|Default|GetMaterial))))