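; BP_Saver is a level actor that loads game state at start and handles quick save and load.
; On BeginPlay it loads the GameInstance's slot through the GameState's SaveService; dev maps first generate the map from a tilemap and save afterwards.
; It binds to the player pawn's save and load events, using a QuickSave slot.
; Quick load would reopen MapLand, but HasQuickSave always returns false, leaving it inert.
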(event Custom|Save
  (bind _gamestate (Variables|Default|GetGameState))
  (Class|SaveService|SaveGame (Class|GameStateDefault|GetSaveService _gamestate) _gamestate "QuickSave" (Variables|Default|GetIsDevMap)))

(event Custom|Load
  (bind _result (CallFunction|HasQuickSave))
  (if _result
    (bind _asgame_instance_default (Utilities|Casting|CastToGameInstanceDefault (Game|GetGameInstance)))
    (Variables|/Script/GBTeam6.GameInstanceDefault|SetGameSaveSlot _asgame_instance_default "QuickSave")
    (Game|OpenLevel(byName) "Map/PlayMap/MapLand")))

(event EventBeginPlay
  (bind _isdevmap (Variables|Default|GetIsDevMap))
  (Utilities|FlowControl|DelayUntilNextTick)
  (bind _asgame_state_default (Utilities|Casting|CastToGameStateDefault (Game|GetGameState)))
  (Variables|Default|SetGameState _asgame_state_default)
  (Utilities|FlowControl|Sequence
    (:then_0
      (if _isdevmap
        (CallFunction|GenerateMapbyTilemap)))
    (:then_1
      (bind _asgame_instance_default (Utilities|Casting|CastToGameInstanceDefault (Game|GetGameInstance)))
      (Class|SaveService|LoadGame (Class|GameStateDefault|GetSaveService (Variables|Default|GetGameState)) (Variables|Default|GetGameState) (Variables|/Script/GBTeam6.GameInstanceDefault|GetGameSaveSlot _asgame_instance_default) _isdevmap))
    (:then_2
      (if _isdevmap
        (Class|SaveService|SaveGame (Class|GameStateDefault|GetSaveService (Variables|Default|GetGameState)) (Variables|Default|GetGameState) "" true)))
    (:then_3
      (bind _asbp_player_pawn_default (Utilities|Casting|CastToBP_PlayerPawnDefault (Game|Player|GetPlayerPawn 0)))
      (EventDispatchers|BindEventtoOnSave _asbp_player_pawn_default (delegate Custom|Save))
      (EventDispatchers|BindEventtoOnLoad _asbp_player_pawn_default (delegate Custom|Load)))))

(event Collision|EventActorBeginOverlap
  (params (OtherActor :type Actor%20Object%20Reference)))

(event EventTick
  (params (DeltaSeconds :type Float%20%28single-precision%29)))

(fn ConstructionScript)

(fn GenerateMapbyTilemap
  (Class|MappingService|GenerateMap (Class|GameStateDefault|GetMappingService (Variables|Default|GetGameState)) (Variables|/Script/Paper2D.PaperTileMapComponent|GetTileMap (Variables|/Script/Paper2D.PaperTileMapActor|GetRenderComponent (Variables|Default|GettileMap))) (Variables|Default|GetTileLayerName)))

(fn HasQuickSave
  (return false))